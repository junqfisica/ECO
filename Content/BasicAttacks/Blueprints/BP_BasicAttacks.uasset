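; Base actor for elemental ball attacks, charged and then thrown at a target by a VR motion controller or AI.
; A timeline scales mesh and damage during charge; hand velocity (or an AI-supplied factor) sets launch speed, and slow throws explode.
; A physics impulse hands over to homing projectile movement, with timer-updated inverse-square acceleration and a one-time velocity snap near the target.
; Hits deal damage and exchange Qi through interfaces, then explode.
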(event `self.ReceiveBeginPlay`
  (bind _returnvalue (`self.GetOwner`))
  ;[0.5925 1 0.9701] Sets possible Owner
  (set `self.SpellScale` (`SceneComponent.K2_GetComponentScale` (`self.StaticMeshComponent`)))
  (set `self.OwnerActor` _returnvalue)
  (bind _asbp_motion_controller (cast `/Game/VirtualRealityBP/Blueprints/BP_MotionController` _returnvalue))
  (set `self.PlayerHand` _asbp_motion_controller)
  (set `self.Myself` self))

(event `CastBaseAttack`
  (params (TargetToHit :type "Actor Object Reference"))
  (bind _staticmeshcomponent (`self.StaticMeshComponent`))
  (bind _staticmeshcomponent_2 (`self.StaticMeshComponent`))
  ;[0.635 0.635 0.635] Player cast Node
  ;;[0.2572 0.819 1] Stop the Spell to Charge
  (`self.StopCharge`)
  (`/Engine/EditorBlueprintResources/StandardMacros.IsValid` TargetToHit
    (:`Is Valid`
      ;;[0.5198 0.6751 1] Set the tartget
      (set `self.ProjectileTarget` TargetToHit)
      ;;[0.6432 1 0.5073] Cancel wrist moviments. Makes casting more difficult
      (bind _return (`/Game/VirtualRealityBP/Blueprints/BP_MotionController.IsAngularVelocityPerpendicularToLinearVelocity` (`self.PlayerHand`) false))
      (set `self.SpeedFactor` (`self.GetFactorFromVelocityAndSetActorVelocityVariable`))
      (if (<= (`self.SpeedFactor`) 0.1)
        ;;[1 0.4302 0.3604] Fail To cast
        (`self.DestroyActorAndCastEmitter` "/Game/StarterContent/Particles/P_Explosion.P_Explosion" "/Game/StarterContent/Audio/Explosion_Cue.Explosion_Cue")
        (else
          ;[1 0.9184 0.3915] Set physics to true and add velocity
          (set `self.BaseSpeed` (`KismetMathLibrary.FClamp` (* (`self.SpeedFactor`) (`self.BaseSpeed`)) 500.0 4000.0) :!label _label)
          (`PrimitiveComponent.SetSimulatePhysics` _staticmeshcomponent_2 true)
          (`PrimitiveComponent.AddImpulse` _staticmeshcomponent_2 (* (`KismetMathLibrary.Normal` (`self.ActorVelocity`)) (`self.BaseSpeed`)) "None" true)
          (`KismetSystemLibrary.Delay` 0.0) ; Necessary to cause a small delay
          (`|ExecutionSequence`
            (:`then_0`
              ;[0.6756 0.7708 1] Set Homing Missile
              (bind _returnvalue (`PrimitiveComponent.GetPhysicsLinearVelocity` _staticmeshcomponent "None")))
            (:`then_1`
              (`PrimitiveComponent.SetSimulatePhysics` _staticmeshcomponent false))
            (:`then_2`
              (`SceneComponent.K2_SetWorldRotation` :`self` _staticmeshcomponent)
              (`self.SetHomingMissile` _returnvalue)
              (set `self.BaseAcceleration` (* (`self.GetAccelerationFromBaseSpeed`) (`self.Rescale`)))
              (bind _returnvalue_2 (`KismetSystemLibrary.K2_SetTimerDelegate` (delegate `ModifyVelocity`) 0.05 true))
              (set `self.ModifyVelocityTimeHandler` _returnvalue_2))))))
    (:`Is Not Valid`
      (`KismetSystemLibrary.PrintText` "No target found"))))

(event `CastBaseAttackAI`
  (params (TargetToHit :type "Actor Object Reference") (VelocityDirection :type "Vector Structure") (Factor :type "Float (double-precision)"))
  ;[0.425 0.425 0.425] AI Cast node
  (set `self.SpeedFactor` Factor)
  (set `self.ActorVelocity` VelocityDirection)
  (`/Engine/EditorBlueprintResources/StandardMacros.IsValid` TargetToHit
    (:`Is Valid`
      ;;[0.5198 0.6751 1] Set the tartget
      (set `self.ProjectileTarget` TargetToHit)
      (goto _label))
    (:`Is Not Valid`
      (`KismetSystemLibrary.PrintText` "No target found"))))

(event `ModifyVelocity`
  ;[1 0.8467 0.5559] Modify Velocity Event Node
  (if (`KismetSystemLibrary.K2_IsTimerActiveHandle` (`self.ModifyVelocityTimeHandler`))
    (bind _returnvalue (`PrimitiveComponent.GetPhysicsLinearVelocity` (`self.StaticMeshComponent`) "None"))
    (set `self.ProjectileVelocity` _returnvalue)
    (set `ProjectileMovementComponent.HomingAccelerationMagnitude` (/ (`self.BaseAcceleration`) (+ (`KismetMathLibrary.VSizeSquared` (- (`self.K2_GetActorLocation` (`self.ProjectileTarget`)) (`SceneComponent.K2_GetComponentLocation` (`self.StaticMeshComponent`)))) 1.0)) (`self.ProjectileMovement`))
    (`self.IsProjectileCloseToTarget`
      (:`Yes`
        (if (not (`self.isInitialVelocityReset`))
          ;;[0.9086 1 0.6564] Change velocity to target's direction
          (`ProjectileMovementComponent.SetVelocityInLocalSpace` (`self.ProjectileMovement`) (* (`KismetMathLibrary.Normal` (- (`self.K2_GetActorLocation` (`self.ProjectileTarget`)) (`SceneComponent.K2_GetComponentLocation` (`self.StaticMeshComponent`)))) (`KismetMathLibrary.VSize` (`self.ProjectileVelocity`))))
          (set `self.isInitialVelocityReset` true))))))

(event `self.StaticMeshComponent.OnComponentHit`
  (params (HitComponent :type "PrimitiveComponent Object Reference") (OtherActor :type "Actor Object Reference") (OtherComp :type "PrimitiveComponent Object Reference") (NormalImpulse :type "Vector Structure") (Hit :type "HitResult Structure (by ref)"))
  (bind _actorhitbyattack (`self.ActorHitByAttack`))
  (bind _returnvalue (`self.GetOwner` (`self.ActorHitByAttack`)))
  (set `self.ActorHitByAttack` OtherActor)
  (`|ExecutionSequence`
    (:`then_0`
      ;[0.7602 1 0.6404] Call OnDamage if the actor has the BPI_TakeDamage implement.
      (if (`KismetSystemLibrary.DoesImplementInterface` (`self.ActorHitByAttack`) "/Game/Interfaces/BPI_TakeDamage.BPI_TakeDamage_C")
        (message `/Game/Interfaces/BPI_TakeDamage.OnDamage` _actorhitbyattack (`self.BaseDamage`))
        (`KismetSystemLibrary.PrintText` (`KismetTextLibrary.Conv_StringToText` (`KismetStringLibrary.Concat_StrStr` "Attack hit: " (`KismetSystemLibrary.GetDisplayName` _actorhitbyattack))))))
    (:`then_1`
      ;[0.6377 0.8887 1] Call Recive Qi to give the players or the AI certain amount of Qi
      ;;[0.5503 0.59 0.4513] If hit actor implements GiveQi interface
      (if (`KismetSystemLibrary.DoesImplementInterface` (`self.ActorHitByAttack`) "/Game/Interfaces/BPI_GiveQi.BPI_GiveQi_C")
        ;;[0.5801 0.6921 1] Gets the amount of Qi recived
        (bind (_returnamount _giveqitoowner) (message `/Game/Interfaces/BPI_GiveQi.GiveQi` (`self.ActorHitByAttack`) (`self.GiveQi`)))
        (`|ExecutionSequence`
          (:`then_0`
            ;;[1 0.6561 0.8575] Owner recives Qi
            (if (`KismetSystemLibrary.DoesImplementInterface` (`self.OwnerActor`) "/Game/Interfaces/BPI_reciveQi.BPI_ReciveQi_C")
              (message `/Game/Interfaces/BPI_reciveQi.ReciveQi` (`self.OwnerActor`) _returnamount)))
          (:`then_1`
            ;;[0.5377 0.8265 1] Give Qi to the owner of the Barrier or Shield
            (if _giveqitoowner
              (if (`KismetSystemLibrary.DoesImplementInterface` _returnvalue "/Game/Interfaces/BPI_reciveQi.BPI_ReciveQi_C")
                (message `/Game/Interfaces/BPI_reciveQi.ReciveQi` _returnvalue _returnamount)))))))
    (:`then_2`
      ;[1 0.5601 0.5302] Cast Explosion on hit
      (`self.DestroyActorAndCastEmitter` "/Game/StarterContent/Particles/P_Explosion.P_Explosion" "/Game/StarterContent/Audio/Explosion_Cue.Explosion_Cue"))))

(event `/Game/Interfaces/BPI_IsChargeble.StartCharge`
  (bind _myself (`self.Myself`))
  ;[0.1113 0.3075 0.53 0.5] Start/Stop Charge Attack. Each attack has to implent its own Events
  (`KismetSystemLibrary.PrintText` "Default Start Charge")
  (bind (_direction _percentdamage _percentscale) (`Timeline|ChargeSpell` :!via `PlayFromStart` :!label _label_2)
    (:`Update`
      ;;[0.255 0.255 0.255] Update Node
      ;;;[0.5705 0.6356 1] Change the scale of the mesh
      (`SceneComponent.SetWorldScale3D` (`self.StaticMeshComponent`) (* (`self.SpellScale`) _percentscale))
      ;;;[0.5245 1 0.7717] Charge the damage
      (set `self.DamageCharged` (* _percentdamage (`KismetMathLibrary.Conv_IntToDouble` (`self.BaseDamage`)))))
    (:`Finished`
      ;;[0.5412 1 0.9801] When damage is 0, reverse the scale and destroy the spell
      (switch `ETimelineDirection` _direction
        (:`Backward`
          (`self.K2_DestroyActor`))))
    (:`ChangeVisualFire`
      ;;[0.7764 0.5728 1] Change the visual of each element based on event tracks
      (bind _asbp_fire_ball (cast `/Game/BasicAttacks/Blueprints/BP_FireBall` _myself))
      (`/Game/BasicAttacks/Blueprints/BP_FireBall.ChangeVisualFire` _asbp_fire_ball))
    (:`ChangeVisualEarth`
      (bind _asbp_earth_ball (cast `/Game/BasicAttacks/Blueprints/BP_EarthBall` _myself))
      (`/Game/BasicAttacks/Blueprints/BP_EarthBall.ChangeEarthVisual` _asbp_earth_ball))
    (:`ChangeVisualWind`
      (bind _asbp_wind_ball (cast `/Game/BasicAttacks/Blueprints/BP_WindBall` _myself))
      (`/Game/BasicAttacks/Blueprints/BP_WindBall.ChangeWindVisual` _asbp_wind_ball))
    (:`ChangeVisualWater`
      (bind _asbp_water_ball (cast `/Game/BasicAttacks/Blueprints/BP_WaterBall` _myself))
      (`/Game/BasicAttacks/Blueprints/BP_WaterBall.ChangeWaterVisual` _asbp_water_ball))))

(event `/Game/Interfaces/BPI_IsChargeble.StopCharge`
  ;[0.1113 0.3075 0.53 0.5] Start/Stop Charge Attack. Each attack has to implent its own Events
  (`KismetSystemLibrary.PrintText` "Default Stop Charge")
  (bind _output_get (set `self.BaseDamage` (`KismetMathLibrary.Round` (`self.DamageCharged`))))
  (if (> _output_get 0)
    (goto _label_2 :!via `Stop`)
    (else
      (`TimelineComponent.SetPlayRate` (`self.ChargeSpell`) (`self.FadeOutPlayRate`))
      (goto _label_2 :!via `Reverse`))))

(fn `DestroyActorAndCastEmitter`
  (params (Emitter :type "ParticleSystem Object Reference") (Sound :type "SoundBase Object Reference"))
  (`/Engine/EditorBlueprintResources/StandardMacros.DoOnce` false
    (:`Completed`
      (bind _returnvalue (`GameplayStatics.SpawnEmitterAtLocation` Emitter (`SceneComponent.K2_GetComponentLocation` (`self.StaticMeshComponent`))))
      (`GameplayStatics.SpawnSoundAttached` Sound _returnvalue "None" (0.0 0.0 0.0) (struct) "KeepRelativeOffset" false 1.0 0.4)
      (`self.K2_DestroyActor`))))

(fn `GetAccelerationFromBaseSpeed`
  (returns (BaseAcceleration :type "Float (double-precision)"))
  (return (+ (* (`self.BaseSpeed`) 0.00095) 0.18)))

(fn `GetFactorFromVelocityAndSetActorVelocityVariable`
  (returns (Factor :type "Float (double-precision)"))
  ;[1 0.9832 0.5925] Convert the hand speed to a factot between 0-1
  (bind _actorvelocity (`self.GetVelocityWithoutSmallVariations`))
  (`self.K2_DetachFromActor` "KeepWorld" "KeepWorld" "KeepWorld")
  (set `self.ActorVelocity` _actorvelocity)
  (bind _factor (`/Game/FunctionLibrary/MyFunctions.ConvertSpeedToFactorZeroToOne` (`KismetMathLibrary.VSize` (`self.ActorVelocity`)) (`self.MaxPlayerSpeedInput`) (`self.SpeedAt30PercentFactor`)))
  (return _factor))

(fn `GetVelocityWithoutSmallVariations`
  (returns (ActorVelocity :type "Vector Structure"))
  (locals (Zero :type "Float (double-precision)") (VelocityArray :type "Array of Float (double-precision)") (Velocity :type "Vector Structure") (VectorLength :type "Float (double-precision)" :default 1.0) (CutSpeedArray :type "Array of Float (double-precision)"))
  (bind _velocityarray (`local.VelocityArray`))
  (bind _vectorlength (`local.VectorLength`))
  (bind _cutanglesvariationof (`self.CutAnglesVariationOf`))
  (bind _returnvalue (`KismetMathLibrary.DegSin` _cutanglesvariationof))
  (bind _returnvalue_2 (* (`KismetMathLibrary.DegCos` _cutanglesvariationof) _returnvalue _vectorlength))
  (bind _returnvalue_3 (`PrimitiveComponent.GetPhysicsLinearVelocity` (`self.StaticMeshComponent`) "None"))
  (`|ExecutionSequence`
    (:`then_0`
      ;[1 1 1] Set the vector leght if it is zero vector length is equal 1
      (bind _output_get (set `local.Velocity` (`KismetMathLibrary.MakeVector` (.x _returnvalue_3) (.y _returnvalue_3) (.z _returnvalue_3))))
      (bind _returnvalue_4 (`KismetMathLibrary.VSize` _output_get))
      (if (!= _returnvalue_4 0.0)
        (set `local.VectorLength` _returnvalue_4)
        ;[1 1 1] Get the cut speed values for each component of velocity. The cut is based on the angle cut.
        (set `local.CutSpeedArray` (`|MakeArray` _returnvalue_2 _returnvalue_2 (* _returnvalue _vectorlength)))))
    (:`then_1`
      (bind _output_get_2 (set `local.VelocityArray` (`|MakeArray` (.x _returnvalue_3) (.y _returnvalue_3) (.z _returnvalue_3))))
      (for (_array_element _array_index) _output_get_2
        ;[1 0.8453 0.3813] LoopBody: Check if Vi/V is smaller than the cut value, if so set vi to zero. Where i = x,y,z
        (if (< (`KismetMathLibrary.Abs` _array_element) (`KismetArrayLibrary.Array_Get` (`local.CutSpeedArray`) _array_index))
          (`KismetArrayLibrary.Array_Set` _velocityarray _array_index (`local.Zero`))))
      (return (`KismetMathLibrary.MakeVector` (`KismetArrayLibrary.Array_Get` _velocityarray) (`KismetArrayLibrary.Array_Get` _velocityarray 1) (`KismetArrayLibrary.Array_Get` _velocityarray 2))))))

(fn `UserConstructionScript`
  (locals (DamageTrack :type Name :default "PercentDamage") (ScaleTrack :type Name :default "PercentScale"))
  (bind _chargespell (`self.ChargeSpell`))
  ;[0.642 0.9501 1] Sets the curve for each element
  (`TimelineComponent.SetFloatCurve` _chargespell (`self.UseScaleCurve`) (`local.ScaleTrack`))
  (`TimelineComponent.SetFloatCurve` _chargespell (`self.UseDamageCurve`) (`local.DamageTrack`)))