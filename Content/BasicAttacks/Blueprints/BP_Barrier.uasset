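; Barrier actor for a basic attack, cast by the motion-controller player pawn or an AI enemy at a Qi cost.
; On BeginPlay it charges the owner's Qi or destroys itself, then offsets the mesh vertically, sets life and applies a randomly signed rotation offset.
; Functions raise and lower it within Z limits and return scaled Qi.
; Damage drains life until it expires; a separate event sets a timed lifespan.
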(event `self.ReceiveBeginPlay`
  (bind _staticmeshcomponent (`self.StaticMeshComponent`))
  (bind _player (`self.OwnerIsAPlayer`)
    (:`Yes`
      ;[0 1 0.6776] See if Player has enough Qi to Cast this barrier
      (`self.CanBeCast` _player
        (:`Yes`
          _)))
    (:`No`
      (bind _asaienemy_bp (cast `/Game/AI/AIEnemy_BP` (`self.GetOwner` self)))
      (`self.CanBeCastAI` _asaienemy_bp
        (:`Yes`
          _))))
  (`|ExecutionSequence`
    (:`then_0`
      ;[1 0.6995 0.8682] Set the OffSet
      (`SceneComponent.K2_AddWorldOffset` (`self.StaticMeshComponent`) (`KismetMathLibrary.MakeVector` 0.0 0.0 (`self.StartZLocation`)) false false))
    (:`then_1`
      ;[1 0.3944 0.8064] Set initial life
      (set `self.CurrentLife` (`self.BaseBarrierLife`))
      ;[1 0.506 0.8554] Set off set rotation
      (if (`KismetMathLibrary.RandomBoolWithWeight` 0.5)
        (set `self.DirectionOfRotation` 1.0)
        (else
          (set `self.DirectionOfRotation` -1.0)))
      (`SceneComponent.K2_SetWorldRotation` _staticmeshcomponent (`KismetMathLibrary.ComposeRotators` (* (`self.RotationOffSet`) (`self.DirectionOfRotation`)) (`SceneComponent.K2_GetComponentRotation` _staticmeshcomponent)) false false))))

(event `/Game/Interfaces/BPI_TakeDamage.OnDamage`
  (params (Damage :type Integer))
  ;[0.6301 1 0.94] On Barrier Damage
  (bind _output_get (set `self.CurrentLife` (- (`self.CurrentLife`) Damage)))
  (if (<= _output_get 0)
    (`self.SetLifeSpan` 0.2)))

(event `SelfDestroyAfterTimeLife`
  ;[0.3904 0.6632 1] Self Destroy after a given time
  (`self.SetLifeSpan` (`self.TimeLife`)))

(fn `BringDownBarrierAtZDirection`
  (params (DetaZ :type "Float (double-precision)"))
  (bind _returnvalue (`self.GetTransform`))
  ;[1 0.7759 0.6537] Bring Down the barrier by deltaZ
  (`self.K2_SetActorTransform` (`KismetMathLibrary.MakeTransform` (`KismetMathLibrary.MakeVector` (.x (.location _returnvalue)) (.y (.location _returnvalue)) (`KismetMathLibrary.FClamp` (- (.z (.location _returnvalue)) DetaZ) (`self.EndZLocation_0`) (`self.StartZLocation`))) (.rotation _returnvalue) (.scale _returnvalue))))

(fn `GiveQi`
  (params (InitialAmount :type Integer))
  (returns (ReturnAmount :type Integer) (GiveQiToOwner :type Boolean))
  (return (`KismetMathLibrary.FTrunc` (* InitialAmount (`self.QiMultiplier`))) true))

(fn `GrowBarrierAtZDirection`
  (params (DeltaZ :type "Float (double-precision)" :default 0.0))
  (bind _returnvalue (`self.GetTransform`))
  ;[1 0.7759 0.6537] Grow the barrier by deltaZ
  (`self.K2_SetActorTransform` (`KismetMathLibrary.MakeTransform` (`KismetMathLibrary.MakeVector` (.x (.location _returnvalue)) (.y (.location _returnvalue)) (`KismetMathLibrary.FClamp` (+ (.z (.location _returnvalue)) DeltaZ) (`self.StartZLocation`) (`self.EndZLocation_0`))) (.rotation _returnvalue) (.scale _returnvalue))))

(fn `UserConstructionScript`)