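; Dummy_BP is a target dummy that ragdolls when hit and replaces itself with a fresh copy.
; The first hit on its skeletal mesh enables physics, launches it along the impact normal and starts a short lifespan.
; After a brief delay it spawns a new dummy at a fixed transform and sets it as the MPMotionControllerPawn player's EnemyTarget.
; GetTargetComponent exposes the Body component for targeting.
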(event `self.SkeletalMesh.OnComponentHit`
  (params (HitComponent :type "PrimitiveComponent Object Reference") (OtherActor :type "Actor Object Reference") (OtherComp :type "PrimitiveComponent Object Reference") (NormalImpulse :type "Vector Structure") (Hit :type "HitResult Structure (by ref)"))
  (bind _skeletalmesh (`self.SkeletalMesh`))
  (if (not (`SceneComponent.IsSimulatingPhysics` (`self.SkeletalMesh`) "None"))
    (`PrimitiveComponent.SetSimulatePhysics` _skeletalmesh true)
    (`PrimitiveComponent.AddImpulse` _skeletalmesh (* (`KismetMathLibrary.Normal` (`.ImpactNormal` (`GameplayStatics.BreakHitResult` Hit))) 10000.0) "None" true)
    (`self.SetLifeSpan` 5.0)
    (`KismetSystemLibrary.Delay` 1.0)
    (bind _returnvalue (`|SpawnActorFromClass` "Dummy_BP_C" (`KismetMathLibrary.MakeTransform` (0.0 0.0 80.0) (struct :`Yaw` 90.0)) "AdjustIfPossibleButAlwaysSpawn" "OverrideRootScale"))
    (bind _asmpmotion_controller_pawn (cast `/Game/VirtualRealityBP/Blueprints/MPMotionControllerPawn` (`GameplayStatics.GetPlayerPawn` 0)))
    (set `/Game/VirtualRealityBP/Blueprints/MPMotionControllerPawn.EnemyTarget` _returnvalue _asmpmotion_controller_pawn)))

(fn `GetTargetComponent`
  (returns (Target :type "StaticMeshComponent Object Reference"))
  (return (`self.Body`)))

(fn `UserConstructionScript`)