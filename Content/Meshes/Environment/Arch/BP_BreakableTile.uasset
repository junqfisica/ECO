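; BP_BreakableTile is an environment tile that shatters when a BP_Barrier overlaps its box.
; On overlap it hides the intact static mesh, shows the destructible mesh and applies radius damage at that mesh's location to fracture it with an impulse.
; A timer then destroys the actor a few seconds later, clearing the debris.
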(event `self.Box.OnComponentBeginOverlap`
  (params (OverlappedComponent :type "PrimitiveComponent Object Reference") (OtherActor :type "Actor Object Reference") (OtherComp :type "PrimitiveComponent Object Reference") (OtherBodyIndex :type Integer) (bFromSweep :type Boolean) (SweepResult :type "HitResult Structure (by ref)"))
  (bind _sm_tilebreakable_dm (`self.SM_TileBreakable_DM`))
  (cast `/Game/Spells/Blueprints/BP_Barrier` OtherActor)
  (`SceneComponent.SetVisibility` (`self.SM_TileBreakable`) false false)
  (`SceneComponent.SetVisibility` (`self.SM_TileBreakable_DM`) true false)
  (`DestructibleComponent.ApplyRadiusDamage` _sm_tilebreakable_dm 1000.0 (`SceneComponent.K2_GetComponentLocation` _sm_tilebreakable_dm) 200.0 100.0 true)
  (`KismetSystemLibrary.K2_SetTimerDelegate` (delegate `Destroy Self`) 7.0))

(event `Destroy Self`
  (`/Engine/EditorBlueprintResources/StandardMacros.IsValid` self
    (:`Is Valid`
      (`self.K2_DestroyActor`))))

(fn `UserConstructionScript`)