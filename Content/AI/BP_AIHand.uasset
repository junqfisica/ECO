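; BP_AIHand is one hand of an AI enemy, casting basic attacks and raising shields for its owner.
; Randomized timers drive volleys of charged spells, each launched along a random cone direction that projectile path prediction tests for obstructions.
; Shielding cancels any active attack, then a looping timer rotates the spring-arm-mounted shield using traces toward the tracked target.
; When that target is lost, a timeline returns the shield to rest and destroys it.
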(event `self.ReceiveBeginPlay`
  (bind _arrow (`self.Arrow`))
  (`|ExecutionSequence`
    (:`then_0`
      (`KismetSystemLibrary.Delay` 0.2)
      (bind _asbp_aienemy_update (cast `/Game/AI/BP_AIEnemy_Update` (`ActorComponent.GetOwner` (`SceneComponent.GetAttachParent` (`self.DefaultSceneRoot`)))))
      (set `self.AIOwner` _asbp_aienemy_update))
    (:`then_1`
      (switch `EControllerHand` (`self.Hand`)
        (:`Left`
          (`SceneComponent.K2_AddRelativeRotation` _arrow (struct :`Pitch` -80.0) false false))
        (:`Right`
          (`SceneComponent.K2_AddRelativeRotation` _arrow (struct :`Pitch` 80.0) false false))))))

(event `StartBasicAttack`
  (params (WhatToCast :type "Actor Class Reference"))
  (bind _aiowner (`self.AIOwner`))
  ;[1 1 1] Basic Attack Node
  (if (not (or (`KismetSystemLibrary.K2_IsTimerActiveHandle` (`self.ChargeAttackTimerHandler`)) (`KismetSystemLibrary.K2_IsTimerActiveHandle` (`self.ActivateAttackTimeHandler`))))
    (set `self.WhatToCast` WhatToCast)
    (bind _returnvalue (`KismetSystemLibrary.K2_SetTimerDelegate` (delegate `IniticiateAttack`) (`KismetMathLibrary.RandomFloatInRange` (`/Game/AI/BP_AIEnemy_Update.MinimunTimeToTriggerBasicAttack` _aiowner) (`/Game/AI/BP_AIEnemy_Update.MaximumTimeToTriggerBasicAttack` _aiowner))))
    (set `self.ChargeAttackTimerHandler` _returnvalue)))

(event `IniticiateAttack`
  ;[1 1 1] Basic Attack Node
  ;;[0.5431 1 0.6432] Activate and charge each attack
  (switch `/Game/VirtualRealityBP/Enumerates/ECastStatus` (`self.CastStatus`)
    (:`NewEnumerator4`
      ;;;[0.7143 1 0.5284] Activate BasicAttack
      (`self.ActivateBasicAttack` (`self.WhatToCast`))
      ;;[0.3521 0.6058 1] Checks if timer is active, if not activate.
      (`/Game/FunctionLibrary/MyMacroLibrary.IsTimeHandlerActive` (`self.ActivateAttackTimeHandler`)
        (:`False`
          ;;[0.2868 0.9202 1] Starts timer and reset initial parameters
          (bind _returnvalue (`KismetSystemLibrary.K2_SetTimerDelegate` (delegate `ReleaseOnPunch`) 0.5 true))
          (set `self.ActivateAttackTimeHandler` _returnvalue)
          (set `self.AttacksRelesed` 0)
          (`self.ResetPunch`))))))

(event `ReleaseOnPunch`
  (bind _firerate (`/Game/AI/BP_AIEnemy_Update.Firerate` (`self.AIOwner`)))
  ;[1 1 1] Basic Attack Node
  (`/Engine/EditorBlueprintResources/StandardMacros.DoOnce` false :!label _label
    (:`Completed`
      (`KismetSystemLibrary.Delay` (`self.GetTimeToChargeAttack`))
      (`/Engine/EditorBlueprintResources/StandardMacros.CompareInt` (`self.AttacksRelesed`) 4
        (:`==`
          ;;[1 0.7865 0.3997] Last attack. After cast deactivate the attack stoping the timer.
          (`self.CastAttack`)
          (`/Engine/EditorBlueprintResources/StandardMacros.IncrementInt` (`self.AttacksRelesed`)
            (:`  `
              (`KismetSystemLibrary.Delay` 0.2)
              (`self.DeactivateAndDestroySpell`)
              (`self.ResetPunch`))))
        (:`<`
          ;;[0.4574 1 0.9701] Attack is not over yet. Keep Spawing more.
          (`self.CastAttack`)
          (`KismetSystemLibrary.Delay` 0.2) ; Necessary to don't overlap actions
          (`/Game/FunctionLibrary/MyMacroLibrary.IsTimeHandlerActive` (`self.ActivateAttackTimeHandler`)
            (:`True`
              (`self.IniticiateAttack`)
              (`KismetSystemLibrary.Delay` (`KismetMathLibrary.RandomFloatInRange` (- _firerate (* _firerate 0.1)) _firerate))
              (`/Engine/EditorBlueprintResources/StandardMacros.IncrementInt` (`self.AttacksRelesed`)
                (:`  `
                  (`self.ResetPunch`))))))))))

(event `ResetPunch`
  ;[1 1 1] Basic Attack Node
  (goto _label :!via `Reset`))

(event `CastAttack`
  (bind _activespell (`self.ActiveSpell`))
  ;[1 1 1] Basic Attack Node
  ;;[1 0.8962 0.5284] Execute Attack
  (`/Engine/EditorBlueprintResources/StandardMacros.IsValid` _activespell
    (:`Is Valid`
      (bind _asbp_basic_attacks (cast `/Game/Spells/Blueprints/BP_BasicAttacks` _activespell))
      (`self.CastBasicAttack` (`/Game/AI/BP_AIEnemy_Update.EnemyTarget` (`self.AIOwner`)) _asbp_basic_attacks)
      (`self.DeactivateSpell`))
    (:`Is Not Valid`
      (`KismetSystemLibrary.PrintText` "No Spell Active")
      (`self.DeactivateSpell`))))

(event `ActivateShield`
  (params (ShieldToCast :type "/Game/Spells/Blueprints/BP_Shield Class Reference") (TargetToFollow :type "Actor Object Reference"))
  (switch `/Game/VirtualRealityBP/Enumerates/ECastStatus` (`self.CastStatus`)
    (:`NewEnumerator4`
      _)
    (:`NewEnumerator0`
      (`self.DeactivateandDestroySpell`))
    (:`NewEnumerator1`
      _))
  (`|ExecutionSequence`
    (:`then_0`
      (`/Engine/EditorBlueprintResources/StandardMacros.IsValid` (`self.ShieldActive`)
        (:`Is Not Valid`
          (`self.ActivateShiled` ShieldToCast))))
    (:`then_1`
      (`/Engine/EditorBlueprintResources/StandardMacros.IsValid` (`self.CurrentFollowingTarget`)
        (:`Is Not Valid`
          (set `self.CurrentFollowingTarget` TargetToFollow))))
    (:`then_2`
      (`/Game/FunctionLibrary/MyMacroLibrary.IsTimeHandlerActive` (`self.FollowingTargetTimerHandler`)
        (:`False`
          (bind _returnvalue (`KismetSystemLibrary.K2_SetTimerDelegate` (delegate `FollowTarget`) 0.1 true))
          (set `self.FollowingTargetTimerHandler` _returnvalue))))))

(event `RestShield`
  (bind _springarm (`self.SpringArm`))
  ;[0.2923 1 0.4974] Rest Shield
  (`/Engine/EditorBlueprintResources/StandardMacros.DoOnce` false :!label _label_2
    (:`Completed`
      (`TimelineComponent.SetPlayRate` (`self.PutShieldToRest`) (/ 1.0 (`/Game/AI/BP_AIEnemy_Update.MaximumTimeForReactionInSec` (`self.AIOwner`))))
      (bind (_direction _alpha) (`Timeline|PutShieldToRest` :!via `PlayFromStart`)
        (:`Update`
          ;;[1 0.6832 0.8279] Once the target is not avaible anymore start to rotate the shiled back to its original position.
          (`SceneComponent.K2_SetRelativeRotation` _springarm (`KismetMathLibrary.RLerp` (`SceneComponent.RelativeRotation` _springarm) (struct) _alpha true) false false))
        (:`Finished`
          ;;[1 0.6063 0.4135] Clear Timer when projectile is not valide. This makes the function to stop been called
          (`self.DeactivateandDestroySpell`)
          (`self.OpenRestShield`)
          (goto _label_2 :!via `Reset`))))))

(event `FollowTarget`
  ;[0.7021 0.7342 1] This function moves the shield to block the attacks
  (bind _isfinished (`self.MovesShieldToDefend` (`self.CurrentFollowingTarget`)))
  (if _isfinished
    ;;[0.4999 1 0.9901] Put shield to rest after x secs, if there is no target to follow.
    (`/Engine/EditorBlueprintResources/StandardMacros.DoOnce` false :!label _label_3
      (:`Completed`
        (`KismetSystemLibrary.Delay` (`KismetMathLibrary.RandomFloatInRange` 2.0 4.0))
        (`/Engine/EditorBlueprintResources/StandardMacros.IsValid` (`self.CurrentFollowingTarget`)
          (:`Is Valid`
            (`self.OpenRestShield`))
          (:`Is Not Valid`
            (`self.RestShield`)))))))

(event `OpenRestShield`
  ;[0.7021 0.7342 1] This function moves the shield to block the attacks
  (goto _label_3 :!via `Reset`))

(fn `ActivateBasicAttack`
  (params (SpawnAttackOfClass :type "Actor Class Reference"))
  ;[0.5955 1 0.9198] Activate Base attack
  (bind _returnvalue (`|SpawnActorFromClass` SpawnAttackOfClass (`KismetMathLibrary.MakeTransform` (0.0 0.0 0.0) (struct) (1.0 1.0 1.0)) "AlwaysSpawn" "OverrideRootScale" (`self.AIOwner`)))
  (bind _output_get (set `self.ActiveSpell` _returnvalue))
  (`self.K2_AttachToComponent` _output_get (`self.OnlyVisualToTest`) "None" "KeepRelative" "KeepRelative" "KeepRelative" true)
  ;;[0.4432 1 0.8384] Charge Basic attack
  (message `/Game/Interfaces/BPI_IsChargeble.StartCharge` _output_get)
  (set `self.CastStatus` "NewEnumerator0"))

(fn `ActivateShiled`
  (params (ShieldToSpawn :type "/Game/Spells/Blueprints/BP_Shield Class Reference"))
  (bind _returnvalue (`|SpawnActorFromClass` ShieldToSpawn (`KismetMathLibrary.MakeTransform` (0.0 0.0 0.0) (struct :`Pitch` 90.0)) "AlwaysSpawn" "OverrideRootScale" (`self.AIOwner`)))
  (bind _output_get (set `self.ShieldActive` _returnvalue))
  (`SceneComponent.K2_AttachToComponent` (`StaticMeshActor.StaticMeshComponent` _output_get) (`self.SpringArm`) "None" "KeepRelative" "KeepRelative" "KeepRelative" false)
  (set `self.CastStatus` "NewEnumerator1"))

(fn `CastBasicAttack`
  (params (TargetToHit :type "Actor Object Reference") (BasicAttack :type "/Game/Spells/Blueprints/BP_BasicAttacks Object Reference"))
  (locals (LocalZAxis :type "Float (double-precision)" :default 2.0) (SpawnPoint :type "Vector Structure") (LDirectionToCast :type "Vector Structure") (LSpawnAttack :type "/Game/Spells/Blueprints/BP_BasicAttacks Object Reference") (SpeedyFactor :type "Float (double-precision)") (ObjectTypestoScan :type "Array of EObjectTypeQuery Enum") (EnemyTarget :type "Actor Object Reference") (LIgnoreCollision :type "Array of Actor Object Reference"))
  (bind _lspawnattack (`local.LSpawnAttack`))
  ;[0.5955 1 0.9198] Cast Base attack
  (set `local.EnemyTarget` TargetToHit)
  (set `local.LSpawnAttack` BasicAttack)
  (set `local.LIgnoreCollision` (`|MakeArray` self (`local.LSpawnAttack`) (`local.EnemyTarget`) (`self.AIOwner`) :!type "Actor Object Reference"))
  (set `local.SpawnPoint` (`self.K2_GetActorLocation`))
  (for _index (range 101)
    (bind _output_get (set `local.LDirectionToCast` (`KismetMathLibrary.RandomUnitVectorInConeWithYawAndPitch` (`KismetMathLibrary.Normal` (`SceneComponent.GetForwardVector` (`self.Arrow`))) 90.0 90.0)))
    ;;[0.06647 0.0886 0.1746] Check if vector is antiparallel
    (`/Game/FunctionLibrary/MyMacroLibrary.VectorsAreOpposite?` (`KismetMathLibrary.MakeVector` (.x _output_get) (.y _output_get)) (`SceneComponent.GetForwardVector` (`self.Arrow`))
      (:`NotOpposite`
        (`/Engine/EditorBlueprintResources/StandardMacros.IsValid` (`local.LSpawnAttack`)
          (:`Is Valid`
            ;;[0 0 0] Calculation of velocity
            (bind _output_get_2 (set `local.SpeedyFactor` (`KismetMathLibrary.RandomFloatInRange` 0.7 1.0)))
            ;;[0 0 0] Check if hit barrier
            (bind (_outhit _outpathpositions _outlasttracedestination _returnvalue) (`GameplayStatics.Blueprint_PredictProjectilePath_ByObjectType` (`local.SpawnPoint`) (* (`local.LDirectionToCast`) (* _output_get_2 (`/Game/Spells/Blueprints/BP_BasicAttacks.BaseSpeed` (`local.LSpawnAttack`)))) true 20.0 (`local.ObjectTypestoScan`) false (`local.LIgnoreCollision`) "None" 2.0 4.0 2.0 (* (`/Game/Spells/Blueprints/BP_BasicAttacks.GravityScale` (`local.LSpawnAttack`)) -981.0)))
            (if (not _returnvalue)
              (break)))
          (:`Is Not Valid`
            (break))))))
  (`/Engine/EditorBlueprintResources/StandardMacros.IsValid` _lspawnattack
    (:`Is Valid`
      (`/Game/Spells/Blueprints/BP_BasicAttacks.CastBaseAttackAI` _lspawnattack (`local.EnemyTarget`) (`local.LDirectionToCast`) (`local.SpeedyFactor`)))))

(fn `DeactivateandDestroySpell`
  (`KismetSystemLibrary.K2_ClearAndInvalidateTimerHandle` (`self.ActivateAttackTimeHandler`))
  (`KismetSystemLibrary.K2_ClearAndInvalidateTimerHandle` (`self.FollowingTargetTimerHandler`))
  (if (not (`|EnumEquality` (`self.CastStatus`) "NewEnumerator2"))
    (set `self.CastStatus` "NewEnumerator4"))
  (`|ExecutionSequence`
    (:`then_0`
      (`/Engine/EditorBlueprintResources/StandardMacros.IsValid` (`self.ActiveSpell`)
        (:`Is Valid`
          ;[0.3711 0.7216 1] Destroy Attacks
          (bind _asbp_basic_attacks (cast `/Game/Spells/Blueprints/BP_BasicAttacks` (`self.ActiveSpell`)))
          (`self.K2_DestroyActor` _asbp_basic_attacks)
          (set `self.ActiveSpell` null))))
    (:`then_1`
      (`/Engine/EditorBlueprintResources/StandardMacros.IsValid` (`self.ShieldActive`)
        (:`Is Valid`
          ;[0.5705 1 0.6356] Destroy shield
          (`self.K2_DestroyActor` (`self.ShieldActive`))
          (set `self.ShieldActive` null))))))

(fn `DeactivateSpell`
  (if (not (`|EnumEquality` (`self.CastStatus`) "NewEnumerator2"))
    (set `self.CastStatus` "NewEnumerator4"))
  (set `self.ActiveSpell` null))

(fn `GetTimeToChargeAttack`
  (returns (Time :type "Float (double-precision)"))
  (locals (MaxWaitingTime :type "Float (double-precision)"))
  (bind _activespell (`self.ActiveSpell`))
  (bind _asbp_basic_attacks (cast `/Game/Spells/Blueprints/BP_BasicAttacks` _activespell)
    (:`then`
      (`/Engine/EditorBlueprintResources/StandardMacros.IsValid` _activespell
        (:`Is Valid`
          (set `local.MaxWaitingTime` (`/Game/Spells/Blueprints/BP_BasicAttacks.TimeToCharge` _asbp_basic_attacks))
          (if (`KismetMathLibrary.RandomBoolWithWeight` 0.6)
            (return (`local.MaxWaitingTime`))
            (else
              (return (`KismetMathLibrary.RandomFloatInRange` (* (`local.MaxWaitingTime`) 0.3) (* (`local.MaxWaitingTime`) 1.5))))))
        (:`Is Not Valid`
          (return 0.1))))
    (:`CastFailed`
      (return 0.1))))

(fn `MovesShieldToDefend`
  (params (TargetToFollow :type "Actor Object Reference"))
  (returns (isFinished :type Boolean))
  (bind _shieldactive (`self.ShieldActive`))
  ;[0.6475 0.8886 1] Check if the projectile is valide and gets its location
  (`/Engine/EditorBlueprintResources/StandardMacros.IsValid` TargetToFollow
    (:`Is Valid`
      ;[0.6157 1 0.7897] Gets shield location
      (`/Engine/EditorBlueprintResources/StandardMacros.IsValid` _shieldactive
        (:`Is Valid`
          ;[0.9919 0.5477 1] Rotates the arm to face the projectile
          (bind _outhit (`KismetSystemLibrary.LineTraceSingle` :`Start` (`SceneComponent.K2_GetComponentLocation` (`StaticMeshActor.StaticMeshComponent` _shieldactive)) :`End` (`self.K2_GetActorLocation` TargetToFollow) :`TraceChannel` "TraceTypeQuery1" :`DrawTime` 1.0))
          (`SceneComponent.K2_SetWorldRotation` (`self.SpringArm`) (`KismetMathLibrary.Conv_VectorToRotator` (`.Normal` (`GameplayStatics.BreakHitResult` _outhit))) false false)
          (return false))
        (:`Is Not Valid`
          _)))
    (:`Is Not Valid`
      _))
  (return true))

(fn `UserConstructionScript`)