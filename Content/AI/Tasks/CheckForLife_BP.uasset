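; Behavior tree task that decides whether an AI enemy should keep casting its attack, based on life checks.
; It reads the pawn's IsCastActive flag; when false, it sets the IsGameOver blackboard key and stops casting.
; Otherwise it clears that flag if the controller's target, another AI or the VR player, is out.
; Failed casts of the pawn or controller log an error without finishing the task.
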(event `self.ReceiveExecute`
  (params (OwnerActor :type "Actor Object Reference"))
  (bind _returnvalue (`AIBlueprintHelperLibrary.GetAIController` OwnerActor))
  ;[0.6672 1 0.217] Check the own AI life, if dead stop casting
  (bind _asaienemy_bp (cast `/Game/AI/AIEnemy_BP` (`Controller.K2_GetPawn` _returnvalue))
    (:`then`
      (if (`/Game/AI/AIEnemy_BP.isCastActive` _asaienemy_bp)
        ;[0.6875 1 1] Check the enemy Life. If enemy is dead stop casting
        (bind _asaienemy_controler (cast `/Game/AI/AIEnemyControler` _returnvalue)
          (:`then`
            (bind _enemy (`/Game/AI/AIEnemyControler.Enemy` _asaienemy_controler))
            (bind _asaienemy_bp_2 (cast `/Game/AI/AIEnemy_BP` _enemy)
              (:`then`
                (if (not (`/Game/AI/AIEnemy_BP.isCastActive` _asaienemy_bp_2))
                  (set `/Game/AI/AIEnemy_BP.isCastActive` false _asaienemy_bp :!label _label)))
              (:`CastFailed`
                ;;[1 0.9315 0.6979] Check for the life for the VR Player
                (bind _asmotion_controller_pawn (cast `/Game/VirtualRealityBP/Blueprints/MotionControllerPawn` _enemy)
                  (:`then`
                    (if (`/Game/VirtualRealityBP/Blueprints/MotionControllerPawn.isGameOver` _asmotion_controller_pawn)
                      (goto _label)
                      (else
                        _)))
                  (:`CastFailed`
                    _))))
            (`self.FinishExecute` true))
          (:`CastFailed`
            (`VisualLoggerKismetLibrary.LogText` "Fail in Cast To AIEnemyControler. Check task CheckForLife" "Error")))
        (else
          (`BTFunctionLibrary.SetBlackboardValueAsBool` (`self.isGameOver`) true)
          ;;[1 0.4886 0.5185] Stop Casting
          (`/Game/AI/AIEnemy_BP.StopAttackCasting` _asaienemy_bp)
          (`self.FinishExecute` true))))
    (:`CastFailed`
      (`VisualLoggerKismetLibrary.LogText` "Fail in Cast To AIEnemy. Check task CheckForLife" "Error"))))