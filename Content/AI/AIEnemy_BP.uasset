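; AI enemy for a VR duel against the motion-controller player, spending regenerating Qi on projectiles and shields, with stats loaded from a data table by difficulty level.
; StartCasting starts timed random-cone attacks that re-roll paths predicted to hit obstacles, or raises a shield.
; Incoming projectiles trigger shields with Gaussian life-based odds, rotated on a timer to face them.
; They may also grow barriers at the nearest free predicted-impact point.
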(event `self.ReceiveBeginPlay`
  (bind _player (`self.Player`))
  (`|ExecutionSequence`
    (:`then_0`
      (`self.SetInitialConditions`))
    (:`then_1`
      ;[1 0.9431 0.4333] Set the locations of each spawn point where the barrier might be casted
      (for (_array_element _array_index) (`SceneComponent.GetChildrenComponents` (`self.LocationToCastBarrier`) false)
        (`KismetArrayLibrary.Array_Set` (`self.SpawnBarrierLocations`) _array_index (`SceneComponent.K2_GetComponentLocation` _array_element) true)
        (`KismetArrayLibrary.Array_Set` (`self.IsBarrierActiveAtThisLocation`) _array_index (not (`KismetSystemLibrary.IsValid` _array_element)) true)))
    (:`then_2`
      ;[1 0.5277 0.9101] Activate spell after x secs
      (set `self.isCastActive` true)
      (if (`KismetSystemLibrary.IsValid` _player)
        (`KismetSystemLibrary.Delay` (`/Game/VirtualRealityBP/Blueprints/MotionControllerPawn.StartFightIn` _player))
        (else
          (`KismetSystemLibrary.Delay` 4.0) ; For test
        ))
      (set `self.AICurrentMode` "NewEnumerator1")
      ;[0.1356 0.08866 0.1274] Set Regeneration Timer
      (`KismetSystemLibrary.K2_SetTimerDelegate` (delegate `/Game/Interfaces/BPI_HasQi.RegenerateQi`) 1.0 true))))

(event `StartComputeAttackTrajectory`
  ;[0.62 0.62 0.62] Shield node
  ;;[0.7021 0.7342 1] This function moves the shield to block the attacks
  (`self.MovesShieldToDefend` (stale `self.DetectIncomingAttack.OnComponentBeginOverlap` _output_get)))

(event `/Game/Interfaces/BPI_reciveQi.ReciveQi`
  (params (Amount :type Integer))
  ;[0.2854 0.2935 1] Recive Qi
  (`self.AddQi` Amount))

(event `/Game/Interfaces/BPI_HasQi.RegenerateQi`
  ;[0.1356 0.08866 0.1274] Set Regeneration Timer
  (`self.RegenerateQiFunction`))

(event `/Game/Interfaces/BPI_HasQi.ConsumeQi`
  (params (Cost :type Integer))
  ;[0.6655 1 0.6641] Consume Qi Event
  (`self.Consume QiFunction` Cost))

(event `/Game/Interfaces/BPI_TakeDamage.OnDamage`
  (params (Damage :type Integer))
  ;[0.4762 0.8485 1] On Damage
  (`|ExecutionSequence`
    (:`then_0`
      ;;[0.5956 1 0.5852] Subtract damage from life
      (set `self.Life` (- (`self.Life`) Damage)))
    (:`then_1`
      ;;[0.6408 1 0.8232] Set Health on Health Bar UI
      (`/Game/WidgetBP/HealthQiBar_BP.SetHealthBarPercent` (`self.WidgetHealthBar`) (`KismetMathLibrary.FClamp` (/ (`KismetMathLibrary.Conv_IntToDouble` (`self.Life`)) (`KismetMathLibrary.Conv_IntToDouble` (`self.BaseLife`)))))
      ;;[0.8409 0.602 1] Check if is Dead
      (if (<= (`self.Life`) 0)
        ;;;[0.145 0.08811 0.07942] Dead
        (`|ExecutionSequence`
          (:`then_0`
            (set `/Game/VirtualRealityBP/Blueprints/MotionControllerPawn.isGameOver` true (`self.Player`)))
          (:`then_1`
            (set `self.isCastActive` false))
          (:`then_2`
            (`PrimitiveComponent.SetSimulatePhysics` (`self.Mesh`) true)))))))

(event `self.DetectIncomingAttack.OnComponentBeginOverlap`
  (params (OverlappedComponent :type "PrimitiveComponent Object Reference") (OtherActor :type "Actor Object Reference") (OtherComp :type "PrimitiveComponent Object Reference") (OtherBodyIndex :type Integer) (bFromSweep :type Boolean) (SweepResult :type "HitResult Structure (by ref)"))
  (bind _asbp_basic_attacks (cast `/Game/Spells/Blueprints/BP_BasicAttacks` OtherActor))
  ;[0.292 1 0.1971] From Sweep. If True means the attack come from outside the volume, otherwise it come from within the volume.
  (if bFromSweep
    ;[0.62 0.62 0.62] Shield node
    (if (`KismetSystemLibrary.IsValid` (`self.ShieldActive`))
      (if (not (`KismetSystemLibrary.K2_IsTimerActiveHandle` (`self.FollowingTargetTimerHandler`)))
        ;;[0.5705 1 0.8995] Sets the target for the shield to follow and starts the move funciton.
        (bind _output_get (set `self.ActiveTargetToFollow` _asbp_basic_attacks :!label _label))
        (bind _returnvalue (`KismetSystemLibrary.K2_SetTimerDelegate` (delegate `StartComputeAttackTrajectory`) (`self.TimeRatio the MoveShield function is called`) true))
        (set `self.FollowingTargetTimerHandler` _returnvalue))
      (else
        ;;[0.6013 1 0.8681] Probability to cast a shield based on the AI life
        (bind _val (`self.ProbabilityOfCastingShield` (`KismetMathLibrary.Conv_IntToDouble` (`self.Life`)) (`self.FractionOfLifeWithHalfProbability`)))
        (if (`KismetMathLibrary.RandomBoolWithWeight` _val)
          (`self.CastShield` (`self.WhatToCastOnShield`))
          (goto _label)
          (else
            _))))
    ;[0.7455 0.7541 0.78] Barrier Defense node
    ;;[0.505 1 0.9301] Logic to trigger the barrier growth. On Attack overleap spawn a barrier
    (bind _val_2 (`/Game/FunctionLibrary/MyFunctions.ExponentialFunction` 0.8 0.47 (`KismetMathLibrary.Conv_IntToDouble` (`self.NumberOfActiveBarrier`))))
    (bind _staticmeshcomponent (`StaticMeshActor.StaticMeshComponent` _asbp_basic_attacks))
    ;;[1 0.4965 0.7016] Gets the position and velocity to compute where and the probability of a barrier been casted
    (bind (_indexofthenearbox _probabilytocastatthislocation) (`self.GetsTheNearSpawnLocationFromAPoint` (`SceneComponent.K2_GetComponentLocation` _staticmeshcomponent) (`SceneComponent.GetComponentVelocity` _staticmeshcomponent)))
    (if (`KismetMathLibrary.RandomBoolWithWeight` (* _val_2 _probabilytocastatthislocation))
      (if (not (`self.isCastingBarrier`))
        (bind _returnvalue_2 (`KismetSystemLibrary.K2_SetTimerDelegate` (delegate `GrowBarrier`) 0.05 true))
        (set `self.GrowBarrierTimerHandle` _returnvalue_2)
        (`KismetSystemLibrary.Delay` (`KismetMathLibrary.RandomFloatInRange` 0.3 1.0))
        (`self.StopGrowingBarrier`)))))

(event `GrowBarrier`
  ;[0.7455 0.7541 0.78] Barrier Defense node
  ;;[0.5998 1 0.6576] Start Grow the Barrier
  (`self.CastTheBarrier` (`self.WhatToCastOnLeftBarrrier`) true (stale `self.DetectIncomingAttack.OnComponentBeginOverlap` _indexofthenearbox)))

(event `StopGrowingBarrier`
  ;[0.7455 0.7541 0.78] Barrier Defense node
  ;;[0.6892 0.7951 1] Stop Growing the Barrier
  (if (`KismetSystemLibrary.K2_IsTimerActiveHandle` (`self.GrowBarrierTimerHandle`))
    (`self.CastTheBarrier` (`self.WhatToCastOnLeftBarrrier`))
    (`KismetSystemLibrary.K2_ClearAndInvalidateTimerHandle` (`self.GrowBarrierTimerHandle`))))

(event `Attack`
  ;[0.535 0.535 0.535] Basic Attack node
  (bind _return (`self.ShouldAttackWithBothHands` 0.5))
  (if _return
    ;;[1 0.9431 0.4333] Cast Right/Left Attack
    (`self.CastBaseAttack` (`self.WhatClassToSpawn`) (`self.RightAttackBox`))
    (`KismetSystemLibrary.Delay` (`KismetMathLibrary.RandomFloatInRange` 0.2 0.5))
    ;;[1 0.9431 0.4333] Cast Left Attack
    (`self.CastBaseAttack` (`self.WhatClassToSpawn`) (`self.LeftAttackBox`) :!label _label_2)
    (elif (`KismetMathLibrary.RandomBoolWithWeight` 0.5)
      (goto _label_2)
      (else
        ;;[1 0.9431 0.4333] Cast Right Attack
        (`self.CastBaseAttack` (`self.WhatClassToSpawn`) (`self.RightAttackBox`))))))

(event `self.LocationToCastBarrier.OnComponentBeginOverlap`
  (params (OverlappedComponent :type "PrimitiveComponent Object Reference") (OtherActor :type "Actor Object Reference") (OtherComp :type "PrimitiveComponent Object Reference") (OtherBodyIndex :type Integer) (bFromSweep :type Boolean) (SweepResult :type "HitResult Structure (by ref)"))
  ;[1 0.9725 0.7771] Update the number of barrier casted
  (bind _asbp_barrier (cast `/Game/Spells/Blueprints/BP_Barrier` OtherActor))
  (set `self.NumberOfActiveBarrier` (+ (`self.NumberOfActiveBarrier`) 1))
  (bind _output_get (set `/Game/Spells/Blueprints/BP_Barrier.CastedAtIndexLocation` (stale `self.DetectIncomingAttack.OnComponentBeginOverlap` _indexofthenearbox) _asbp_barrier)) ; Storege the index's position on each  barrier casted
  (`KismetArrayLibrary.Array_Set` (`self.IsBarrierActiveAtThisLocation`) _output_get true) ; Set as true for this location
)

(event `StartCasting`
  ;[0.7244 0.6508 1] Start Casting
  (switch `/Game/AI/EAIModes` (`self.AICurrentMode`)
    (:`NewEnumerator1`
      ;[0.535 0.535 0.535] Basic Attack node
      (if (not (`KismetSystemLibrary.K2_IsTimerActiveHandle` (`self.AttackTimerHandler`)))
        (bind _returnvalue (`KismetSystemLibrary.K2_SetTimerDelegate` (delegate `Attack`) (`self.Firerate`) true))
        (set `self.AttackTimerHandler` _returnvalue)))
    (:`NewEnumerator2`
      ;[0.4655 0.7054 1] Cast the shield if it doesn't exist
      (if (not (`KismetSystemLibrary.IsValid` (`self.ShieldActive`)))
        (`self.CastShield` (`self.WhatToCastOnShield`))))))

(event `self.LocationToCastBarrier.OnComponentEndOverlap`
  (params (OverlappedComponent :type "PrimitiveComponent Object Reference") (OtherActor :type "Actor Object Reference") (OtherComp :type "PrimitiveComponent Object Reference") (OtherBodyIndex :type Integer))
  ;[1 0.9725 0.7771] Update the number of barrier casted
  (bind _asbp_barrier (cast `/Game/Spells/Blueprints/BP_Barrier` OtherActor))
  (set `self.NumberOfActiveBarrier` (- (`self.NumberOfActiveBarrier`) 1))
  (`KismetArrayLibrary.Array_Set` (`self.IsBarrierActiveAtThisLocation`) (`/Game/Spells/Blueprints/BP_Barrier.CastedAtIndexLocation` _asbp_barrier) false) ; Set to false when the barrier is destroed
)

(event `StopAttackCasting`
  (bind _attacktimerhandler (`self.AttackTimerHandler`))
  ;[0.7625 0.7292 1] Stop Casting Attack
  (if (`KismetSystemLibrary.K2_IsTimerActiveHandle` _attacktimerhandler)
    (`KismetSystemLibrary.K2_ClearAndInvalidateTimerHandle` _attacktimerhandler)))

(event `self.ReceiveTick`
  (params (DeltaSeconds :type "Float (single-precision)"))
  ;[1 0.1666 0.1765] Old
)

(fn `AddQi`
  (params (Cost :type Integer))
  (if (< (`self.Qi`) (`self.BaseQi`))
    (set `self.Qi` (+ (`self.Qi`) Cost))
    (`self.UpdateQiBar`)))

(fn `CastBaseAttack`
  (params (SpawnAttackOfClass :type "Actor Class Reference") (AttackFrom :type "BoxComponent Object Reference"))
  (locals (LocalZAxis :type "Float (double-precision)" :default 0.0) (LocalDirectionToCast :type "Vector Structure" :default (0.0 0.0 0.0)) (SpawnPoint :type "Vector Structure") (TraceLineLength :type "Float (double-precision)" :default 450.0) (SpawnAttack :type "Actor Object Reference") (RandomFloatInRange :type "Float (double-precision)"))
  (bind (_origin _boxextent) (`KismetSystemLibrary.GetComponentBounds` AttackFrom))
  ;[0.5955 1 0.9198] Cast a Base attack
  (bind _output_get (set `local.SpawnPoint` (`KismetMathLibrary.RandomPointInBoundingBox` _origin _boxextent)))
  (bind _returnvalue (`|SpawnActorFromClass` SpawnAttackOfClass (`KismetMathLibrary.MakeTransform` _output_get (struct) (1.0 1.0 1.0)) "AlwaysSpawn" "OverrideRootScale" self))
  (bind _output_get_2 (set `local.SpawnAttack` _returnvalue))
  (bind _qicost (`/Game/Spells/Blueprints/BP_BasicAttacks.QiCost` (cast `/Game/Spells/Blueprints/BP_BasicAttacks` _output_get_2 :!pure true)))
  ;;[0.2287 0.2363 0.43] Checking for QI
  (bind _return (`self.HasEnoughQi` _qicost))
  (if _return
    (`self.ConsumeQi` _qicost)
    (bind _output_get_3 (set `local.LocalDirectionToCast` (`KismetMathLibrary.RandomUnitVectorInConeWithYawAndPitch` (+ (`SceneComponent.GetForwardVector` (`self.ArrowComponent`)) (`KismetMathLibrary.MakeVector` 0.0 0.0 (`local.LocalZAxis`))) 90.0 80.0) :!label _label))
    ;;[0.06647 0.0886 0.1746] Check if vector is antiparallel
    (`/Game/FunctionLibrary/MyMacroLibrary.VectorsAreOpposite?` (`KismetMathLibrary.MakeVector` (.x _output_get_3) (.y _output_get_3)) (`SceneComponent.GetForwardVector` (`self.ArrowComponent`))
      (:`IsOpposite`
        (goto _label))
      (:`NotOpposite`
        ;;[0 0 0] Calculation of velocity
        (bind _output_get_4 (set `local.RandomFloatInRange` (`KismetMathLibrary.RandomFloatInRange` 0.4 1.0)))
        ;;[0 0 0] Check if hit barrier
        (bind (_outhit _outpathpositions _outlasttracedestination _returnvalue_2) (`GameplayStatics.Blueprint_PredictProjectilePath_ByObjectType` (`local.SpawnPoint`) (* (`local.LocalDirectionToCast`) (* _output_get_4 (`/Game/Spells/Blueprints/BP_BasicAttacks.BaseSpeed` (cast `/Game/Spells/Blueprints/BP_BasicAttacks` (`local.SpawnAttack`) :!pure true)))) true 10.0 (`self.ObjectTypestoScan`) false (`|MakeArray` self (`local.SpawnAttack`) :!type "Actor Object Reference") "None" 2.0 1.0 0.5 -981.0))
        (if _returnvalue_2
          (goto _label)
          (else
            (`/Game/Spells/Blueprints/BP_BasicAttacks.CastBaseAttackAI` (cast `/Game/Spells/Blueprints/BP_BasicAttacks` (`local.SpawnAttack`) :!pure true) (`self.Target`) (`local.LocalDirectionToCast`) (`local.RandomFloatInRange`))))))
    (else
      (`self.K2_DestroyActor` (`local.SpawnAttack`)))))

(fn `CastShield`
  (params (ShieldClassToSpawn :type "Actor Class Reference"))
  (bind _returnvalue (`|SpawnActorFromClass` ShieldClassToSpawn (`KismetMathLibrary.MakeTransform` (0.0 0.0 0.0) (struct :`Pitch` 90.0)) "AlwaysSpawn" "OverrideRootScale" self))
  (bind _asbp_shield (cast `/Game/Spells/Blueprints/BP_Shield` _returnvalue :!pure true))
  (bind _output_get (set `self.ShieldActive` _asbp_shield))
  (bind _qicost (`/Game/Spells/Blueprints/BP_Shield.QiCost` _asbp_shield))
  (bind _return (`self.HasEnoughQi` _qicost))
  (if _return
    (`self.ConsumeQi` _qicost)
    (`SceneComponent.K2_AttachToComponent` (`StaticMeshActor.StaticMeshComponent` _output_get) (`self.LeftArm`) "None" "KeepRelative" "KeepRelative" "KeepRelative" false)
    (else
      (set `self.ShieldActive` null)
      (`self.K2_DestroyActor` _returnvalue))))

(fn `CastTheBarrier`
  (params (SpawnBarrierOfClass :type "Actor Class Reference") (isGrowing :type Boolean) (IndexOftheBarrierLocation :type Integer))
  (bind _defensebarrier (`self.DefenseBarrier`))
  (bind (_item_x _item_y) (`KismetMathLibrary.BreakVector` (`KismetArrayLibrary.Array_Get` (`self.SpawnBarrierLocations`) IndexOftheBarrierLocation)))
  (bind (_returnvalue_x _returnvalue_y) (`KismetMathLibrary.BreakVector` (`SceneComponent.K2_GetComponentLocation` (`self.ReferencePointToBarrierRotation`))))
  ;[1 1 1] Cast Barrier for the Left Hand
  ;;[0.6457 1 0.9901] Check  if button is pressed
  (if isGrowing
    ;;[0.6652 1 0.9701] If is the first time spawn, otherwise grow the nbarrier
    (if (`self.isCastingBarrier`)
      ;;[1 0.7759 0.6537] Grow the barrier at constant speedy
      (bind _asbp_barrier (cast `/Game/Spells/Blueprints/BP_Barrier` (`self.DefenseBarrier`)))
      (`/Game/Spells/Blueprints/BP_Barrier.GrowBarrierAtZDirection` _asbp_barrier 70.0)
      (else
        ;;[0.662 1 0.6828] Spawn the barrier
        (set `self.isCastingBarrier` true)
        (bind _returnvalue (`|SpawnActorFromClass` SpawnBarrierOfClass (`KismetMathLibrary.MakeTransform` (`KismetMathLibrary.MakeVector` _item_x _item_y 0.0) (`KismetMathLibrary.FindLookAtRotation` (`KismetMathLibrary.MakeVector` _returnvalue_x _returnvalue_y) (`KismetMathLibrary.MakeVector` _item_x _item_y))) "Undefined" "OverrideRootScale" self))
        (set `self.DefenseBarrier` _returnvalue)))
    (else
      (set `self.isCastingBarrier` false)
      ;;[0.4597 1 0.4957] Stops the grow sound
      (`/Engine/EditorBlueprintResources/StandardMacros.IsValid` _defensebarrier
        (:`Is Valid`
          (bind _asbp_barrier_2 (cast `/Game/Spells/Blueprints/BP_Barrier` _defensebarrier))
          (`|ExecutionSequence`
            (:`then_0`
              (`AudioComponent.Stop` (`/Game/Spells/Blueprints/BP_Barrier.GrowSound` _asbp_barrier_2)))
            (:`then_1`
              ;;[0.5828 0.9801 1] Set Barrier to be destroy and set DefenseBarrierLeft to none
              (`/Game/Spells/Blueprints/BP_Barrier.SelfDestroyAfterTimeLife` _asbp_barrier_2)
              (set `self.DefenseBarrier` null))))
        (:`Is Not Valid`
          (set `self.DefenseBarrier` null))))))

(fn `Consume QiFunction`
  (params (Cost :type Integer))
  (if (>= (`self.Qi`) 0)
    (set `self.Qi` (- (`self.Qi`) Cost))
    (`self.UpdateQiBar`)))

(fn `GetsTheNearSpawnLocationFromAPoint`
  (params (Point :type "Vector Structure") (velocity :type "Vector Structure"))
  (returns (IndexOftheNearBox :type Integer) (ProbabilyToCastAtThisLocation :type "Float (double-precision)"))
  (locals (Distance :type "Float (double-precision)" :default 999999995904.0) (IndexOftheNearBoxLocalVar :type Integer))
  (if (> (`KismetMathLibrary.VSize` (- Point (`SceneComponent.K2_GetComponentLocation` (`self.Mesh`)))) 300.0)
    (for (_array_element _array_index) (`self.SpawnBarrierLocations`)
      (bind _returnvalue (`KismetMathLibrary.VSize` (- _array_element (+ Point (* (`KismetMathLibrary.Normal` velocity) 600.0)))))
      ;[1 0.6314 0.9219] Loop. Finds the closer location from the projectile to cast the barrier
      (if (< _returnvalue (`local.Distance`))
        (set `local.Distance` _returnvalue)
        (set `local.IndexOftheNearBoxLocalVar` _array_index)))
    (if (`KismetArrayLibrary.Array_Get` (`self.IsBarrierActiveAtThisLocation`) (`local.IndexOftheNearBoxLocalVar`))
      ;[1 0.3224 0.3124] Returns null probability of casting a barrier
      (return (`local.IndexOftheNearBoxLocalVar`) 0.0)
      (else
        ;[0.4467 1 0.4084] Return the index of the closest position to cast the barrier.
        (return (`local.IndexOftheNearBoxLocalVar`) 1.0)))
    (else
      ;[1 0.3224 0.3124] Returns null probability of casting a barrier
      (return (`local.IndexOftheNearBoxLocalVar`) 0.0))))

(fn `GiveQi`
  (params (InitialAmount :type Integer))
  (returns (ReturnAmount :type Integer) (GiveQiToOwner :type Boolean))
  (return (`KismetMathLibrary.FTrunc` (* InitialAmount (`self.QiMultiplier`))) false))

(fn `HasEnoughQi`
  (params (Cost :type Integer))
  (returns (Return :type Boolean))
  (if (>= (`self.Qi`) Cost)
    (return true)
    (else
      (return false))))

(fn `MovesShieldToDefend`
  (params (TargetToFollow :type "Actor Object Reference"))
  (bind _alphaforrotation (`self.AlphaForRotation`))
  (bind _leftarm (`self.LeftArm`))
  (bind _shieldactive (`self.ShieldActive`))
  ;[0.6475 0.8886 1] Check if the projectile is valide and gets its location
  (if (`KismetSystemLibrary.IsValid` TargetToFollow)
    ;[0.6157 1 0.7897] Gets shield location
    (`/Engine/EditorBlueprintResources/StandardMacros.IsValid` _shieldactive
      (:`Is Valid`
        ;[0.9919 0.5477 1] Rotates the arm to face the projectile
        (bind _outhit (`KismetSystemLibrary.LineTraceSingle` :`Start` (`self.K2_GetActorLocation` TargetToFollow) :`End` (`SceneComponent.K2_GetComponentLocation` (`StaticMeshActor.StaticMeshComponent` _shieldactive)) :`TraceChannel` "TraceTypeQuery1" :`DrawTime` 1.0))
        (`SceneComponent.K2_SetWorldRotation` (`self.LeftArm`) (`KismetMathLibrary.Conv_VectorToRotator` (* (`.Normal` (`GameplayStatics.BreakHitResult` _outhit)) -1.0)) false false)))
    (else
      ;[1 0.6832 0.8279] Once the target is not avaible anymore start to rotate the shiled back to its original position.
      (`SceneComponent.K2_SetRelativeRotation` _leftarm (`KismetMathLibrary.RLerp` (`SceneComponent.RelativeRotation` _leftarm) (`self.ShieldDefensePosition`) (`self.AlphaForRotation`) true) false false)
      (if (>= _alphaforrotation 1.0)
        (set `self.AlphaForRotation` 0.0)
        ;[1 0.6063 0.4135] Clear Timer when projectile is not valide. This makes the function to stop been called
        (`KismetSystemLibrary.K2_ClearAndInvalidateTimerHandle` (`self.FollowingTargetTimerHandler`))
        (else
          (set `self.AlphaForRotation` (`KismetMathLibrary.FClamp` (+ _alphaforrotation (/ (`self.TimeRatio the MoveShield function is called`) (`self.MaximumTimeForReactionInSec`))))))))))

(fn `ProbabilityOfCastingShield`
  (params (Life :type "Float (double-precision)") (PercentageOfLifeWithHalfProbability :type "Float (double-precision)"))
  (returns (val :type "Float (double-precision)"))
  (bind _val (`/Game/FunctionLibrary/MyFunctions.Gaussian` 1.0 (/ (* PercentageOfLifeWithHalfProbability (`KismetMathLibrary.Conv_IntToDouble` (`self.BaseLife`))) (`KismetMathLibrary.Sqrt` (* (`KismetMathLibrary.Loge` 0.5) -2.0))) 0.0 Life))
  (return _val))

(fn `RegenerateQiFunction`
  (if (< (`self.Qi`) (`self.BaseQi`))
    (set `self.Qi` (+ (`self.Qi`) (`self.QiRegeneration`)))
    (`self.UpdateQiBar`)))

(fn `SetInitialConditions`
  (`|ExecutionSequence`
    (:`then_0`
      ;[0.365 1 0.566] Sets Life
      (set `self.Life` (`self.BaseLife`))
      ;[0.3411 0.4424 1] Set Initial Qi
      (set `self.Qi` 0))
    (:`then_1`
      ;[0.4333 0.6597 1] Sets Player reference
      (bind _asmotion_controller_pawn (cast `/Game/VirtualRealityBP/Blueprints/MotionControllerPawn` (`GameplayStatics.GetPlayerPawn` 0)))
      (set `self.Player` _asmotion_controller_pawn))
    (:`then_2`
      ;[0.6596 1 0.5198] Sets the reference for the Health bar
      (bind _ashealth_qi_bar_bp (cast `/Game/WidgetBP/HealthQiBar_BP` (`WidgetComponent.GetUserWidgetObject` (`self.HealthBarWidget`)))
        (:`then`
          (set `self.WidgetHealthBar` _ashealth_qi_bar_bp))
        (:`CastFailed`
          (`KismetSystemLibrary.PrintText` "Fail to Cast to Player Health bar."))))))

(fn `SetVariablesFromDataBase`
  (params (RowName :type Name))
  (bind _returnvalue (`|GetDataTableRow` "/Game/AI/Data/AIDataStructure.AIDataStructure" RowName)
    (:`then`
      (`|ExecutionSequence`
        (:`then_0`
          (bind (_life _firerate) (break `/Game/AI/Data/AILevelStructure` _returnvalue))
          (set `self.BaseLife` _life))
        (:`then_1`
          (set `self.Firerate` _firerate))))
    (:`RowNotFound`
      (`VisualLoggerKismetLibrary.LogText` "Warning: Row not found at AI SetVariablesFromDataBase" "Error"))))

(fn `ShouldAttackWithBothHands`
  (params (Probability :type "Float (double-precision)"))
  (returns (Return :type Boolean))
  (return (`KismetMathLibrary.RandomBoolWithWeight` Probability)))

(fn `UserConstructionScript`
  (bind _mesh (`self.Mesh`))
  (`|ExecutionSequence`
    (:`then_0`
      (bind _returnvalue (`PrimitiveComponent.CreateDynamicMaterialInstance` _mesh 0 (`PrimitiveComponent.GetMaterial` _mesh 0)))
      (set `self.BodyMaterial` _returnvalue))
    (:`then_1`
      ;[1 0.9283 0.1475] Sets the AI DataBase.
      (`self.SetVariablesFromDataBase` (`KismetStringLibrary.Conv_StringToName` (`|GetEnumeratorNameAsString` (`self.AILevel`)))))))