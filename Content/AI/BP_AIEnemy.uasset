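; Elemental spellcaster enemy that duels the motion-controller player, with stats, elements and blocked abilities loaded from a data table by AI level.
; Two spawned hand actors cast attacks and shields, while the body tracks health and regenerating Qi.
; Incoming attacks trigger random defenses: shields weighted by a Gaussian of life, growing barriers by barrier count at the point nearest the projectile's extrapolated position.
; Attack launches sample random arcs using path prediction to avoid obstacles.
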(event `self.ReceiveBeginPlay`
  (bind _player (`self.Player`))
  (`|ExecutionSequence`
    (:`then_0`
      ;[0.2923 1 0.4974] Sets parameters from data table
      (`self.SetVariablesFromDataBase` (`KismetStringLibrary.Conv_StringToName` (`|GetEnumeratorNameAsString` (`self.AILevel`))))
      (`self.SetInitialConditions`))
    (:`then_1`
      ;[1 0.9431 0.4333] Set the locations of each spawn point where the barrier might be casted
      (for (_array_element _array_index) (`SceneComponent.GetChildrenComponents` (`self.LocationToCastBarrier`) false)
        (`KismetArrayLibrary.Array_Set` (`self.SpawnBarrierLocations`) _array_index (`SceneComponent.K2_GetComponentLocation` _array_element) true)
        (`KismetArrayLibrary.Array_Set` (`self.IsBarrierActiveAtThisLocation`) _array_index (not (`KismetSystemLibrary.IsValid` _array_element)) true)))
    (:`then_2`
      ;[1 1 1] Spawn AI hands
      (bind _returnvalue (`|SpawnActorFromClass` "/Game/AI/BP_AIHand.BP_AIHand_C" (`KismetMathLibrary.MakeTransform` (0.0 0.0 0.0)) "Undefined" "OverrideRootScale" null "Left"))
      (bind _output_get (set `self.LeftHand` _returnvalue))
      (`self.K2_AttachToComponent` _output_get (`self.Mesh`) "LeftArm" "KeepRelative" "KeepRelative" "KeepRelative" false)
      (bind _returnvalue_2 (`|SpawnActorFromClass` "/Game/AI/BP_AIHand.BP_AIHand_C" (`KismetMathLibrary.MakeTransform` (0.0 0.0 0.0) (struct :`Pitch` 180.0)) "Undefined" "OverrideRootScale" null "Right"))
      (bind _output_get_2 (set `self.RightHand` _returnvalue_2))
      (`self.K2_AttachToComponent` _output_get_2 (`self.Mesh`) "RightArm" "KeepRelative" "KeepRelative" "KeepRelative" false))
    (:`then_3`
      ;[1 0.5277 0.9101] Activate spell after x secs
      (set `self.isCastActive` true)
      (if (`KismetSystemLibrary.IsValid` _player)
        (`KismetSystemLibrary.Delay` (`/Game/VirtualRealityBP/Blueprints/MotionControllerPawn.StartFightIn` _player))
        (else
          (`KismetSystemLibrary.Delay` 4.0) ; For test
        ))
      (set `/Game/AI/BP_AIHand.CastStatus` "NewEnumerator4" (`self.LeftHand`))
      (set `/Game/AI/BP_AIHand.CastStatus` "NewEnumerator4" (`self.RightHand`))
      ;[0.1356 0.08866 0.1274] Set Regeneration Timer
      (`KismetSystemLibrary.K2_SetTimerDelegate` (delegate `/Game/Interfaces/BPI_HasQi.RegenerateQi`) 1.0 true))))

(event `CastShieldLeft`
  (if (not (`self.BlockLeftShield`))
    (`/Game/AI/BP_AIHand.ActivateShield` (`self.LeftHand`) (`self.WhatToCastOnShieldLeft`) (`self.PossibleAttack`))))

(event `CastShieldRight`
  (if (not (`self.BlockRightShield`))
    (`/Game/AI/BP_AIHand.ActivateShield` (`self.RightHand`) (`self.WhatToCastOnShieldRight`) (`self.PossibleAttack`))))

(event `/Game/Interfaces/BPI_HasQi.RegenerateQi`
  ;[0.1356 0.08866 0.1274] Set Regeneration Timer
  (`self.RegenerateQiFunction`))

(event `/Game/Interfaces/BPI_reciveQi.ReciveQi`
  (params (Amount :type Integer))
  ;[0.2854 0.2935 1] Recive Qi
  (`self.AddQi` Amount))

(event `/Game/Interfaces/BPI_HasQi.ConsumeQi`
  (params (Cost :type Integer))
  ;[0.6655 1 0.6641] Consume Qi Event
  (`self.Consume QiFunction` Cost))

(event `/Game/Interfaces/BPI_TakeDamage.OnDamage`
  (params (Instigator :type "Actor Object Reference") (Damage :type Integer))
  ;[0.4762 0.8485 1] On Damage
  (`|ExecutionSequence`
    (:`then_0`
      ;;[0.5956 1 0.5852] Subtract damage from life
      (set `self.Life` (- (`self.Life`) Damage)))
    (:`then_1`
      ;;[0.6408 1 0.8232] Set Health on Health Bar UI
      (`/Game/WidgetBP/HealthQiBar_BP.SetHealthBarPercent` (`self.WidgetHealthBar`) (`KismetMathLibrary.FClamp` (/ (`KismetMathLibrary.Conv_IntToDouble` (`self.Life`)) (`KismetMathLibrary.Conv_IntToDouble` (`self.BaseLife`)))))
      ;;[0.8409 0.602 1] Check if is Dead
      (if (<= (`self.Life`) 0)
        ;;;[0.145 0.08811 0.07942] Dead
        (`|ExecutionSequence`
          (:`then_0`
            (set `/Game/VirtualRealityBP/Blueprints/MotionControllerPawn.isGameOver` true (`self.Player`)))
          (:`then_1`
            (set `self.isCastActive` false))
          (:`then_2`
            (`PrimitiveComponent.SetSimulatePhysics` (`self.Mesh`) true)))))))

(event `CastBarrier`
  (bind _possibleattack (`self.PossibleAttack`))
  (if (not (`self.BlockBarrier`))
    ;[0.7455 0.7541 0.78] Barrier Defense node
    ;;[0.505 1 0.9301] Logic to trigger the barrier growth. On Attack overleap spawn a barrier
    (bind _val (`/Game/FunctionLibrary/MyFunctions.ExponentialFunction` 0.8 0.47 (`KismetMathLibrary.Conv_IntToDouble` (`self.CurrentNumberOfBarries`))))
    ;;[1 0.4965 0.7016] Gets the position and velocity to compute where and the probability of a barrier been casted
    (bind (_indexofthenearbox _probabilytocastatthislocation) (`self.GetsTheNearSpawnLocationFromAPoint` (`self.K2_GetActorLocation` _possibleattack) (`self.GetVelocity` _possibleattack)))
    (if (`KismetMathLibrary.RandomBoolWithWeight` (* _val _probabilytocastatthislocation))
      (if (not (`self.isCastingBarrier`))
        (bind _returnvalue (`KismetSystemLibrary.K2_SetTimerDelegate` (delegate `GrowBarrier`) 0.05 true))
        (set `self.GrowBarrierTimerHandle` _returnvalue)
        (`KismetSystemLibrary.Delay` (`KismetMathLibrary.RandomFloatInRange` 0.3 1.0))
        (`self.StopGrowingBarrier`)))))

(event `self.DetectIncomingAttack.OnComponentBeginOverlap`
  (params (OverlappedComponent :type "PrimitiveComponent Object Reference") (OtherActor :type "Actor Object Reference") (OtherComp :type "PrimitiveComponent Object Reference") (OtherBodyIndex :type Integer) (bFromSweep :type Boolean) (SweepResult :type "HitResult Structure (by ref)"))
  (bind _possibleattack (`self.PossibleAttack`))
  (bind _asbp_basic_attacks (cast `/Game/Spells/Blueprints/BP_BasicAttacks` OtherActor)
    (:`then`
      (set `self.PossibleAttack` _asbp_basic_attacks))
    (:`CastFailed`
      (bind _asbp_advanced_attacks (cast `/Game/AdvanceAttacks/BluePrints/BP_AdvancedAttacks` OtherActor))
      (set `self.PossibleAttack` _asbp_advanced_attacks)))
  ;[0.292 1 0.1971] From Sweep. If True means the attack come from outside the volume, otherwise it come from within the volume.
  (if bFromSweep
    (`|ExecutionSequence` :!label _label
      (:`then_0`
        ;[0.62 0.62 0.62] Shield node
        ;;[0.6013 1 0.8681] Probability to cast a shield based on the AI life
        (bind _val (`self.ProbabilityOfCastingShield` (`KismetMathLibrary.Conv_IntToDouble` (`self.Life`)) (`self.FractionOfLifeWithHalfProbability`)))
        (if (`KismetMathLibrary.RandomBoolWithWeight` _val)
          ;;;[0.278 0.4444 1] Add later a better left/right shield logic
          (`self.ShiledFrom`
            (:`Left`
              (`self.CastShieldLeft`))
            (:`Right`
              (`self.CastShieldRight`))
            (:`Chose`
              (if (`KismetMathLibrary.RandomBoolWithWeight` 0.5)
                (`self.CastShieldLeft`)
                (else
                  (`self.CastShieldRight`)))))))
      (:`then_1`
        ;[0.3664 0.5107 1] Probality of casting barriers
        (if (`KismetMathLibrary.RandomBoolWithWeight` (`self.ProbabilityToGrowBarrier`))
          (`self.CastBarrier`))))
    (else
      ;[1 0.3694 0.1989] Fix for defend air attack. I have no idea why for air this is inverted.
      (cast `/Game/AdvanceAttacks/BluePrints/BP_AirAttackTailProjectile` _possibleattack)
      (`/Engine/EditorBlueprintResources/StandardMacros.IsValid` _possibleattack
        (:`Is Valid`
          (if (`KismetMathLibrary.RandomBoolWithWeight` 0.1)
            (goto _label)))))))

(event `GrowBarrier`
  ;[0.7455 0.7541 0.78] Barrier Defense node
  ;;[0.5998 1 0.6576] Start Grow the Barrier
  (`self.CastTheBarrier` (`self.WhatToCastOnLeftBarrrier`) true (stale `CastBarrier` _indexofthenearbox)))

(event `StopGrowingBarrier`
  ;[0.7455 0.7541 0.78] Barrier Defense node
  ;;[0.6892 0.7951 1] Stop Growing the Barrier
  (if (`KismetSystemLibrary.K2_IsTimerActiveHandle` (`self.GrowBarrierTimerHandle`))
    (`self.CastTheBarrier` (`self.WhatToCastOnLeftBarrrier`))
    (`KismetSystemLibrary.K2_ClearAndInvalidateTimerHandle` (`self.GrowBarrierTimerHandle`))))

(event `StartBasicAttackRight`
  ;[0.1874 1 0.2705] Initialte BasicAttacks
  (if (not (`self.BlockRightAttack`))
    (`/Game/AI/BP_AIHand.StartBasicAttack` (`self.RightHand`) (`self.WhatBasicAttackToSpawnRight`))))

(event `self.LocationToCastBarrier.OnComponentBeginOverlap`
  (params (OverlappedComponent :type "PrimitiveComponent Object Reference") (OtherActor :type "Actor Object Reference") (OtherComp :type "PrimitiveComponent Object Reference") (OtherBodyIndex :type Integer) (bFromSweep :type Boolean) (SweepResult :type "HitResult Structure (by ref)"))
  ;[1 0.9725 0.7771] Storege where the barrier was cast
  (bind _asbp_barrier (cast `/Game/Spells/Blueprints/BP_Barrier` OtherActor))
  (bind _output_get (set `/Game/Spells/Blueprints/BP_Barrier.CastedAtIndexLocation` (stale `CastBarrier` _indexofthenearbox) _asbp_barrier)) ; Storege the index's position on each  barrier casted
  (`KismetArrayLibrary.Array_Set` (`self.IsBarrierActiveAtThisLocation`) _output_get true) ; Set as true for this location
)

(event `self.LocationToCastBarrier.OnComponentEndOverlap`
  (params (OverlappedComponent :type "PrimitiveComponent Object Reference") (OtherActor :type "Actor Object Reference") (OtherComp :type "PrimitiveComponent Object Reference") (OtherBodyIndex :type Integer))
  ;[1 0.9725 0.7771] Storege where the barrier was cast
  (bind _asbp_barrier (cast `/Game/Spells/Blueprints/BP_Barrier` OtherActor))
  (`KismetArrayLibrary.Array_Set` (`self.IsBarrierActiveAtThisLocation`) (`/Game/Spells/Blueprints/BP_Barrier.CastedAtIndexLocation` _asbp_barrier)) ; Set to false when the barrier is destroed
)

(event `StartBasicAttackLeft`
  ;[0.1874 1 0.2705] Initialte BasicAttacks
  (if (not (`self.BlockLeftAttack`))
    (`/Game/AI/BP_AIHand.StartBasicAttack` (`self.LeftHand`) (`self.WhatBasicAttackToSpawnLeft`))))

(event `/Game/Interfaces/BPI_SpellRules.AddBarrier`
  ;[0.3105 1 0.6903] Add and Remove number of castted Barriers
  (`/Engine/EditorBlueprintResources/StandardMacros.IncrementInt` (`self.CurrentNumberOfBarries`)))

(event `/Game/Interfaces/BPI_SpellRules.RemoveBarrier`
  ;[0.3105 1 0.6903] Add and Remove number of castted Barriers
  (if (> (`self.CurrentNumberOfBarries`) 0)
    (`/Engine/EditorBlueprintResources/StandardMacros.DecrementInt` (`self.CurrentNumberOfBarries`))))

(event `StopRightAttack`
  (bind _righthand (`self.RightHand`))
  (bind _chargeattacktimerhandler (`/Game/AI/BP_AIHand.ChargeAttackTimerHandler` _righthand))
  ;[1 1 1] Stop Basic Attacks
  ;;[0.7625 0.7292 1] Stop Casting Attack Right
  (`/Game/AI/BP_AIHand.DeactivateandDestroySpell` _righthand)
  (`/Game/FunctionLibrary/MyMacroLibrary.IsTimeHandlerActive` _chargeattacktimerhandler
    (:`True`
      (`KismetSystemLibrary.K2_ClearAndInvalidateTimerHandle` _chargeattacktimerhandler))))

(event `StopLeftAttack`
  (bind _lefthand (`self.LeftHand`))
  (bind _chargeattacktimerhandler (`/Game/AI/BP_AIHand.ChargeAttackTimerHandler` _lefthand))
  ;[1 1 1] Stop Basic Attacks
  ;;[0.7625 0.7292 1] Stop Casting Attack Left
  (`/Game/AI/BP_AIHand.DeactivateandDestroySpell` _lefthand)
  (`/Game/FunctionLibrary/MyMacroLibrary.IsTimeHandlerActive` _chargeattacktimerhandler
    (:`True`
      (`KismetSystemLibrary.K2_ClearAndInvalidateTimerHandle` _chargeattacktimerhandler))))

(event `StopAttackBothHands`
  ;[1 1 1] Stop Basic Attacks
  (`|ExecutionSequence`
    (:`then_0`
      (`self.StopRightAttack`))
    (:`then_1`
      (`self.StopLeftAttack`))))

(fn `ActivateBasicAttack`
  (params (SpawnAttackOfClass :type "Actor Class Reference") (AttackFrom :type "BoxComponent Object Reference"))
  (returns (AttackSpawn :type "/Game/Spells/Blueprints/BP_BasicAttacks Object Reference"))
  (locals (SpawnPoint :type "Vector Structure") (SpawnAttack :type "Actor Object Reference"))
  (bind (_origin _boxextent) (`KismetSystemLibrary.GetComponentBounds` AttackFrom))
  ;[0.5955 1 0.9198] Activate Base attack
  (bind _output_get (set `local.SpawnPoint` (`KismetMathLibrary.RandomPointInBoundingBox` _origin _boxextent)))
  (bind _returnvalue (`|SpawnActorFromClass` SpawnAttackOfClass (`KismetMathLibrary.MakeTransform` _output_get (struct) (1.0 1.0 1.0)) "AlwaysSpawn" "OverrideRootScale" self))
  (bind _output_get_2 (set `local.SpawnAttack` _returnvalue))
  ;;[0.4432 1 0.8384] Charge Basic attack
  (message `/Game/Interfaces/BPI_IsChargeble.StartCharge` _output_get_2)
  (return (cast `/Game/Spells/Blueprints/BP_BasicAttacks` (`local.SpawnAttack`) :!pure true)))

(fn `AddQi`
  (params (Cost :type Integer))
  (if (< (`self.Qi`) (`self.BaseQi`))
    (set `self.Qi` (+ (`self.Qi`) Cost))
    (`self.UpdateQiBar`)))

(fn `CastBasicAttack`
  (params (BasicAttack :type "/Game/Spells/Blueprints/BP_BasicAttacks Object Reference"))
  (locals (LocalZAxis :type "Float (double-precision)" :default 2.0) (LocalDirectionToCast :type "Vector Structure" :default (0.0 0.0 0.0)) (SpawnPoint :type "Vector Structure") (TraceLineLength :type "Float (double-precision)" :default 450.0) (LSpawnAttack :type "/Game/Spells/Blueprints/BP_BasicAttacks Object Reference") (SpeedyFactor :type "Float (double-precision)"))
  (bind _lspawnattack (`local.LSpawnAttack`))
  (bind _lspawnattack_2 (`local.LSpawnAttack`))
  ;[0.5955 1 0.9198] Cast Base attack
  (bind _output_get (set `local.LSpawnAttack` BasicAttack))
  (set `local.SpawnPoint` (`self.K2_GetActorLocation` _output_get))
  (for _ (range 101)
    (bind _output_get_2 (set `local.LocalDirectionToCast` (`KismetMathLibrary.RandomUnitVectorInConeWithYawAndPitch` (+ (`SceneComponent.GetForwardVector` (`self.ArrowComponent`)) (`KismetMathLibrary.MakeVector` 0.0 0.0 (`local.LocalZAxis`))) 90.0 80.0)))
    ;;[0.06647 0.0886 0.1746] Check if vector is antiparallel
    (`/Game/FunctionLibrary/MyMacroLibrary.VectorsAreOpposite?` (`KismetMathLibrary.MakeVector` (.x _output_get_2) (.y _output_get_2)) (`SceneComponent.GetForwardVector` (`self.ArrowComponent`))
      (:`NotOpposite`
        (`/Engine/EditorBlueprintResources/StandardMacros.IsValid` (`local.LSpawnAttack`)
          (:`Is Valid`
            ;;[0 0 0] Calculation of velocity
            (bind _output_get_3 (set `local.SpeedyFactor` (`KismetMathLibrary.RandomFloatInRange` 0.4 1.0)))
            ;;[0 0 0] Check if hit barrier
            (bind (_outhit _outpathpositions _outlasttracedestination _returnvalue) (`GameplayStatics.Blueprint_PredictProjectilePath_ByObjectType` (`local.SpawnPoint`) (* (`local.LocalDirectionToCast`) (* _output_get_3 (`/Game/Spells/Blueprints/BP_BasicAttacks.BaseSpeed` (`local.LSpawnAttack`)))) true 10.0 (`self.ObjectTypestoScan`) false (`|MakeArray` self _lspawnattack :!type "Actor Object Reference") "None" 1.0 2.0 2.0 (* (`/Game/Spells/Blueprints/BP_BasicAttacks.GravityScale` _lspawnattack) -981.0)))
            (if (not _returnvalue)
              (break)))
          (:`Is Not Valid`
            (break))))))
  (`/Engine/EditorBlueprintResources/StandardMacros.IsValid` _lspawnattack_2
    (:`Is Valid`
      (`/Game/Spells/Blueprints/BP_BasicAttacks.CastBaseAttackAI` _lspawnattack_2 (`self.EnemyTarget`) (`local.LocalDirectionToCast`) (`local.SpeedyFactor`)))))

(fn `CastTheBarrier`
  (params (SpawnBarrierOfClass :type "Actor Class Reference") (isGrowing :type Boolean) (IndexOftheBarrierLocation :type Integer))
  (bind _defensebarrier (`self.DefenseBarrier`))
  (bind _defensebarrier_2 (`self.DefenseBarrier`))
  (bind (_returnvalue_x _returnvalue_y) (`KismetMathLibrary.BreakVector` (`SceneComponent.K2_GetComponentLocation` (`self.ReferencePointToBarrierRotation`))))
  (bind (_output_x _output_y) (`KismetMathLibrary.BreakVector` (`|GetArrayItem` (`self.SpawnBarrierLocations`) IndexOftheBarrierLocation)))
  ;[1 1 1] Cast Barrier for the Left Hand
  ;;[0.6457 1 0.9901] Check  if button is pressed
  (if isGrowing
    ;;[0.6652 1 0.9701] If is the first time spawn, otherwise grow the nbarrier
    (if (`self.isCastingBarrier`)
      ;;[1 0.7759 0.6537] Grow the barrier at constant speedy
      (`/Engine/EditorBlueprintResources/StandardMacros.IsValid` _defensebarrier
        (:`Is Valid`
          (bind _asbp_barrier (cast `/Game/Spells/Blueprints/BP_Barrier` _defensebarrier))
          (`/Game/Spells/Blueprints/BP_Barrier.GrowBarrierAtZDirection` _asbp_barrier 70.0)))
      (else
        ;;[0.662 1 0.6828] Spawn the barrier
        (set `self.isCastingBarrier` true)
        (bind _returnvalue (`|SpawnActorFromClass` SpawnBarrierOfClass (`KismetMathLibrary.MakeTransform` (`KismetMathLibrary.MakeVector` _output_x _output_y 0.0) (`KismetMathLibrary.FindLookAtRotation` (`KismetMathLibrary.MakeVector` _returnvalue_x _returnvalue_y) (`KismetMathLibrary.MakeVector` _output_x _output_y))) "Undefined" "OverrideRootScale" self))
        (set `self.DefenseBarrier` _returnvalue)))
    (else
      (set `self.isCastingBarrier` false)
      ;;[0.4597 1 0.4957] Stops the grow sound
      (`/Engine/EditorBlueprintResources/StandardMacros.IsValid` _defensebarrier_2
        (:`Is Valid`
          (bind _asbp_barrier_2 (cast `/Game/Spells/Blueprints/BP_Barrier` _defensebarrier_2))
          (`|ExecutionSequence`
            (:`then_0`
              (`AudioComponent.Stop` (`/Game/Spells/Blueprints/BP_Barrier.GrowSound` _asbp_barrier_2)))
            (:`then_1`
              ;;[0.5828 0.9801 1] Set Barrier to be destroy and set DefenseBarrierLeft to none
              (`/Game/Spells/Blueprints/BP_Barrier.SelfDestroyAfterTimeLife` _asbp_barrier_2)
              (set `self.DefenseBarrier` null))))
        (:`Is Not Valid`
          (set `self.DefenseBarrier` null))))))

(fn `Consume QiFunction`
  (params (Cost :type Integer))
  (if (>= (`self.Qi`) 0)
    (set `self.Qi` (- (`self.Qi`) Cost))
    (`self.UpdateQiBar`)))

(fn `DeactivateAISpells`
  (`/Game/AI/BP_AIHand.DeactivateandDestroySpell` (`self.LeftHand`))
  (`/Game/AI/BP_AIHand.DeactivateandDestroySpell` (`self.RightHand`)))

(fn `GetsTheNearSpawnLocationFromAPoint`
  (params (Point :type "Vector Structure") (velocity :type "Vector Structure"))
  (returns (IndexOftheNearBox :type Integer) (ProbabilyToCastAtThisLocation :type "Float (double-precision)"))
  (locals (Distance :type "Float (double-precision)" :default 999999995904.0) (IndexOftheNearBoxLocalVar :type Integer))
  (if (> (`KismetMathLibrary.VSize` (- Point (`SceneComponent.K2_GetComponentLocation` (`self.Mesh`)))) 300.0)
    (for (_array_element _array_index) (`self.SpawnBarrierLocations`)
      (bind _returnvalue (`KismetMathLibrary.VSize` (- _array_element (+ Point (* (`KismetMathLibrary.Normal` velocity) 600.0)))))
      ;[1 0.6314 0.9219] Loop. Finds the closer location from the projectile to cast the barrier
      (if (< _returnvalue (`local.Distance`))
        (set `local.Distance` _returnvalue)
        (set `local.IndexOftheNearBoxLocalVar` _array_index)))
    (if (`|GetArrayItem` (`self.IsBarrierActiveAtThisLocation`) (`local.IndexOftheNearBoxLocalVar`))
      ;[1 0.3224 0.3124] Returns null probability of casting a barrier
      (return (`local.IndexOftheNearBoxLocalVar`) 0.0)
      (else
        ;[0.4467 1 0.4084] Return the index of the closest position to cast the barrier.
        (return (`local.IndexOftheNearBoxLocalVar`) 1.0)))
    (else
      ;[1 0.3224 0.3124] Returns null probability of casting a barrier
      (return (`local.IndexOftheNearBoxLocalVar`) 0.0))))

(fn `GetTargetComponent`
  (returns (Target :type "StaticMeshComponent Object Reference"))
  (return (`self.Body`)))

(fn `GiveQi`
  (params (InitialAmount :type Integer))
  (returns (ReturnAmount :type Integer) (GiveQiToOwner :type Boolean))
  (return (`KismetMathLibrary.FTrunc` (* InitialAmount (`self.QiMultiplier`))) false))

(fn `HasEnoughQi`
  (params (Cost :type Integer))
  (returns (Return :type Boolean))
  (if (>= (`self.Qi`) Cost)
    (return true)
    (else
      (return false))))

(fn `HasMaximumBarriers`
  (returns (Return :type Boolean))
  (return (>= (`self.CurrentNumberOfBarries`) (`self.MaxNumberOfAllowBarries`))))

(fn `ProbabilityOfCastingShield`
  (params (Life :type "Float (double-precision)") (PercentageOfLifeWithHalfProbability :type "Float (double-precision)"))
  (returns (val :type "Float (double-precision)"))
  (bind _val (`/Game/FunctionLibrary/MyFunctions.Gaussian` 1.0 (/ (* PercentageOfLifeWithHalfProbability (`KismetMathLibrary.Conv_IntToDouble` (`self.BaseLife`))) (`KismetMathLibrary.Sqrt` (* (`KismetMathLibrary.Loge` 0.5) -2.0))) 0.0 Life))
  (return _val))

(fn `RegenerateQiFunction`
  (if (< (`self.Qi`) (`self.BaseQi`))
    (set `self.Qi` (+ (`self.Qi`) (`self.QiRegeneration`)))
    (`self.UpdateQiBar`)))

(fn `SetAIOnSilence`
  (set `/Game/AI/BP_AIHand.CastStatus` "NewEnumerator2" (`self.LeftHand`))
  (set `/Game/AI/BP_AIHand.CastStatus` "NewEnumerator2" (`self.RightHand`)))

(fn `SetInitialConditions`
  (`|ExecutionSequence`
    (:`then_0`
      ;[0.365 1 0.566] Sets Life
      (set `self.Life` (`self.BaseLife`))
      ;[0.3411 0.4424 1] Set Initial Qi
      (set `self.Qi` 0))
    (:`then_1`
      ;[0.4333 0.6597 1] Sets Player reference
      (bind _asmotion_controller_pawn (cast `/Game/VirtualRealityBP/Blueprints/MotionControllerPawn` (`GameplayStatics.GetPlayerPawn` 0))
        (:`then`
          (set `self.Player` _asmotion_controller_pawn))
        (:`CastFailed`
          (`KismetSystemLibrary.PrintString` "Error: Player reference null."))))
    (:`then_2`
      ;[0.6596 1 0.5198] Sets the reference for the Health bar
      (bind _ashealth_qi_bar_bp (cast `/Game/WidgetBP/HealthQiBar_BP` (`WidgetComponent.GetUserWidgetObject` (`self.HealthBarWidget`)))
        (:`then`
          (set `self.WidgetHealthBar` _ashealth_qi_bar_bp))
        (:`CastFailed`
          (`KismetSystemLibrary.PrintText` "Fail to Cast to Player Health bar."))))
    (:`then_3`
      ;[0.1874 1 0.2705] Set elemements to be casted
      (`self.SetWhatToCastRight`)
      (`self.SetWhatToCastLeft`))))

(fn `SetVariablesFromDataBase`
  (params (RowName :type Name))
  (bind _returnvalue (`|GetDataTableRow` "/Game/AI/Data/AIDataStructure.AIDataStructure" RowName)
    (:`then`
      (`|ExecutionSequence`
        (:`then_0`
          (bind (_life _firerate _minimumtimetotriggerba _maximumtimetotriggerba _elementatleft _elementatright _blockrightattack _blockleftattack _blockleftshield _blockrightshield _blockbarrier) (break `/Game/AI/Data/AILevelStructure` _returnvalue))
          (set `self.BaseLife` _life))
        (:`then_1`
          (set `self.Firerate` _firerate))
        (:`then_2`
          (set `self.MinimunTimeToTriggerBasicAttack` _minimumtimetotriggerba))
        (:`then_3`
          (set `self.MaximumTimeToTriggerBasicAttack` _maximumtimetotriggerba))
        (:`then_4`
          (set `self.ElementAtLeft` _elementatleft))
        (:`then_5`
          (set `self.ElementAtRight` _elementatright))
        (:`then_6`
          (set `self.BlockRightAttack` _blockrightattack))
        (:`then_7`
          (set `self.BlockLeftAttack` _blockleftattack))
        (:`then_8`
          (set `self.BlockLeftShield` _blockleftshield))
        (:`then_9`
          (set `self.BlockRightShield` _blockrightshield))
        (:`then_10`
          (set `self.BlockBarrier` _blockbarrier))))
    (:`RowNotFound`
      (`VisualLoggerKismetLibrary.LogText` "Warning: Row not found at AI SetVariablesFromDataBase" "Error"))))

(fn `SetWhatToCastLeft`
  (switch `/Game/VirtualRealityBP/Enumerates/EElementSelected` (`self.ElementAtLeft`)
    (:`NewEnumerator1`
      (set `self.WhatToCastOnShieldLeft` "/Game/Spells/Blueprints/BP_FireShield.BP_FireShield_C")
      (set `self.WhatBasicAttackToSpawnLeft` "/Game/Spells/Blueprints/BP_FireBall.BP_FireBall_C")
      (set `self.WhatToCastOnLeftBarrrier` "/Game/Spells/Blueprints/BP_FireBarrier.BP_FireBarrier_C"))
    (:`NewEnumerator2`
      (set `self.WhatToCastOnShieldLeft` "/Game/Spells/Blueprints/BP_EarthShield.BP_EarthShield_C")
      (set `self.WhatBasicAttackToSpawnLeft` "/Game/Spells/Blueprints/BP_EarthBall.BP_EarthBall_C")
      (set `self.WhatToCastOnLeftBarrrier` "/Game/Spells/Blueprints/BP_EarthBarrier.BP_EarthBarrier_C"))
    (:`NewEnumerator3`
      (set `self.WhatToCastOnShieldLeft` "/Game/Spells/Blueprints/BP_WaterShield.BP_WaterShield_C")
      (set `self.WhatBasicAttackToSpawnLeft` "/Game/Spells/Blueprints/BP_WaterBall.BP_WaterBall_C")
      (set `self.WhatToCastOnLeftBarrrier` "/Game/Spells/Blueprints/BP_WaterBarrier.BP_WaterBarrier_C"))
    (:`NewEnumerator4`
      (set `self.WhatToCastOnShieldLeft` "/Game/Spells/Blueprints/BP_WindShield.BP_WindShield_C")
      (set `self.WhatBasicAttackToSpawnLeft` "/Game/Spells/Blueprints/BP_WindBall.BP_WindBall_C")
      (set `self.WhatToCastOnLeftBarrrier` "/Game/Spells/Blueprints/BP_WindBarrier.BP_WindBarrier_C"))))

(fn `SetWhatToCastRight`
  (switch `/Game/VirtualRealityBP/Enumerates/EElementSelected` (`self.ElementAtRight`)
    (:`NewEnumerator1`
      (set `self.WhatToCastOnShieldRight` "/Game/Spells/Blueprints/BP_FireShield.BP_FireShield_C")
      (set `self.WhatBasicAttackToSpawnRight` "/Game/Spells/Blueprints/BP_FireBall.BP_FireBall_C")
      (set `self.WhatToCastOnRightBarrrier` "/Game/Spells/Blueprints/BP_EarthBarrier.BP_EarthBarrier_C"))
    (:`NewEnumerator2`
      (set `self.WhatToCastOnShieldRight` "/Game/Spells/Blueprints/BP_EarthShield.BP_EarthShield_C")
      (set `self.WhatBasicAttackToSpawnRight` "/Game/Spells/Blueprints/BP_EarthBall.BP_EarthBall_C")
      (set `self.WhatToCastOnRightBarrrier` "/Game/Spells/Blueprints/BP_FireBarrier.BP_FireBarrier_C"))
    (:`NewEnumerator3`
      (set `self.WhatToCastOnShieldRight` "/Game/Spells/Blueprints/BP_WaterShield.BP_WaterShield_C")
      (set `self.WhatBasicAttackToSpawnRight` "/Game/Spells/Blueprints/BP_WaterBall.BP_WaterBall_C")
      (set `self.WhatToCastOnRightBarrrier` "/Game/Spells/Blueprints/BP_WaterBarrier.BP_WaterBarrier_C"))
    (:`NewEnumerator4`
      (set `self.WhatToCastOnShieldRight` "/Game/Spells/Blueprints/BP_WindShield.BP_WindShield_C")
      (set `self.WhatBasicAttackToSpawnRight` "/Game/Spells/Blueprints/BP_WindBall.BP_WindBall_C")
      (set `self.WhatToCastOnRightBarrrier` "/Game/Spells/Blueprints/BP_WindBarrier.BP_WindBarrier_C"))))

(fn `ShouldAttackWithBothHands`
  (params (Probability :type "Float (double-precision)"))
  (returns (Return :type Boolean))
  (return (`KismetMathLibrary.RandomBoolWithWeight` Probability)))

(fn `TimeForChargeAttacks`
  (params (ChargingAttack :type "/Game/Spells/Blueprints/BP_BasicAttacks Object Reference"))
  (returns (Time :type "Float (double-precision)"))
  (locals (MaxWaitingTime :type "Float (double-precision)") (CurveTimeScale :type "Float (double-precision)" :default 1.0))
  (`/Engine/EditorBlueprintResources/StandardMacros.IsValid` ChargingAttack
    (:`Is Valid`
      (set `local.MaxWaitingTime` (`/Game/Spells/Blueprints/BP_BasicAttacks.TimeToCharge` ChargingAttack))
      (if (`KismetMathLibrary.RandomBoolWithWeight` 0.6)
        (return (`local.MaxWaitingTime`))
        (else
          (return (`KismetMathLibrary.RandomFloatInRange` (* (`local.MaxWaitingTime`) 0.3) (* (`local.MaxWaitingTime`) 1.5))))))
    (:`Is Not Valid`
      (return 0.0))))

(fn `UserConstructionScript`
  (bind _mesh (`self.Mesh`))
  (`|ExecutionSequence`
    (:`then_0`
      (bind _returnvalue (`PrimitiveComponent.CreateDynamicMaterialInstance` _mesh 0 (`PrimitiveComponent.GetMaterial` _mesh 0)))
      (set `self.BodyMaterial` _returnvalue))
    (:`then_1`
      ;[1 0.9283 0.1475] Sets the AI DataBase.
      (`self.SetVariablesFromDataBase` (`KismetStringLibrary.Conv_StringToName` (`|GetEnumeratorNameAsString` (`self.AILevel`)))))))