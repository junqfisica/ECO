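; Actor that hosts the VR networking menus on a widget component, switching between main, host, server, loading and error screens.
; On BeginPlay it passes itself to the main network menu widget as owner actor.
; Each Show event receives a widget, displays it at a screen-specific draw size and, except for loading, passes itself as owner; the main menu also re-enables buttons.
; BackToMainMenu is only a print stub.
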(event `self.ReceiveBeginPlay`
  (bind _asmain_network_vrmenu (cast `/Game/WidgetBP/MainNetworkVRMenu` (`WidgetComponent.GetUserWidgetObject` (`self.Widget`))))
  (bind _output_get (set `self.MainNetworkingMenu` _asmain_network_vrmenu))
  ;[0.3812 1 0.6277] Pass this actor to the widget
  (`/Game/WidgetBP/MainNetworkVRMenu.SetOwnerActor` _output_get self))

(event `ShowMainMenu`
  (params (Widget :type "/Game/WidgetBP/MainNetworkVRMenu Object Reference"))
  ;[0.8934 1 0.4631] Sets Main menu
  (set `/Game/WidgetBP/MainNetworkVRMenu.EnableButtons` true Widget)
  (`WidgetComponent.SetWidget` (`self.Widget`) Widget)
  (`WidgetComponent.SetDrawSize` (`self.Widget`) (500.0 500.0))
  (`/Game/WidgetBP/MainNetworkVRMenu.SetOwnerActor` Widget self))

(event `ShowHostMenu`
  (params (Widget :type "/Game/WidgetBP/HostMenuVR Object Reference"))
  ;[0.5109 0.7834 1] Sets VR Host Menu
  (`WidgetComponent.SetWidget` (`self.Widget`) Widget)
  (`WidgetComponent.SetDrawSize` (`self.Widget`) (1000.0 1000.0))
  (`/Game/WidgetBP/HostMenuVR.SetOwnerActor` Widget self))

(event `ShowServerMenu`
  (params (Widget :type "/Game/WidgetBP/ServerMenuVR Object Reference"))
  ;[0.5415 1 0.8371] Sets VR Server Menu
  (`WidgetComponent.SetWidget` (`self.Widget`) Widget)
  (`WidgetComponent.SetDrawSize` (`self.Widget`) (800.0 500.0))
  (`/Game/WidgetBP/ServerMenuVR.SetOwnerActor` Widget self))

(event `ShowLoadingScreen`
  (params (Widget :type "/Game/WidgetBP/LoadingScreen Object Reference"))
  ;[0.633 0.6611 1] Sets VR Loading Screen
  (`WidgetComponent.SetWidget` (`self.Widget`) Widget)
  (`WidgetComponent.SetDrawSize` (`self.Widget`) (800.0 400.0)))

(event `ShowErrorDiag`
  (params (Widget :type "/Game/WidgetBP/ErrorDialog Object Reference"))
  ;[1 0.4317 0.3719] Sets VR ErrorDig Screen
  (`WidgetComponent.SetWidget` (`self.Widget`) Widget)
  (`WidgetComponent.SetDrawSize` (`self.Widget`) (800.0 400.0))
  (`/Game/WidgetBP/ErrorDialog.SetOwnerActor` Widget self))

(event `BackToMainMenu`
  ;[0.5051 0.508 1] Implement this
  (`KismetSystemLibrary.PrintString` "Back to main menu"))

(fn `UserConstructionScript`)