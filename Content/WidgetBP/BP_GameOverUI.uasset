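; Actor that hosts the WBP_GameOver widget through a widget component, serving as the in-world game over menu.
; On BeginPlay it caches the widget and passes it the restart and menu levels to load from its two buttons.
; Tick mirrors the actor's hidden state to the widget's enabled state, disabling the menu while it is hidden during match flow.
; SetVictoryText sets the widget's title.
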(event `self.ReceiveBeginPlay`
  (bind _aswbp_game_over (cast `/Game/WidgetBP/WBP_GameOver` (`WidgetComponent.GetUserWidgetObject` (`self.GameOverWidget`))))
  (set `self.GameOver` _aswbp_game_over)
  ;[0.8286 0.5374 1] Set default levels to be loaded.
  (`self.SetRestartLevel` (`self.LevelToLoadOnRestart`))
  (`self.SetMenuLevel` (`self.LevelToLoadOnMenu`)))

(event `self.ReceiveTick`
  (params (DeltaSeconds :type "Float (single-precision)"))
  (bind _gameover (`self.GameOver`))
  ;[1 1 1] When this actor is not visible, disable its associated widget - used during match flow
  (if (`self.bHidden`)
    (`Widget.SetIsEnabled` _gameover false)
    (else
      (`Widget.SetIsEnabled` _gameover true))))

(fn `SetMenuLevel`
  (params (LevelToLoadOnMenu :type Name))
  (set `/Game/WidgetBP/WBP_GameOver.LevelToLoadOnB2` LevelToLoadOnMenu (`self.GameOver`)))

(fn `SetRestartLevel`
  (params (LevelToLoadOnRestart :type Name))
  (set `/Game/WidgetBP/WBP_GameOver.LevelToLoadOnB1` LevelToLoadOnRestart (`self.GameOver`)))

(fn `SetVictoryText`
  (params (Text :type Text))
  (`/Game/WidgetBP/WBP_GameOver.SetTitleText` (`self.GameOver`) Text))

(fn `UserConstructionScript`)