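; 3D character status display showing health, segmented Qi, and per-hand element colours and basic-attack counters.
; Construction gives each hand's sphere and counters a shared dynamic material, and collects "Qi"-tagged children of QiBarHolder as bar segments.
; Events set material colours, toggle counter visibility, and scale meshes on X for fill, with Qi filling segment by segment.
; An unfinished not-enough-Qi timeline enlarges the Qi holder and plays a voice cue.
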(event `self.ReceiveBeginPlay`
  ;[0.4328 1 0.9302] Sets black color as default
  (`self.SetFeedBackColor` "Left")
  (`self.SetFeedBackColor` "Right"))

(event `PlayNotEnoughtQiAnim`
  ;[1 1 1] Play animation when player don't have engouth Qi. Still need implementation
  (`TimelineComponent.SetPlayRate` (`self.NotEnoghtQi`) 1.0)
  (bind (_direction _alpha) (`Timeline|NotEnoghtQi` :!via `PlayFromStart`)
    (:`Update`
      (`SceneComponent.SetWorldScale3D` (`self.QiBarHolder`) (`KismetMathLibrary.VLerp` (1.0 1.0 1.0) (1.5 1.5 1.5) _alpha)))
    (:`PlaySound`
      ;;[1 1 1] Play the voice sound here
      (`GameplayStatics.SpawnSoundAtLocation` "/Game/SoundsEffects/Cues/CUE_VO_NotEnoughQi.CUE_VO_NotEnoughQi" (`SceneComponent.K2_GetComponentLocation` (`self.DefaultSceneRoot`))))))

(event `SetFeedBackColor`
  (params (Hand :type "EControllerHand Enum") (BaseColor :type "LinearColor Structure") (SecundaryColor :type "LinearColor Structure"))
  (bind _leftelement (`self.LeftElement`))
  (bind _rightelement (`self.RightElement`))
  (switch `EControllerHand` Hand
    (:`Left`
      ;[1 1 1] Changes color of material for left sphere
      (`MaterialInstanceDynamic.SetVectorParameterValue` _leftelement "BaseColor" BaseColor)
      (`MaterialInstanceDynamic.SetVectorParameterValue` _leftelement "SecundaryColor" SecundaryColor))
    (:`Right`
      ;[1 1 1] Changes color of material for right sphere
      (`MaterialInstanceDynamic.SetVectorParameterValue` _rightelement "BaseColor" BaseColor)
      (`MaterialInstanceDynamic.SetVectorParameterValue` _rightelement "SecundaryColor" SecundaryColor))))

(event `Set Percent`
  (params (Percent :type "Float (double-precision)"))
  ;[0.6457 0.9901 1] Set Health Bar Percent
  (`SceneComponent.SetRelativeScale3D` (`self.SM_HealthBar`) (`KismetMathLibrary.MakeVector` (`KismetMathLibrary.FClamp` Percent) 1.0 1.0)))

(event `Set QI Percent`
  (params (Percent :type "Float (double-precision)"))
  (bind _bar0 (`self.Bar0`))
  (bind _bar1 (`self.Bar1`))
  (bind _bar2 (`self.Bar2`))
  (bind _bar3 (`self.Bar3`))
  (bind _bar4 (`self.Bar4`))
  (bind _returnvalue (* (`KismetMathLibrary.FClamp` Percent) (`KismetMathLibrary.Conv_IntToDouble` (`self.TotalNumberOfVisibleQiBar`))))
  (bind _returnvalue_2 (`KismetMathLibrary.FTrunc` _returnvalue))
  ;[0.9124 0.6437 1] Set Qi bars
  (`self.Clear IQ Bars`)
  (set `self.LPercent` (- _returnvalue (`KismetMathLibrary.Conv_IntToDouble` _returnvalue_2)))
  (`|ExecutionSequence`
    (:`then_0`
      (if (== _returnvalue_2 (`self.TotalNumberOfVisibleQiBar`))
        ;[0.5103 0.8054 1] Sets all to 1 when percent is equal 1
        (for _array_element (`self.QiBars`)
          (`SceneComponent.SetRelativeScale3D` _array_element (`KismetMathLibrary.MakeVector` 1.0 1.0 1.0)))
        (else
          ;[1 1 1] Scale each bar
          (for (_array_element_2 _array_index) (`self.QiBars`)
            (if (< (- _returnvalue_2 1) _array_index)
              (break)
              (else
                (`SceneComponent.SetRelativeScale3D` _array_element_2 (`KismetMathLibrary.MakeVector` 1.0 1.0 1.0)))))
          (`SceneComponent.SetRelativeScale3D` (`|GetArrayItem` (`self.QiBars`) _array_index) (`KismetMathLibrary.MakeVector` (`self.LPercent`) 1.0 1.0)))))
    (:`then_1`
      ;[1 1 1] Visablility
      (`|ExecutionSequence`
        (:`then_0`
          (if (<= (.x (`SceneComponent.RelativeScale3D` (`self.Bar1`))) 0.0)
            (`SceneComponent.SetVisibility` _bar1 false false)
            (else
              (`SceneComponent.SetVisibility` _bar1 true false))))
        (:`then_1`
          (if (<= (.x (`SceneComponent.RelativeScale3D` (`self.Bar2`))) 0.0)
            (`SceneComponent.SetVisibility` _bar2 false false)
            (else
              (`SceneComponent.SetVisibility` _bar2 true false))))
        (:`then_2`
          (if (<= (.x (`SceneComponent.RelativeScale3D` (`self.Bar3`))) 0.0)
            (`SceneComponent.SetVisibility` _bar3 false false)
            (else
              (`SceneComponent.SetVisibility` _bar3 true false))))
        (:`then_3`
          (if (<= (.x (`SceneComponent.RelativeScale3D` (`self.Bar4`))) 0.0)
            (`SceneComponent.SetVisibility` _bar4 false false)
            (else
              (`SceneComponent.SetVisibility` _bar4 true false))))
        (:`then_4`
          (if (<= (.x (`SceneComponent.RelativeScale3D` (`self.Bar0`))) 0.0)
            (`SceneComponent.SetVisibility` _bar0 false false)
            (else
              (`SceneComponent.SetVisibility` _bar0 true false))))))))

(event `UpdateBasicAttackCount`
  (params (Hand :type "EControllerHand Enum") (Index :type Integer))
  ;[1 1 1] Ian - Basic attack count
  (switch `EControllerHand` Hand
    (:`Left`
      (`SceneComponent.SetVisibility` (`|GetArrayItem` (`self.LeftHandBasicAttackCount`) (+ Index -1)) false false))
    (:`Right`
      (`SceneComponent.SetVisibility` (`|GetArrayItem` (`self.RightHandBasicAttackCount`) (+ Index -1)) false false))))

(event `ResetAttackCount`
  (params (Hand :type "EControllerHand Enum"))
  ;[1 1 1] Ian - Basic attack count
  (switch `EControllerHand` Hand
    (:`Left`
      (for _array_element (`self.LeftHandBasicAttackCount`)
        (`SceneComponent.SetVisibility` _array_element true false)))
    (:`Right`
      (for _array_element_2 (`self.RightHandBasicAttackCount`)
        (`SceneComponent.SetVisibility` _array_element_2 true false)))))

(event `ClearAttackCount`
  (params (Hand :type "EControllerHand Enum"))
  ;[1 1 1] Ian - Basic attack count
  (switch `EControllerHand` Hand
    (:`Left`
      (for _array_element (`self.LeftHandBasicAttackCount`)
        (`SceneComponent.SetVisibility` _array_element false false)))
    (:`Right`
      (for _array_element_2 (`self.RightHandBasicAttackCount`)
        (`SceneComponent.SetVisibility` _array_element_2 false false)))))

(fn `Clear IQ Bars`
  (for _array_element (`self.QiBars`)
    (`SceneComponent.SetRelativeScale3D` _array_element (`KismetMathLibrary.MakeVector` 0.0 1.0 1.0))))

(fn `UserConstructionScript`
  (set `self.LeftHandBasicAttackCount` (`|MakeArray` (`self.Basic attack left1`) (`self.Basic attack left2`)))
  (set `self.RightHandBasicAttackCount` (`|MakeArray` (`self.Basic attack right1`) (`self.Basic attack right2`)))
  (`|ExecutionSequence`
    (:`then_0`
      (bind _returnvalue (`KismetMaterialLibrary.CreateDynamicMaterialInstance` "/Game/Meshes/M_HealthBar.M_HealthBar"))
      (bind _output_get (set `self.LeftElement` _returnvalue))
      (`PrimitiveComponent.SetMaterial` (`self.LeftHandBall`) 0 _output_get)
      (for _array_element (`self.LeftHandBasicAttackCount`)
        (`PrimitiveComponent.SetMaterial` _array_element 0 (`self.LeftElement`))))
    (:`then_1`
      (bind _returnvalue_2 (`KismetMaterialLibrary.CreateDynamicMaterialInstance` "/Game/Meshes/M_HealthBar.M_HealthBar"))
      (bind _output_get_2 (set `self.RightElement` _returnvalue_2))
      (`PrimitiveComponent.SetMaterial` (`self.RightHandBall`) 0 _output_get_2)
      (for _array_element_2 (`self.RightHandBasicAttackCount`)
        (`PrimitiveComponent.SetMaterial` _array_element_2 0 (`self.RightElement`))))
    (:`then_2`
      ;[1 1 1] Create refrence for each Qi bar and keep into an array
      (for _array_element_3 (`SceneComponent.GetChildrenComponents` (`self.QiBarHolder`) false)
        (bind _asstatic_mesh_component (cast `StaticMeshComponent` _array_element_3))
        (if (`ActorComponent.ComponentHasTag` _asstatic_mesh_component "Qi")
          (`KismetArrayLibrary.Array_AddUnique` (`self.QiBars`) _asstatic_mesh_component)
          (`/Engine/EditorBlueprintResources/StandardMacros.IncrementInt` (`self.TotalNumberOfVisibleQiBar`))))
      (for (_array_element_4 _array_index) (`self.QiBars`)
        ;[1 1 1] Create a material instance for each QiBar and set this as a material
        (bind _returnvalue_3 (`KismetMaterialLibrary.CreateDynamicMaterialInstance` "/Game/Meshes/M_ManaBar.M_ManaBar"))
        (`KismetArrayLibrary.Array_AddUnique` (`self.ManaInstances`) _returnvalue_3)
        (`PrimitiveComponent.SetMaterial` _array_element_4 0 (`|GetArrayItem` (`self.ManaInstances`) _array_index))))))