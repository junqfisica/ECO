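; WindBall_BP is a chargeable wind ball spell that grows in size and damage while charged.
; StartCharge plays the ChargeWind timeline, which scales the mesh from SpellScale and computes DamageCharged from BaseDamage.
; A timeline event steps EventTracker through visual stages, which so far only print debug text labelled "Fire".
; StopCharge halts the timeline and overwrites BaseDamage with the rounded charged damage.
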(event `self.StartCharge`
  (`KismetSystemLibrary.PrintText` "Wind is Chanring")
  (bind (_direction _percentdamage _percentscale) (`Timeline|ChargeWind` :!via `PlayFromStart` :!label _label)
    (:`Update`
      ;[0.255 0.255 0.255] Update Node
      ;;[0.5705 0.6356 1] Change the scale of the mesh
      (`SceneComponent.SetWorldScale3D` (`self.StaticMeshComponent`) (* (`self.SpellScale`) _percentscale))
      ;;[0.5245 1 0.7717] Charge the damage
      (set `self.DamageCharged` (* _percentdamage (`KismetMathLibrary.Conv_IntToDouble` (`self.BaseDamage`)))))
    (:`ChangeVisual`
      (switch `int` (`self.EventTracker`)
        (:`0`
          (`KismetSystemLibrary.PrintText` "Fire Visual changed: 1")
          (`/Engine/EditorBlueprintResources/StandardMacros.IncrementInt` (`self.EventTracker`)))
        (:`1`
          (`KismetSystemLibrary.PrintText` "Fire Visual changed: 2"))))))

(event `self.StopCharge`
  (`KismetSystemLibrary.PrintText` "Wind Stop Charge")
  (set `self.BaseDamage` (`KismetMathLibrary.Round` (`self.DamageCharged`)))
  (goto _label :!via `Stop`))

(fn `UserConstructionScript`
  (`parent.UserConstructionScript`))