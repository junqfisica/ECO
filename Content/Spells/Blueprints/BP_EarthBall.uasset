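; BP_EarthBall is a chargeable earth projectile spell built on a parent spell's charge and fire logic.
; On charge start it spawns randomly scaled BP_Rising_Ground_Earth actors around the caster's location and gives them a reference to the ball.
; They are destroyed on overlapping the sphere, or when the attack fires.
; ChangeEarthVisual uses a counter to step audio and particles through charge stages, tuning projectile emitter parameters.
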(event `self.ReceiveBeginPlay`
  (`parent.ReceiveBeginPlay`))

(event `ChangeEarthVisual`
  (bind _p_projectile (`self.P_Projectile`))
  (bind _p_projectile_2 (`self.P_Projectile`))
  ;[0.7846 0.5094 1] Trigger Events to change visual.
  (switch `int` (`self.EventTracker`)
    (:`0`
      (`self.ClientPlayAudioWithTransition` (`self.Cue_Stage1`) (`self.Cue_TrigerStage2`) 0.1)
      (`self.ClientPlayAudio` (`self.Cue_Stage2`))
      (`self.SwitchParticle` (`self.P_InitialCharge`) (`self.P_Projectile`))
      (`/Engine/EditorBlueprintResources/StandardMacros.IncrementInt` (`self.EventTracker`)))
    (:`1`
      (`self.ClientPlayAudioWithTransition` (`self.Cue_Stage2`) (`self.Cue_TrigerStage3`) 0.1)
      (`self.ClientPlayAudio` (`self.Cue_Stage3`))
      (`self.SwitchParticle` _p_projectile_2 _p_projectile_2)
      (`ParticleSystemComponent.SetVectorParameter` _p_projectile "SockWaveSize" (20.0 20.0 20.0))
      (`ParticleSystemComponent.SetFloatParameter` _p_projectile "NumberOfGrains" 3.0)
      (`ParticleSystemComponent.SetEmitterEnable` _p_projectile "EarthCollapse" false))))

(event `self.StartCharge`
  ;[1 1 1] Line Trace to ground and set random points in bounds
  (`parent.StartCharge`)
  (set `self.GroundLocation` (`self.K2_GetActorLocation` (`self.GetOwner`)))
  (`self.Spawn Water From Ground`))

(event `Spawn Water From Ground`
  ;[1 1 1] Spawns water from ground
  (for _ (range 17)
    (bind _returnvalue (`|SpawnActorFromClass` "/Game/Spells/Blueprints/SupportBlueprints/BP_Rising_Ground_Earth.BP_Rising_Ground_Earth_C" (`KismetMathLibrary.MakeTransform` (`KismetMathLibrary.RandomPointInBoundingBox` (`self.GroundLocation`) (`KismetMathLibrary.MakeVector` 300.0 300.0)) (`KismetMathLibrary.RandomRotator` false) (`KismetMathLibrary.Conv_DoubleToVector` (`KismetMathLibrary.RandomFloatInRange` 0.1 1.0))) "Undefined" "OverrideRootScale"))
    (set `/Game/Spells/Blueprints/SupportBlueprints/BP_Rising_Ground_Earth.EarthBallBP` self _returnvalue)
    (`KismetArrayLibrary.Array_Add` (`self.WaterFromGround`) _returnvalue)))

(event `self.Sphere.OnComponentBeginOverlap`
  (params (OverlappedComponent :type "PrimitiveComponent Object Reference") (OtherActor :type "Actor Object Reference") (OtherComp :type "PrimitiveComponent Object Reference") (OtherBodyIndex :type Integer) (bFromSweep :type Boolean) (SweepResult :type "HitResult Structure (by ref)"))
  ;[1 1 1] Destroy water from ground when it hits ball
  (bind _asbp_rising_ground_earth (cast `/Game/Spells/Blueprints/SupportBlueprints/BP_Rising_Ground_Earth` OtherActor))
  (`self.K2_DestroyActor` _asbp_rising_ground_earth))

(event `self.FiresBasicAttack`
  (params (TargetToHit :type "Actor Object Reference") (AttackDirection :type "Vector Structure") (SpeedFactor :type "Float (single-precision)"))
  ;[1 1 1] Destroys water from ground when spell is fired
  (`parent.FiresBasicAttack` TargetToHit AttackDirection SpeedFactor)
  (for _array_element (`self.WaterFromGround`)
    (`/Engine/EditorBlueprintResources/StandardMacros.IsValid` _array_element
      (:`Is Valid`
        (`self.K2_DestroyActor` _array_element)))))

(fn `UserConstructionScript`
  (`parent.UserConstructionScript`))