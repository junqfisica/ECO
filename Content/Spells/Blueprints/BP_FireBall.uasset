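; BP_FireBall is a fireball spell Blueprint that escalates its look and sound through charge stages.
; Each ChangeVisualFire call reads EventTracker to pick the stage, crossfading client audio into a trigger cue and playing that stage's cue.
; The first stage swaps the initial charge particle for the projectile particle with blue fire off.
; The next restarts the projectile particle with the BlueFire emitter on and a blue flame color.
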(event `self.ReceiveBeginPlay`
  (`parent.ReceiveBeginPlay`))

(event `ChangeVisualFire`
  (bind _p_projectile (`self.P_Projectile`))
  (bind _p_projectile_2 (`self.P_Projectile`))
  ;[0.7846 0.5094 1] Trigger Events to change visual.
  (switch `int` (`self.EventTracker`)
    (:`0`
      (`self.ClientPlayAudioWithTransition` (`self.Cue_Stage1`) (`self.Cue_TrigerStage2`) 0.1)
      (`self.ClientPlayAudio` (`self.Cue_Stage2`))
      (`self.SwitchParticle` (`self.P_InitialCharge`) _p_projectile)
      (`ParticleSystemComponent.SetEmitterEnable` _p_projectile "BlueFire" false)
      (`/Engine/EditorBlueprintResources/StandardMacros.IncrementInt` (`self.EventTracker`)))
    (:`1`
      (`self.ClientPlayAudioWithTransition` (`self.Cue_Stage2`) (`self.Cue_TrigerStage3`) 0.1)
      (`self.ClientPlayAudio` (`self.Cue_Stage3`))
      (`self.SwitchParticle` _p_projectile_2 _p_projectile_2)
      (`ParticleSystemComponent.SetEmitterEnable` (`self.P_Projectile`) "BlueFire" true)
      (`ParticleSystemComponent.SetColorParameter` (`self.P_Projectile`) "FlameColor" (struct :`R` 0.03 :`G` 0.2 :`B` 1.0 :`A` 1.0)))))

(fn `UserConstructionScript`
  (`parent.UserConstructionScript`))