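; Water ball spell Blueprint that changes its particle visuals and hand vibration in stages.
; ChangeWaterVisual uses an EventTracker counter to pick the stage on each call.
; The first call swaps the initial charge particle for the trail with a brief, light vibration.
; Later calls activate the projectile and an enlarged initial charge particle with stronger vibration, both vibrations being marked as temporary test code.
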(event `self.ReceiveBeginPlay`
  (`parent.ReceiveBeginPlay`))

(event `ChangeWaterVisual`
  (bind _p_initialcharge (`self.P_InitialCharge`))
  ;[0.7846 0.5094 1] Trigger Events to change visual.
  (switch `int` (`self.EventTracker`)
    (:`0`
      (`self.SetHandsVibration` 0.1 0.3) ; Remove...test yet
      (`self.SwitchParticle` (`self.P_InitialCharge`) (`self.P_Trail`))
      (`/Engine/EditorBlueprintResources/StandardMacros.IncrementInt` (`self.EventTracker`)))
    (:`1`
      (`self.SetHandsVibration` 0.5 -1.0) ; Remove...test yet
      (`ActorComponent.Activate` (`self.P_Projectile`) false)
      (`ActorComponent.Activate` _p_initialcharge false)
      (`SceneComponent.SetRelativeScale3D` _p_initialcharge (1.5 1.5 1.5)))))

(fn `UserConstructionScript`
  (`parent.UserConstructionScript`))