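; Shield spell actor attached to a motion controller hand, absorbing damage until its life runs out.
; Life starts from a base value at BeginPlay and drops with each shield damage event.
; At zero, it briefly disables spells on the owning BP_MotionController, found through the mesh's attach parent, then destroys itself shortly after.
; A separate event applies per-hand location and rotation offsets to the mesh for left or right casting.
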(event `self.ReceiveBeginPlay`
  ;[1 0.3944 0.8064] Set initial life
  (set `self.CurrentLife` (`self.BaseShieldLife`)))

(event `OnShieldDamage`
  (params (Damage :type Integer))
  ;[0.6301 1 0.94] On Shield Damage
  (bind _output_get (set `self.CurrentLife` (- (`self.CurrentLife`) Damage)))
  (if (<= _output_get 0)
    ;;[1 1 1] Deals with the Player
    (bind _asbp_motion_controller (cast `/Game/VirtualRealityBP/Blueprints/BP_MotionController` (`ActorComponent.GetOwner` (`SceneComponent.GetAttachParent` (`self.StaticMeshComponent`))))
      (:`then`
        (`/Game/VirtualRealityBP/Blueprints/BP_MotionController.DisableSpellTemporaly` _asbp_motion_controller 0.5))
      (:`CastFailed`
        _))
    ;;[1 0.6961 0.6159] Destroy Shield after 0.1 secs
    (`self.SetLifeSpan` 0.1)))

(event `SetOffSeet`
  (params (CastToHand :type "EControllerHand Enum"))
  ;[1 0.3638 0.8973] Set an off set for the Left/Right shield.
  (switch `EControllerHand` CastToHand
    (:`Left`
      (`|ExecutionSequence`
        (:`then_0`
          (`SceneComponent.K2_AddRelativeLocation` (`self.StaticMeshComponent`) (`self.LocationOffsetForLeftHand`) false false))
        (:`then_1`
          (`SceneComponent.K2_AddRelativeRotation` (`self.StaticMeshComponent`) (`self.RotationOffsetForLeftHand`) false false))))
    (:`Right`
      (`|ExecutionSequence`
        (:`then_0`
          (`SceneComponent.K2_AddRelativeLocation` (`self.StaticMeshComponent`) (`self.LocationOffsetForRightHand`) false false))
        (:`then_1`
          (`SceneComponent.K2_AddRelativeRotation` (`self.StaticMeshComponent`) (`self.RotationOffsetForRightHand`) false false))))))

(fn `UserConstructionScript`)