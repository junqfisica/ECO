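; Elemental barrier spell actor that takes damage until it explodes or sinks away through a timeline.
; On authority BeginPlay, it enforces the owner's barrier cap via BPI_SpellRules and charges Qi from single-player, multiplayer or AI casters, then applies a Z offset and randomly signed rotation.
; Construction loads life and lifetime from a data table row named after the elemental class.
; Helper functions move it within Z limits, and destruction decrements the owner's barrier count.
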(event `self.ReceiveBeginPlay`
  (bind _staticmeshcomponent (`self.StaticMeshComponent`))
  (bind _returnvalue (`self.GetOwner` self))
  (`/Engine/EditorBlueprintResources/ActorMacros.Switch Has Authority` ; Avoid the Client to flip back the barrier
    (:`Authority`
      ;[1 0.588 0.2686] Check if player has more than the allow number of barriers. Need to test this for MP.
      (if (`KismetSystemLibrary.DoesImplementInterface` _returnvalue "/Game/Interfaces/BPI_SpellRules.BPI_SpellRules_C")
        (bind _return (message `/Game/Interfaces/BPI_SpellRules.HasMaximumBarriers` _returnvalue))
        (if _return
          (message `/Game/Interfaces/BPI_SpellRules.AddBarrier` (`self.GetOwner` self))
          (`self.K2_DestroyActor`)
          (else
            (bind (_sinlgeplayerref _multiplayerref _ai_ref) (`/Game/FunctionLibrary/MyMacroLibrary.WhichPlayerIs` _returnvalue)
              (:`SinglePlayer`
                ;[0 1 0.6776] See if Player has enough Qi to Cast this barrier
                (`self.CanBeCast` _sinlgeplayerref _multiplayerref :!label _label
                  (:`Yes`
                    (`|ExecutionSequence` :!label _label_2
                      (:`then_0`
                        ;[0.3476 0.4402 1] Add Barrier to owner
                        (message `/Game/Interfaces/BPI_SpellRules.AddBarrier` (`self.GetOwner` self))
                        ;[1 0.6995 0.8682] Set the OffSet
                        (`SceneComponent.K2_AddWorldOffset` (`self.StaticMeshComponent`) (`KismetMathLibrary.MakeVector` 0.0 0.0 (`self.StartZLocation`)) false false))
                      (:`then_1`
                        ;[1 0.3944 0.8064] Set initial life
                        (set `self.CurrentLife` (`self.BaseBarrierLife`))
                        ;[1 0.506 0.8554] Set off set rotation
                        (if (`KismetMathLibrary.RandomBoolWithWeight` 0.5)
                          (set `self.DirectionOfRotation` 1.0)
                          (else
                            (set `self.DirectionOfRotation` -1.0)))
                        (`SceneComponent.K2_SetWorldRotation` _staticmeshcomponent (`KismetMathLibrary.ComposeRotators` (* (`self.RotationOffSet`) (`self.DirectionOfRotation`)) (`SceneComponent.K2_GetComponentRotation` _staticmeshcomponent)) false false))))
                  (:`No`
                    (`self.K2_DestroyActor`))))
              (:`Multiplayer`
                (goto _label))
              (:`AI`
                (`self.CanBeCastAI` _ai_ref
                  (:`Yes`
                    (goto _label_2))
                  (:`No`
                    (`self.K2_DestroyActor`)))))))))))

(event `ClientPlayExplosion`
  (bind _returnvalue (`GameplayStatics.SpawnEmitterAtLocation` (`self.BarrierExplosion`) (`SceneComponent.K2_GetComponentLocation` (`self.ExplostionPoint`))))
  (`SceneComponent.SetWorldScale3D` _returnvalue (`self.EmitterScale`))
  (`GameplayStatics.SpawnSoundAttached` (`self.ExplosionSound`) _returnvalue "None" (0.0 0.0 0.0) (struct) "KeepRelativeOffset" false 1.0 1.0))

(event `/Game/Interfaces/BPI_TakeDamage.OnDamage`
  (params (Instigator :type "Actor Object Reference") (Damage :type Integer))
  ;[0.6301 1 0.94] On Barrier Damage
  (bind _output_get (set `self.CurrentLife` (- (`self.CurrentLife`) Damage)))
  (if (<= _output_get 0)
    (`self.ClientPlayExplosion`)
    (`self.SetLifeSpan` 0.2)))

(event `StartDestroying`
  (bind (_returnvalue_x _returnvalue_y _returnvalue_z) (`KismetMathLibrary.BreakVector` (`SceneComponent.K2_GetComponentLocation` (`self.EndPoint`))))
  (bind _returnvalue (`SceneComponent.K2_GetComponentLocation` (`self.StaticMeshComponent`)))
  ;[0.6185 1 0.6503] Destroy Barrier with timeline
  (`TimelineComponent.SetPlayRate` (`self.DestroyBarrierTimeLine`) (/ 1.0 (`KismetMathLibrary.FClamp` (`self.LifeTime`) 0.01 99999.0)))
  (set `self.StartLocationAtStartDestroying` _returnvalue)
  (set `self.EndlocationAtStartDestroying` (- _returnvalue (`KismetMathLibrary.MakeVector` 0.0 0.0 _returnvalue_z)))
  (bind (_direction _alpha) (`Timeline|DestroyBarrierTimeLine` :!via `PlayFromStart`)
    (:`Update`
      (`SceneComponent.K2_SetWorldLocation` (`self.StaticMeshComponent`) (`KismetMathLibrary.VLerp` (`self.StartLocationAtStartDestroying`) (`self.EndlocationAtStartDestroying`) _alpha) false false))
    (:`Finished`
      (`self.SetLifeSpan` 0.2))
    (:`PlayDestroyingSound`
      (`AudioComponent.Play` (`self.GrowSound`) 0.0))))

(event `SelfDestroyAfterTimeLife`
  ;[0.3904 0.6632 1] Self Destroy after a given time
  (`self.StartDestroying`))

(event `self.ReceiveDestroyed`
  (bind _returnvalue (`self.GetOwner` self))
  ;[0.3632 0.9602 1] Remove Barrier from the counter
  (if (`KismetSystemLibrary.DoesImplementInterface` _returnvalue "/Game/Interfaces/BPI_SpellRules.BPI_SpellRules_C")
    (message `/Game/Interfaces/BPI_SpellRules.RemoveBarrier` _returnvalue)))

(fn `BringDownBarrierAtZDirection`
  (params (DetaZ :type "Float (double-precision)"))
  (bind _returnvalue (`self.GetTransform`))
  ;[1 0.7759 0.6537] Bring Down the barrier by deltaZ
  (`self.K2_SetActorTransform` (`KismetMathLibrary.MakeTransform` (`KismetMathLibrary.MakeVector` (.x (.location _returnvalue)) (.y (.location _returnvalue)) (`KismetMathLibrary.FClamp` (- (.z (.location _returnvalue)) DetaZ) (`self.EndZLocation`) (`self.StartZLocation`))) (.rotation _returnvalue) (.scale _returnvalue))))

(fn `GiveQi`
  (params (InitialAmount :type Integer))
  (returns (ReturnAmount :type Integer) (GiveQiToOwner :type Boolean))
  (return (`KismetMathLibrary.Round` (* InitialAmount (`self.QiMultiplier`))) true))

(fn `GrowBarrierAtZDirection`
  (params (DeltaZ :type "Float (double-precision)" :default 0.0))
  (bind _returnvalue (`self.GetTransform`))
  ;[1 0.7759 0.6537] Grow the barrier by deltaZ
  (`self.K2_SetActorTransform` (`KismetMathLibrary.MakeTransform` (`KismetMathLibrary.MakeVector` (.x (.location _returnvalue)) (.y (.location _returnvalue)) (`KismetMathLibrary.FClamp` (+ (.z (.location _returnvalue)) DeltaZ) (`self.StartZLocation`) (`self.EndZLocation`))) (.rotation _returnvalue) (.scale _returnvalue))))

(fn `SetParametersFromDataTable`
  (params (Row :type Name))
  (locals (RowToText :type Text :default "NSLOCTEXT(\"\", \"C8D23B9649A22F06BCE868B9A4D548E9\", \"None\")"))
  (bind _returnvalue (`KismetTextLibrary.Conv_NameToText` Row))
  (bind _returnvalue_2 (`|GetDataTableRow` "/Game/GameData/BasicSpellsData.BasicSpellsData" Row)
    (:`then`
      (bind (_life _lifetime) (break `/Game/GameData/ClassesStructures/SBarriers` (`.Barriers_8_9FE1A1EF4F94B13142C316BED3BB7EA5` (break `/Game/GameData/RootStructures/SBasicSpells` _returnvalue_2))))
      (set `self.BaseBarrierLife` (`.BaseLife_2_C64370544D88120A2A098EADF4DE2C24` (break `/Game/GameData/SubStructures/SLife` _life)))
      (set `self.LifeTime` _lifetime))
    (:`RowNotFound`
      ;[1 0.3694 0.1989] Find error unless RowToText is equal None.
      (if (`KismetTextLibrary.NotEqual_TextText` _returnvalue (`local.RowToText`))
        (`KismetSystemLibrary.PrintText` (`|FormatText` "Error: Row {name} at data table for BasicSpells not found." _returnvalue))))))

(fn `UserConstructionScript`
  (`self.SetParametersFromDataTable` (`KismetStringLibrary.Conv_StringToName` (`|GetEnumeratorNameAsString` (`self.ElementalClass`)))))