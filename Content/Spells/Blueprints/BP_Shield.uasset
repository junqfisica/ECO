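; Elemental shield spell held by a motion-controller hand in single player or multiplayer, with base life read from a data table by element.
; Hits drain life; depletion briefly disables the hand's spell and destroys the shield.
; Hits from other owners pass penetration-scaled damage to the parent actor, and that multiplier also scales returned Qi.
; An optional timeline drag trails the shield toward the hand's spawn point using swept lerps.
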(event `ClientPlayAudio`
  (params (Audio :type "AudioComponent Object Reference"))
  ;[0.1874 1 0.2705] Replicate. Play Audio
  (`AudioComponent.Play` Audio 0.0))

(event `self.ReceiveBeginPlay`
  ;[1 0.3944 0.8064] Set initial life
  (set `self.CurrentLife` (`self.BaseShieldLife`))
  ;[0.4999 1 0.9901] Start main audio with a fade in
  (`self.ClientPlayAudioWithFadeIn` (`self.Cue_MainLoop`) 1.0)
  ;[0.5426 0.5431 1] Start drag
  (if (`self.shouldDrag`)
    (`KismetSystemLibrary.Delay` 0.2)
    (`self.StartDrag`)))

(event `ClientPlayAudioWithFadeIn`
  (params (PlayAudio :type "AudioComponent Object Reference") (FadeTime :type "Float (double-precision)"))
  ;[0.1874 1 0.2705] Replication. Make a fade in transition.
  (`AudioComponent.FadeIn` PlayAudio FadeTime 1.0 0.0))

(event `SetOffSet`
  (params (CastToHand :type "EControllerHand Enum"))
  ;[1 0.3638 0.8973] Set an off set for the Left/Right shield.
  (switch `EControllerHand` CastToHand
    (:`Left`
      (`|ExecutionSequence`
        (:`then_0`
          (`SceneComponent.K2_AddRelativeLocation` (`self.StaticMeshComponent`) (`self.LocationOffsetForLeftHand`) false false))
        (:`then_1`
          (`SceneComponent.K2_AddRelativeRotation` (`self.StaticMeshComponent`) (`self.RotationOffsetForLeftHand`) false false))))
    (:`Right`
      (`|ExecutionSequence`
        (:`then_0`
          (`SceneComponent.K2_AddRelativeLocation` (`self.StaticMeshComponent`) (`self.LocationOffsetForRightHand`) false false))
        (:`then_1`
          (`SceneComponent.K2_AddRelativeRotation` (`self.StaticMeshComponent`) (`self.RotationOffsetForRightHand`) false false))))))

(event `/Game/Interfaces/BPI_TakeDamage.OnDamage`
  (params (Instigator :type "Actor Object Reference") (Damage :type Integer))
  (bind _returnvalue (`ActorComponent.GetOwner` (`SceneComponent.GetAttachParent` (`self.StaticMeshComponent`))))
  (`|ExecutionSequence`
    (:`then_0`
      ;[0.6672 0.8883 1] For use on Tutorial
      (bind _asbp_motion_controller (cast `/Game/VirtualRealityBP/Blueprints/BP_MotionController` (`self.GetOwner`)))
      (`/Game/VirtualRealityBP/Blueprints/BP_MotionController.ShieldWasHit` _asbp_motion_controller))
    (:`then_1`
      ;[0.6301 1 0.94] On Shield Damage
      (bind _output_get (set `self.CurrentLife` (- (`self.CurrentLife`) Damage)))
      (if (<= _output_get 0)
        ;;[1 1 1] Deals with the Player
        (bind (_asbp_motion_controller_2 _asbp_mpmotion_controller) (`self.GetsPlayerHand`)
          (:`MotionController`
            (`/Game/VirtualRealityBP/Blueprints/BP_MotionController.DisableSpellTemporaly` _asbp_motion_controller_2 0.5)
            (`/Game/VirtualRealityBP/Blueprints/BP_MotionController.SetShakeHands` _asbp_motion_controller_2 0.0 0.0 false))
          (:`MPMotionController`
            (`/Game/VirtualRealityBP/Blueprints/BP_MPMotionController.DisableSpellTemporaly` _asbp_mpmotion_controller 0.5)
            (`/Game/VirtualRealityBP/Blueprints/BP_MPMotionController.SetShakeHands` _asbp_mpmotion_controller 0.0 0.0 false))
          (:`CastFailed`
            _))
        ;;[1 0.6961 0.6159] Destroy Shield after 0.1 secs
        (`self.SetLifeSpan` 0.1)))
    (:`then_2`
      (if (not (== (`self.GetOwner` (`self.GetOwner` Instigator)) (`self.GetOwner` (`self.GetOwner`))))
        ;[0.4999 1 0.9901] Deals with Damage and Qi Penetration
        (if (`KismetSystemLibrary.DoesImplementInterface` Instigator "/Game/Interfaces/BPI_HasPenetration.BPI_HasPenetration_C")
          (bind _penetration (message `/Game/Interfaces/BPI_HasPenetration.GetPenetration` Instigator (`self.ElementalClass`)))
          (set `self.QiMultiplier` _penetration)
          (if (`KismetSystemLibrary.DoesImplementInterface` _returnvalue "/Game/Interfaces/BPI_TakeDamage.BPI_TakeDamage_C")
            (message `/Game/Interfaces/BPI_TakeDamage.OnDamage` _returnvalue self (`KismetMathLibrary.Round` (* Damage _penetration)))))))))

(event `StartDrag`
  ;[0.6736 0.7742 0.79] Makes the shield drag. This is running on server and client.
  ;;[0.4999 1 0.9901] Check if is SP or MP
  (bind (_asbp_motion_controller _asbp_mpmotion_controller) (`self.GetsPlayerHand`)
    (:`MotionController`
      (set `self.ShieldSpawnPoint` (`/Game/VirtualRealityBP/Blueprints/BP_MotionController.ShieldSpawPoint` _asbp_motion_controller)))
    (:`MPMotionController`
      (set `self.ShieldSpawnPoint` (`/Game/VirtualRealityBP/Blueprints/BP_MPMotionController.ShieldSpawPoint` _asbp_mpmotion_controller))))
  ;;[0.23 0.23 0.23] Shield Position
  (set `self.StartLocation` (`SceneComponent.K2_GetComponentLocation` (`self.StaticMeshComponent`)))
  (`TimelineComponent.SetPlayRate` (`self.DragTimeLine`) (/ 1.0 (`self.DragTime`)))
  (bind (_direction _alpha) (`Timeline|DragTimeLine` :!via `PlayFromStart`)
    (:`Update`
      (`SceneComponent.K2_SetWorldLocation` (`self.StaticMeshComponent`) (`KismetMathLibrary.VLerp` (`self.StartLocation`) (`self.EndLocation`) _alpha) true false))
    (:`EndTime`
      ;;[0.23 0.23 0.23] Shield Position
      (set `self.StartLocation` (`SceneComponent.K2_GetComponentLocation` (`self.StaticMeshComponent`))))
    (:`StartTime`
      ;;[0.03008 0.315 0.1324] Hand's shield spawn point
      (set `self.EndLocation` (`SceneComponent.K2_GetComponentLocation` (`self.ShieldSpawnPoint`))))))

(fn `GiveQi`
  (params (InitialAmount :type Integer))
  (returns (ReturnAmount :type Integer) (GiveQiToOwner :type Boolean))
  (bind _returnvalue (`KismetMathLibrary.Round` (* InitialAmount (`self.QiMultiplier`))))
  (`KismetSystemLibrary.PrintText` (`|FormatText` "QiBack: {val}" _returnvalue))
  (return _returnvalue true))

(fn `SetParametersFromDataTable`
  (params (Row :type Name))
  (locals (RowToText :type Text :default "NSLOCTEXT(\"\", \"2B4AB39042402CFF5F8EAE887154FD87\", \"None\")"))
  (bind _returnvalue (`KismetTextLibrary.Conv_NameToText` Row))
  (bind _returnvalue_2 (`|GetDataTableRow` "/Game/GameData/BasicSpellsData.BasicSpellsData" Row)
    (:`then`
      (set `self.BaseShieldLife` (`.BaseLife_2_C64370544D88120A2A098EADF4DE2C24` (break `/Game/GameData/SubStructures/SLife` (`.Life_3_5B15C5B446300AD53ABB2496B8FE1C59` (break `/Game/GameData/ClassesStructures/SShields` (`.Shield_9_A017E3C34A058095EA6F9CA3C6C4B8CF` (break `/Game/GameData/RootStructures/SBasicSpells` _returnvalue_2))))))))
    (:`RowNotFound`
      ;[1 0.3694 0.1989] Find error unless RowToText is equal None.
      (if (`KismetTextLibrary.NotEqual_TextText` _returnvalue (`local.RowToText`))
        (`KismetSystemLibrary.PrintText` (`|FormatText` "Error: Row {name} at data table for BasicSpells not found." _returnvalue))))))

(fn `UserConstructionScript`
  (`self.SetParametersFromDataTable` (`KismetStringLibrary.Conv_StringToName` (`|GetEnumeratorNameAsString` (`self.ElementalClass`)))))