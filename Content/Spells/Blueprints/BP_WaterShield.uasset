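; Water shield spell actor with a partly physics-simulated mesh that draws water drops up from the ground.
; On BeginPlay it simulates the bodies below joint1, then spawns a batch of BP_Rising_Ground actors at random points and scales around its owner's location.
; Each drop takes the shield as its follow target and is destroyed when it overlaps the DetectWater component.
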(event `self.ReceiveBeginPlay`
  (`parent.ReceiveBeginPlay`)
  ;[1 1 1] Simulate lower joints
  (`SkeletalMeshComponent.SetAllBodiesBelowSimulatePhysics` (`self.Water_Shield`) (`KismetStringLibrary.Conv_StringToName` "joint1") true false)
  ;[0.004911 0 1] Spawn ground water
  (set `self.GroundLocation` (`self.K2_GetActorLocation` (`self.GetOwner`)))
  (`self.ServerSpawn Water From Ground`))

(event `ServerSpawn Water From Ground`
  ;[1 1 1] spawn Water drop
  (for _ (range 11)
    (bind _returnvalue (`|SpawnActorFromClass` "/Game/Spells/Blueprints/SupportBlueprints/BP_Rising_Ground.BP_Rising_Ground_C" (`KismetMathLibrary.MakeTransform` (`KismetMathLibrary.RandomPointInBoundingBox` (`self.GroundLocation`) (`KismetMathLibrary.MakeVector` 300.0 300.0)) (`KismetMathLibrary.RandomRotator` false) (`KismetMathLibrary.Conv_DoubleToVector` (`KismetMathLibrary.RandomFloatInRange` 0.1 1.0))) "Undefined" "OverrideRootScale" null self "NewEnumerator3"))
    (`KismetArrayLibrary.Array_Add` (`self.WaterFromGround`) _returnvalue)))

(event `self.DetectWater.OnComponentBeginOverlap`
  (params (OverlappedComponent :type "PrimitiveComponent Object Reference") (OtherActor :type "Actor Object Reference") (OtherComp :type "PrimitiveComponent Object Reference") (OtherBodyIndex :type Integer) (bFromSweep :type Boolean) (SweepResult :type "HitResult Structure (by ref)"))
  ;[1 1 1] destroys water drops
  (bind _asbp_rising_ground (cast `/Game/Spells/Blueprints/SupportBlueprints/BP_Rising_Ground` OtherActor))
  (`self.K2_DestroyActor` _asbp_rising_ground))

(fn `UserConstructionScript`
  (`parent.UserConstructionScript`))