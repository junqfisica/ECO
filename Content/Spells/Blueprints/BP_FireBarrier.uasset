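; BP_FireBarrier is a fire barrier spell Blueprint that keeps its particle effect at a fixed height.
; Each Tick compares the ParticleEffects world Z to KeepZLocationAt and, when it drifts beyond a small tolerance, teleports the component back to that height while preserving X and Y.
; BeginPlay and overlap events are inactive stubs, and the construction script only calls its parent.
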(event `self.ReceiveTick`
  (params (DeltaSeconds :type "Float (single-precision)"))
  (bind _particleeffects (`self.ParticleEffects`))
  (bind (_returnvalue_x _returnvalue_y _returnvalue_z) (`KismetMathLibrary.BreakVector` (`SceneComponent.K2_GetComponentLocation` _particleeffects)))
  ;[0.6108 0.8993 1] Keeps the particle effect on place
  (if (not (`KismetMathLibrary.NearlyEqual_FloatFloat` _returnvalue_z (`self.KeepZLocationAt`) 1.0))
    (`SceneComponent.K2_SetWorldLocation` _particleeffects (`KismetMathLibrary.MakeVector` _returnvalue_x _returnvalue_y (`self.KeepZLocationAt`)) false true)))

(fn `UserConstructionScript`
  (`parent.UserConstructionScript`))