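; BP_RisingGroundWater is a short-lived spell support projectile, named as rising ground water, that homes in on a waterball.
; Each Tick it faces the waterball and rebuilds its ProjectileMovement velocity along that rotation, scaling speed up slightly per frame.
; It destroys itself when the waterball reference is invalid, with a timer from BeginPlay as a safeguard cleanup.
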(event `self.ReceiveBeginPlay`
  ;[1 1 1] Safe guard to delete them
  (`KismetSystemLibrary.K2_SetTimerDelegate` (delegate `SelfDestroy`) 2.0))

(event `SelfDestroy`
  ;[1 1 1] Safe guard to delete them
  (`self.K2_DestroyActor`))

(event `self.ReceiveTick`
  (params (DeltaSeconds :type "Float (single-precision)"))
  (bind _waterballbp (`self.waterballBP`))
  ;[1 1 1] Homing to the waterball
  (`/Engine/EditorBlueprintResources/StandardMacros.IsValid` _waterballbp
    (:`Is Valid`
      (`self.K2_SetActorRotation` (`KismetMathLibrary.FindLookAtRotation` (`self.K2_GetActorLocation`) (`self.K2_GetActorLocation` _waterballbp)))
      (set `MovementComponent.Velocity` (* (`KismetMathLibrary.CreateVectorFromYawPitch` (.yaw (`self.K2_GetActorRotation`)) (.pitch (`self.K2_GetActorRotation`)) (`KismetMathLibrary.VSize` (`self.GetVelocity`))) 1.001) (`self.ProjectileMovement`)))
    (:`Is Not Valid`
      (`self.K2_DestroyActor`))))

(fn `UserConstructionScript`)