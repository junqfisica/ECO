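; Destructible rock barrier used by a spell, built on a destructible mesh component.
; Break plays a sound and applies heavy radius damage at the mesh's location to shatter it, then destroys the actor after a short timer.
; Each component fracture adds a strong constant radial force at the hit point to scatter the pieces.
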(event `self.ReceiveBeginPlay`
  (add `DestructibleComponent.OnComponentFracture` (`self.DM_RockTarget_DM`) (delegate `OnComponentFracture_Event_0`)))

(event `OnComponentFracture_Event_0`
  (params (HitPoint :type "Vector Structure (by ref)") (HitDirection :type "Vector Structure (by ref)"))
  (`PrimitiveComponent.AddRadialForce` (`self.DM_RockTarget_DM`) HitPoint 300.0 2000000.0 "RIF_Constant" false))

(event `Break`
  (bind _dm_rocktarget_dm (`self.DM_RockTarget_DM`))
  (`AudioComponent.Play` (`self.Audio`) 0.0)
  (`DestructibleComponent.ApplyRadiusDamage` _dm_rocktarget_dm 10000.0 (`SceneComponent.K2_GetComponentLocation` _dm_rocktarget_dm) 1000.0 1000.0 true)
  (`KismetSystemLibrary.K2_SetTimerDelegate` (delegate `Destroy`) 3.0))

(event `Destroy`
  (`self.K2_DestroyActor`))

(fn `UserConstructionScript`)