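; BP_Rising_Ground is a short-lived spell support projectile that homes in on a target actor, styled as rising Earth or Water material.
; The construction script uses the spawn-set Element to pick a random leaf or dirt effect for Earth, or a missile mesh and rising effect for Water.
; Tick re-aims velocity at the target with slight per-frame acceleration, destroying the actor if the target is invalid, with a lifespan as backup.
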(event `self.ReceiveBeginPlay`
  ;[1 1 1] Safe guard to delete them
  (`self.SetLifeSpan` 2.0))

(event `self.ReceiveTick`
  (params (DeltaSeconds :type "Float (single-precision)"))
  (bind _targettofollow (`self.TargetToFollow`))
  ;[1 1 1] Homing to the waterball
  (`/Engine/EditorBlueprintResources/StandardMacros.IsValid` _targettofollow
    (:`Is Valid`
      (`self.K2_SetActorRotation` (`KismetMathLibrary.FindLookAtRotation` (`self.K2_GetActorLocation`) (`self.K2_GetActorLocation` _targettofollow)))
      (set `MovementComponent.Velocity` (* (`KismetMathLibrary.CreateVectorFromYawPitch` (.yaw (`self.K2_GetActorRotation`)) (.pitch (`self.K2_GetActorRotation`)) (`KismetMathLibrary.VSize` (`self.GetVelocity`))) 1.001) (`self.ProjectileMovement`)))
    (:`Is Not Valid`
      (`self.K2_DestroyActor`))))

(fn `UserConstructionScript`
  (bind _raindrops (`self.Raindrops`))
  (bind _ball (`self.Ball`))
  (switch `/Game/VirtualRealityBP/Enumerates/EElementSelected` (`self.Element`)
    (:`NewEnumerator2`
      ;[0.2923 1 0.4974] Set up for Earth. Ps: Many default values works fine for Earth. If they change this node need to set them.
      (`|MultiGate` true
        (:`Out 0`
          (`ParticleSystemComponent.SetTemplate` _raindrops "/Game/Spells/Blueprints/SupportBlueprints/PFX_EarthLeafFromGround.PFX_EarthLeafFromGround"))
        (:`Out 1`
          (`ParticleSystemComponent.SetTemplate` _raindrops "/Game/Spells/Blueprints/SupportBlueprints/PFX_EarthDirtClumpFromGround.PFX_EarthDirtClumpFromGround"))))
    (:`NewEnumerator3`
      ;[0.278 0.4444 1] Set up for water.
      (`StaticMeshComponent.SetStaticMesh` _ball "/Game/Spells/Blueprints/SupportBlueprints/SM_WaterMissile.SM_WaterMissile")
      (`SceneComponent.SetRelativeScale3D` _ball (-0.17 -0.17 -0.17))
      (`SceneComponent.SetVisibility` (`self.Ball`) true false)
      (`ParticleSystemComponent.SetTemplate` (`self.Raindrops`) "/Game/Spells/Blueprints/SupportBlueprints/PFX_WaterRising.PFX_WaterRising"))))