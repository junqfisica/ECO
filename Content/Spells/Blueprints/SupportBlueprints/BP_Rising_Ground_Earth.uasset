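; BP_Rising_Ground_Earth is a short-lived earth spell projectile that draws a ground debris effect toward an earth ball.
; Its construction script randomly assigns a leaf or dirt clump particle template to the Raindrops component.
; Each tick it turns to face EarthBallBP and redirects its projectile velocity that way, slightly increasing speed.
; It destroys itself when the ball is invalid, with a lifespan set on BeginPlay as a safeguard.
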(event `self.ReceiveBeginPlay`
  ;[1 1 1] Safe guard to delete them
  (`self.SetLifeSpan` 1.0))

(event `self.ReceiveTick`
  (params (DeltaSeconds :type "Float (single-precision)"))
  (bind _earthballbp (`self.EarthBallBP`))
  ;[1 1 1] Homing to the waterball
  (`/Engine/EditorBlueprintResources/StandardMacros.IsValid` _earthballbp
    (:`Is Valid`
      (`self.K2_SetActorRotation` (`KismetMathLibrary.FindLookAtRotation` (`self.K2_GetActorLocation`) (`self.K2_GetActorLocation` _earthballbp)))
      (set `MovementComponent.Velocity` (* (`KismetMathLibrary.CreateVectorFromYawPitch` (.yaw (`self.K2_GetActorRotation`)) (.pitch (`self.K2_GetActorRotation`)) (`KismetMathLibrary.VSize` (`self.GetVelocity`))) 1.001) (`self.ProjectileMovement`)))
    (:`Is Not Valid`
      (`self.K2_DestroyActor`))))

(fn `UserConstructionScript`
  (bind _raindrops (`self.Raindrops`))
  (`|MultiGate` true
    (:`Out 0`
      (`ParticleSystemComponent.SetTemplate` _raindrops "/Game/Spells/Blueprints/SupportBlueprints/PFX_EarthLeafFromGround.PFX_EarthLeafFromGround"))
    (:`Out 1`
      (`ParticleSystemComponent.SetTemplate` _raindrops "/Game/Spells/Blueprints/SupportBlueprints/PFX_EarthDirtClumpFromGround.PFX_EarthDirtClumpFromGround"))))