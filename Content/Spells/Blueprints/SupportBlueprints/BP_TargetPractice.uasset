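; BP_TargetPractice is a spell target that registers itself as the player pawn's EnemyTarget and may randomly flip its mesh at BeginPlay.
; Rise plays audio and lifts the anchor on a timeline, then a short timer enables mesh physics with a radial impulse to shed rocks.
; OnDamage accumulates damage until a threshold, then calls TargetHit, spawns a breaking BP_RockBarrierDM in its place and destroys itself.
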(event `self.ReceiveBeginPlay`
  (bind _skeletalmesh (`self.SkeletalMesh`))
  (`|ExecutionSequence`
    (:`then_0`
      ;[0.02277 0.75 0.1359] Gets Player reference and set this actor (BP_TargetPractice) as the EnemyTarget.
      (bind _outactors (`GameplayStatics.GetAllActorsOfClass` "/Game/VirtualRealityBP/Blueprints/MotionControllerPawn.MotionControllerPawn_C"))
      (set `/Game/VirtualRealityBP/Blueprints/MotionControllerPawn.EnemyTarget` self (`|GetArrayItem` _outactors)))
    (:`then_1`
      (`|MultiGate` true
        (:`Out 1`
          (`/Engine/EditorBlueprintResources/StandardMacros.IsValid` _skeletalmesh
            (:`Is Valid`
              (`SceneComponent.K2_SetRelativeRotation` _skeletalmesh (struct :`Yaw` 180.0) false false))))))))

(event `Rise`
  (`AudioComponent.Play` (`self.Audio`) 0.0)
  (`KismetSystemLibrary.K2_SetTimerDelegate` (delegate `Make Rocks Fall`) 0.2)
  (`TimelineComponent.SetPlayRate` (`self.Movement`) 1.5)
  (bind (_direction _movement_in_z) (`Timeline|Movement`)
    (:`Update`
      (`SceneComponent.K2_SetRelativeLocation` (`self.Anchor`) (`KismetMathLibrary.MakeVector` 0.0 0.0 (`KismetMathLibrary.Lerp` 0.0 500.0 _movement_in_z)) false false))))

(event `Make Rocks Fall`
  (bind _skeletalmesh (`self.SkeletalMesh`))
  (`PrimitiveComponent.SetSimulatePhysics` _skeletalmesh true)
  (`PrimitiveComponent.AddRadialImpulse` _skeletalmesh (`SceneComponent.K2_GetComponentLocation` (`self.Arrow`)) 1000.0 55.0 "RIF_Constant" true))

(event `SpawnBreak BP`
  (`self.TargetHit`)
  (bind _returnvalue (`|SpawnActorFromClass` "/Game/Spells/Blueprints/SupportBlueprints/BP_RockBarrierDM.BP_RockBarrierDM_C" (`SceneComponent.K2_GetComponentToWorld` (`self.SkeletalMesh`)) "Undefined" "OverrideRootScale"))
  (`/Game/Spells/Blueprints/SupportBlueprints/BP_RockBarrierDM.Break` _returnvalue)
  (`self.K2_DestroyActor`))

(event `/Game/Interfaces/BPI_TakeDamage.OnDamage`
  (params (Instigator :type "Actor Object Reference") (Damage :type Integer))
  ;[0.5388 1 0.8583] This will be call when an attack hit this actor.
  (bind _output_get (set `self.Damage Taken` (+ Damage (`self.Damage Taken`))))
  (if (>= _output_get 200)
    (`self.SpawnBreak BP`)))

(fn `GetTargetComponent`
  (returns (Target :type "StaticMeshComponent Object Reference"))
  (return (`self.SMTarget`)))

(fn `UserConstructionScript`)