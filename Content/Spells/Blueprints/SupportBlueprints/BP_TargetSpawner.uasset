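; BP_TargetSpawner spawns BP_TargetPractice targets at one of five spawn locations and raises each one.
; StartSpawning picks the location through a looping MultiGate, whose random mode reads a Random flag that the first output sets to true.
; Each target's TargetHit event is bound back to the spawner, so a hit spawns the next target while ONOff is true.
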(event `Start Spawning`
  (`|MultiGate` (`self.Random`) true
    (:`Out 0`
      (set `self.SpawnTransform` (`SceneComponent.K2_GetComponentToWorld` (`self.SpawnLocation1`)))
      (set `self.Random` true))
    (:`Out 1`
      (set `self.SpawnTransform` (`SceneComponent.K2_GetComponentToWorld` (`self.SpawnLocation2`))))
    (:`Out 2`
      (set `self.SpawnTransform` (`SceneComponent.K2_GetComponentToWorld` (`self.SpawnLocation3`))))
    (:`Out 3`
      (set `self.SpawnTransform` (`SceneComponent.K2_GetComponentToWorld` (`self.SpawnLocation4`))))
    (:`Out 4`
      (set `self.SpawnTransform` (`SceneComponent.K2_GetComponentToWorld` (`self.SpawnLocation5`)))))
  (bind _returnvalue (`|SpawnActorFromClass` "/Game/Spells/Blueprints/SupportBlueprints/BP_TargetPractice.BP_TargetPractice_C" (`self.SpawnTransform`) "Undefined" "OverrideRootScale"))
  (`/Game/Spells/Blueprints/SupportBlueprints/BP_TargetPractice.Rise` _returnvalue)
  (add `/Game/Spells/Blueprints/SupportBlueprints/BP_TargetPractice.TargetHit` _returnvalue (delegate `TargetHit_Event_0`)))

(event `TargetHit_Event_0`
  (if (`self.ON/Off`)
    (`self.Start Spawning`)))

(fn `UserConstructionScript`)