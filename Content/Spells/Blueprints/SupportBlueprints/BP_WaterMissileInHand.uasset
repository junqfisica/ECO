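; Water ball effect for the in-hand stage of a water missile spell, growing through a scale timeline as water gathers from the ground.
; On BeginPlay it line-traces from the ball to a fixed world point below the origin to set a ground location.
; Two waves, half a second apart, spawn randomly placed and scaled BP_RisingGroundWater actors there, each referencing this ball.
; The sphere destroys those actors on overlap.
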(event `self.ReceiveBeginPlay`
  (`|ExecutionSequence`
    (:`then_0`
      (bind (_direction _newtrack_0) (`Timeline|WaterBall`)
        (:`Update`
          (`SceneComponent.SetRelativeScale3D` (`self.Ball`) (`KismetMathLibrary.Conv_DoubleToVector` _newtrack_0)))))
    (:`then_1`
      ;[1 1 1] Line Trace to ground and set random points in bounds
      (bind _outhit (`KismetSystemLibrary.LineTraceSingleForObjects` (`SceneComponent.K2_GetComponentLocation` (`self.Ball`)) (0.0 0.0 -1000.0) (`|MakeArray` "ObjectTypeQuery1" :!type "EObjectTypeQuery Enum")))
      (set `self.GroundLocation` (`.Location` (`GameplayStatics.BreakHitResult` _outhit)))
      (`self.Spawn Water From Ground`)
      (`KismetSystemLibrary.K2_SetTimerDelegate` (delegate `second round of water`) 0.5))))

(event `second round of water`
  ;[1 1 1] Line Trace to ground and set random points in bounds
  (`self.Spawn Water From Ground`))

(event `Spawn Water From Ground`
  (for _ (range 8)
    (bind _returnvalue (`|SpawnActorFromClass` "/Game/Spells/Blueprints/SupportBlueprints/BP_RisingGroundWater.BP_RisingGroundWater_C" (`KismetMathLibrary.MakeTransform` (`KismetMathLibrary.RandomPointInBoundingBox` (`self.GroundLocation`) (`KismetMathLibrary.MakeVector` 300.0 300.0)) (`KismetMathLibrary.RandomRotator` false) (`KismetMathLibrary.Conv_DoubleToVector` (`KismetMathLibrary.RandomFloatInRange` 0.1 0.8))) "Undefined" "OverrideRootScale"))
    (set `/Game/Spells/Blueprints/SupportBlueprints/BP_RisingGroundWater.waterballBP` self _returnvalue)))

(event `self.Sphere.OnComponentBeginOverlap`
  (params (OverlappedComponent :type "PrimitiveComponent Object Reference") (OtherActor :type "Actor Object Reference") (OtherComp :type "PrimitiveComponent Object Reference") (OtherBodyIndex :type Integer) (bFromSweep :type Boolean) (SweepResult :type "HitResult Structure (by ref)"))
  (bind _asbp_rising_ground_water (cast `/Game/Spells/Blueprints/SupportBlueprints/BP_RisingGroundWater` OtherActor))
  (`self.K2_DestroyActor` _asbp_rising_ground_water))

(fn `UserConstructionScript`)