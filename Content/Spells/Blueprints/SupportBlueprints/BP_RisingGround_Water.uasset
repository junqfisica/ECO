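; Water projectile support actor for spells that homes in on an actor assigned to TargetToFollow, apparently a water ball or water shield.
; Each Tick it turns toward the target and redirects its ProjectileMovement velocity along that facing, slightly increasing speed every frame.
; It destroys itself when the target is invalid, with a short lifespan set on BeginPlay as a fallback.
; An older ball-or-shield homing branch remains but never runs.
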(event `self.ReceiveBeginPlay`
  ;[1 1 1] Safe guard to delete them
  (`self.SetLifeSpan` 2.0))

(event `self.ReceiveTick`
  (params (DeltaSeconds :type "Float (single-precision)"))
  (`/Engine/EditorBlueprintResources/StandardMacros.IsValid` (`self.TargetToFollow`)
    (:`Is Valid`
      ;[1 1 1] Homing to the Actor
      (`self.K2_SetActorRotation` (`KismetMathLibrary.FindLookAtRotation` (`self.K2_GetActorLocation`) (`self.K2_GetActorLocation` (`self.TargetToFollow`))))
      (set `MovementComponent.Velocity` (* (`KismetMathLibrary.CreateVectorFromYawPitch` (.yaw (`self.K2_GetActorRotation`)) (.pitch (`self.K2_GetActorRotation`)) (`KismetMathLibrary.VSize` (`self.GetVelocity`))) 1.001) (`self.ProjectileMovement`)))
    (:`Is Not Valid`
      (`self.K2_DestroyActor`))))

(fn `UserConstructionScript`)