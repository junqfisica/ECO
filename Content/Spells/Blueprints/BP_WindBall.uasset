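; BP_WindBall is a wind spell Blueprint that handles the staged visual and audio changes of the wind ball.
; ChangeWindVisual uses EventTracker to pick the stage, fading the old client audio into a trigger cue plus the next stage's cue.
; The first change swaps the initial charge particle for the projectile particle and advances the tracker.
; The second re-triggers the projectile particle and sets its NumberOfSizeByLife parameter.
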(event `self.ReceiveBeginPlay`
  (`parent.ReceiveBeginPlay`))

(event `ChangeWindVisual`
  (bind _p_projectile (`self.P_Projectile`))
  ;[0.7846 0.5094 1] Trigger Events to change visual.
  (switch `int` (`self.EventTracker`)
    (:`0`
      (`self.ClientPlayAudioWithTransition` (`self.Cue_Stage1`) (`self.Cue_TrigerStage2`) 0.1)
      (`self.ClientPlayAudio` (`self.Cue_Stage2`))
      (`self.SwitchParticle` (`self.P_InitialCharge`) (`self.P_Projectile`))
      (`/Engine/EditorBlueprintResources/StandardMacros.IncrementInt` (`self.EventTracker`)))
    (:`1`
      (`self.ClientPlayAudioWithTransition` (`self.Cue_Stage2`) (`self.Cue_TrigerStage3`) 0.1)
      (`self.ClientPlayAudio` (`self.Cue_Stage3`))
      (`self.SwitchParticle` _p_projectile _p_projectile)
      (`ParticleSystemComponent.SetFloatParameter` (`self.P_Projectile`) "NumberOfSizeByLife" 1.0))))

(fn `UserConstructionScript`
  (`parent.UserConstructionScript`))