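; BP_TrainingMaster is a training master that makes an entrance by rising from the ground, then bobs continuously.
; RiseFromGround plays two audio components, activates the PMasterRise effect and breaks each valid entry in BreakableRocks.
; An eased MoveComponentTo lifts Anchor to the Dest component's location, then StartBounceLoop endlessly eases it between LoopBounceLocation and Dest.
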(event `RiseFromGround`
  (`AudioComponent.Play` (`self.Audio`) 0.0)
  (`AudioComponent.Play` (`self.Audio1`) 0.0)
  (`|ExecutionSequence`
    (:`then_0`
      (`ActorComponent.SetActive` (`self.P_MasterRise`) true false)
      (`KismetSystemLibrary.MoveComponentTo` (`self.Anchor`) (`SceneComponent.RelativeLocation` (`self.Dest`)) (struct) true true 2.0)
      (`self.StartBounceLoop`))
    (:`then_1`
      (for _array_element (`self.BreakableRocks`)
        (`/Engine/EditorBlueprintResources/StandardMacros.IsValid` _array_element
          (:`Is Valid`
            (`/Game/Meshes/Environment/Arch/BP_BreakableTile.Break` _array_element)))))))

(event `StartBounceLoop`
  (`KismetSystemLibrary.MoveComponentTo` (`self.Anchor`) (`SceneComponent.RelativeLocation` (`self.LoopBounceLocation`)) (struct) true true 2.0 :!label _label)
  (`KismetSystemLibrary.MoveComponentTo` (`self.Anchor`) (`SceneComponent.RelativeLocation` (`self.Dest`)) (struct) true true 2.0)
  (goto _label))

(fn `UserConstructionScript`)