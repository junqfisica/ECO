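; Advanced fire attack actor that builds on a parent attack class and gets a fixed lifetime on BeginPlay.
; Casting doubles the projectile component's scale before handing the velocity direction to the parent's cast logic.
; Unless end overlaps are ignored, it destroys itself when either of the owner's hands leaves the detector volume.
; A timeline-driven, authority-only spawn movement and a looping sound remain in the graph but never run.
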(event `self.ReceiveBeginPlay`
  (set `self.LifeTime` 15.0)
  (`parent.ReceiveBeginPlay`))

(event `self.CastAdvancedAttack`
  (params (`Velocity direction` :type "Vector Structure"))
  (bind _p_projectile (`self.P_Projectile`))
  ;[1 1 1] Override Event Cast Advanced Attack
  ;;[0.3747 0.9801 1] Increase scale of attack
  (`SceneComponent.SetRelativeScale3D` _p_projectile (* (`SceneComponent.RelativeScale3D` _p_projectile) 2.0))
  (`parent.CastAdvancedAttack` `Velocity direction`))

(event `self.VolumeDetector.OnComponentEndOverlap`
  (params (OverlappedComponent :type "PrimitiveComponent Object Reference") (OtherActor :type "Actor Object Reference") (OtherComp :type "PrimitiveComponent Object Reference") (OtherBodyIndex :type Integer))
  (bind _ownerhands (`self.OwnerHands`))
  ;[0.4222 1 0.7308] Destroy attack if hands get out of this volume
  (if (`self.IgnoreEndOverlap`)
    _
    (elif (or (== (`|GetArrayItem` _ownerhands) OtherActor) (== (`|GetArrayItem` _ownerhands 1) OtherActor))
      (`self.K2_DestroyActor`))))

(fn `UserConstructionScript`
  (`parent.UserConstructionScript`))