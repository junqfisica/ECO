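; BP_WaterProjectile is a water attack projectile that casts itself in a randomized direction biased toward its target and upward.
; On BeginPlay it flattens the vector from its static mesh to ProjectileTarget, normalizes it, then adds an upward component to form a cone axis.
; A random unit vector from that wide, roughly hemispherical cone is passed to CastAdvancedAttack.
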(event `self.ReceiveBeginPlay`
  (bind (_returnvalue_x _returnvalue_y) (`KismetMathLibrary.BreakVector` (- (`self.K2_GetActorLocation` (`self.ProjectileTarget`)) (`SceneComponent.K2_GetComponentLocation` (`self.StaticMeshComponent`)))))
  (bind (_returnvalue_x_2 _returnvalue_y_2) (`KismetMathLibrary.BreakVector2D` (`KismetMathLibrary.Normal2D` (`KismetMathLibrary.MakeVector2D` _returnvalue_x _returnvalue_y))))
  (`self.CastAdvancedAttack` (`KismetMathLibrary.RandomUnitVectorInCone` (`KismetMathLibrary.Normal` (`KismetMathLibrary.MakeVector` _returnvalue_x_2 _returnvalue_y_2 1.0)) 1.57)))

(fn `UserConstructionScript`
  (`parent.UserConstructionScript`))