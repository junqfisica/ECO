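; BP_AirAttackTailProjectile is a projectile, named for a tail air attack, that carries damage and Qi values.
; On BeginPlay, the server divides BaseDamage and GiveQi by NumberOfProjectiles, giving each projectile an equal share.
; The same authority branch starts a one-shot timer that destroys the actor after a short lifespan.
; The graph adds no movement or hit logic, and construction only calls the parent.
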(event `self.ReceiveBeginPlay`
  (bind _number_of_projectiles (`self.Number Of Projectiles`))
  ;[0 1 0.009438] LifeSpan
  (`/Engine/EditorBlueprintResources/ActorMacros.Switch Has Authority`
    (:`Authority`
      (set `self.BaseDamage` (/ (`self.BaseDamage`) _number_of_projectiles))
      (set `self.GiveQi` (/ (`self.GiveQi`) _number_of_projectiles))
      (`KismetSystemLibrary.K2_SetTimerDelegate` (delegate `Destroy Projectile`) 5.0))))

(event `Destroy Projectile`
  ;[0 1 0.009438] LifeSpan
  (`self.K2_DestroyActor`))

(fn `UserConstructionScript`
  (`parent.UserConstructionScript`))