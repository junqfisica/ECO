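; BP_GEarth01 is an earth object, apparently for an advanced attack, that rises into place when spawned.
; On BeginPlay it disables physics and collision, then a timeline lerps the mesh from a fixed low Z up to its placed location.
; When the rise finishes, it re-enables physics and collision, then, if its owner is a MotionControllerPawn, stores it as PlayerOwner and attaches a looping sound.
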(event `self.ReceiveBeginPlay`
  (bind _staticmeshcomponent (`self.StaticMeshComponent`))
  (bind _staticmeshcomponent_2 (`self.StaticMeshComponent`))
  (`parent.ReceiveBeginPlay`)
  (`|ExecutionSequence`
    (:`then_0`
      ;[0.3444 0.5013 1] Turn off physics and collision
      (`PrimitiveComponent.SetSimulatePhysics` _staticmeshcomponent false)
      (`PrimitiveComponent.SetCollisionEnabled` _staticmeshcomponent "NoCollision"))
    (:`then_1`
      ;[0.9487 1 0.5705] Set initial and final location to be played
      (bind _output_get (set `self.EndLocation` (`SceneComponent.K2_GetComponentLocation` (`self.StaticMeshComponent`))))
      (set `self.StartLocation` (`KismetMathLibrary.MakeVector` (.x _output_get) (.y _output_get) -50.0)))
    (:`then_2`
      (`TimelineComponent.SetPlayRate` (`self.SpawnEarth`) 1.0)
      (bind (_direction _alpha) (`Timeline|SpawnEarth` :!via `PlayFromStart`)
        (:`Update`
          ;[0.4549 1 0.7631] Lerp Location from start to end
          (`SceneComponent.K2_SetWorldLocation` (`self.StaticMeshComponent`) (`KismetMathLibrary.VLerp` (`self.StartLocation`) (`self.EndLocation`) _alpha) false false))
        (:`Finished`
          ;[0.5925 1 0.9701] Sets possible Owner
          (`PrimitiveComponent.SetSimulatePhysics` _staticmeshcomponent_2 true)
          (`PrimitiveComponent.SetCollisionEnabled` _staticmeshcomponent_2 "QueryAndPhysics")
          (bind _asmotion_controller_pawn (cast `/Game/VirtualRealityBP/Blueprints/MotionControllerPawn` (`self.GetOwner`)))
          (set `self.PlayerOwner` _asmotion_controller_pawn)
          (`GameplayStatics.SpawnSoundAttached` (`self.LoopingSound`) (`self.StaticMeshComponent`) "None" (0.0 0.0 0.0) (struct) "KeepRelativeOffset" true))))))

(fn `UserConstructionScript`
  (`parent.UserConstructionScript`))