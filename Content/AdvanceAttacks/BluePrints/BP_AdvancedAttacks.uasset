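; Qi-costed projectile attack actor, configured per attack ID from a data table, that homes on a target.
; On spawn it charges the owner Qi or destroys itself; casting launches it by physics impulse, then switches to homing movement.
; A timer scales homing acceleration by inverse squared distance and redirects velocity once near the target.
; Hits, ignoring the owner's hands, deal damage, pass Qi to the owner and explode.
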(event `self.ReceiveBeginPlay`
  (bind _owneractor (`self.OwnerActor`))
  (bind _output_get (set `self.OwnerActor` (`self.GetOwner`)))
  (`|ExecutionSequence`
    (:`then_0`
      (`KismetSystemLibrary.Delay` (`self.LifeTime`))
      (`self.K2_DestroyActor`))
    (:`then_1`
      (if (`KismetSystemLibrary.DoesImplementInterface` _output_get "/Game/Interfaces/BPI_HasQi.BPI_HasQi_C")
        ;[0.278 0.4444 1] Check if owner has enought Qi
        (bind _return (message `/Game/Interfaces/BPI_HasQi.HasEnoughQi` _owneractor (`self.QiCost`)))
        (if _return
          ;[0.1874 1 0.2705] Consume Qi
          (message `/Game/Interfaces/BPI_HasQi.ConsumeQi` (`self.OwnerActor`) (`self.QiCost`))
          (else
            ;[0.59 0.6845 1] Play Qi bar animation on Players.
            (message `/Game/Interfaces/BPI_HasQi.PlayNotEnoghtQiAnim` _owneractor)
            ;[1 0.3694 0.1989] Don't have enough Qi. Destroy Actor.
            (`self.K2_DestroyActor`)))
        (else
          (`KismetSystemLibrary.PrintString` "Error: Owner don't implement Interface HasQi."))))))

(event `ClientPlayExplosion`
  ;[1 1 1] Replicates sound effects when AdvancedAttack hit
  (`self.DestroyActorAndCastEmitter` (`self.ExplosionEmmiter`) (`self.ImpactSound`)))

(event `CastAdvancedAttack`
  (params (`Velocity direction` :type "Vector Structure"))
  (bind _staticmeshcomponent (`self.StaticMeshComponent`))
  (bind _staticmeshcomponent_2 (`self.StaticMeshComponent`))
  (`/Engine/EditorBlueprintResources/StandardMacros.DoOnce` false
    (:`Completed`
      (set `self.VelocityDirection` (`KismetMathLibrary.Normal` `Velocity direction`))
      ;[0.635 0.635 0.635] Player cast Node
      (`GameplayStatics.SpawnSoundAttached` (`self.SoundOnCast`) (`self.StaticMeshComponent`) "None" (0.0 0.0 0.0) (struct) "KeepRelativeOffset" true)
      (`/Engine/EditorBlueprintResources/StandardMacros.IsValid` (`self.ProjectileTarget`)
        (:`Is Valid`
          ;[1 0.9184 0.3915] Set physics to true and add velocity
          (set `self.BaseSpeed` (`KismetMathLibrary.FClamp` (* (`self.SpeedFactor`) (`self.BaseSpeed`)) 500.0 4000.0))
          (`PrimitiveComponent.SetSimulatePhysics` _staticmeshcomponent true)
          (`PrimitiveComponent.AddImpulse` _staticmeshcomponent (* (`self.VelocityDirection`) (`self.BaseSpeed`)) "None" true)
          (`KismetSystemLibrary.Delay` 0.1) ; Necessary to cause a small delay
          (`|ExecutionSequence`
            (:`then_0`
              ;[0.6756 0.7708 1] Set Homing Missile
              (bind _returnvalue (`PrimitiveComponent.GetPhysicsLinearVelocity` _staticmeshcomponent_2 "None"))
              (set `self.InitialVelocity` _returnvalue))
            (:`then_1`
              (`PrimitiveComponent.SetSimulatePhysics` _staticmeshcomponent_2 false))
            (:`then_2`
              (`SceneComponent.K2_SetWorldRotation` :`self` _staticmeshcomponent_2)
              (`self.SetHomingMissile` (`self.InitialVelocity`)
                (:`then`
                  (set `self.BaseAcceleration` (* (`self.GetAccelerationFromBaseSpeed`) (`self.Rescale`)))
                  (bind _returnvalue_2 (`KismetSystemLibrary.K2_SetTimerDelegate` (delegate `ModifyVelocity`) 0.05 true))
                  (set `self.ModifyVelocityTimeHandler` _returnvalue_2))
                (:`Fail`
                  (`KismetSystemLibrary.PrintString` "Fail to set homing missile target. Your target do not implement the interface IsTargetable"))))))
        (:`Is Not Valid`
          (`KismetSystemLibrary.PrintText` "No target found"))))))

(event `ModifyVelocity`
  ;[1 0.8467 0.5559] Modify Velocity Event Node
  (if (`KismetSystemLibrary.K2_IsTimerActiveHandle` (`self.ModifyVelocityTimeHandler`))
    ;;[0.1874 1 0.2705] Check if target is still there.
    (`/Engine/EditorBlueprintResources/StandardMacros.IsValid` (`self.ProjectileTarget`)
      (:`Is Valid`
        (bind _returnvalue (`PrimitiveComponent.GetPhysicsLinearVelocity` (`self.StaticMeshComponent`) "None"))
        (set `self.ProjectileVelocity` _returnvalue)
        (set `ProjectileMovementComponent.HomingAccelerationMagnitude` (/ (`self.BaseAcceleration`) (+ (`KismetMathLibrary.VSizeSquared` (- (`self.K2_GetActorLocation` (`self.ProjectileTarget`)) (`SceneComponent.K2_GetComponentLocation` (`self.StaticMeshComponent`)))) 1.0)) (`self.ProjectileMovement`))
        (`self.IsProjectileCloseToTarget`
          (:`Yes`
            (if (not (`self.isInitialVelocityReset`))
              ;;[0.9086 1 0.6564] Change velocity to target's direction
              (`ProjectileMovementComponent.SetVelocityInLocalSpace` (`self.ProjectileMovement`) (* (`KismetMathLibrary.Normal` (- (`self.K2_GetActorLocation` (`self.ProjectileTarget`)) (`SceneComponent.K2_GetComponentLocation` (`self.StaticMeshComponent`)))) (`KismetMathLibrary.VSize` (`self.ProjectileVelocity`))))
              (set `self.isInitialVelocityReset` true)))))
      (:`Is Not Valid`
        (`KismetSystemLibrary.K2_ClearAndInvalidateTimerHandle` (`self.ModifyVelocityTimeHandler`))))))

(event `self.StaticMeshComponent.OnComponentHit`
  (params (HitComponent :type "PrimitiveComponent Object Reference") (OtherActor :type "Actor Object Reference") (OtherComp :type "PrimitiveComponent Object Reference") (NormalImpulse :type "Vector Structure") (Hit :type "HitResult Structure (by ref)"))
  (bind _ownerhands (`self.OwnerHands`))
  (if (not (or (== OtherActor (`|GetArrayItem` _ownerhands)) (== OtherActor (`|GetArrayItem` _ownerhands 1))))
    (set `self.ActorHitByAttack` OtherActor)
    (`|ExecutionSequence`
      (:`then_0`
        ;[0.7602 1 0.6404] Call OnDamage if the actor has the BPI_TakeDamage implement.
        (if (`KismetSystemLibrary.DoesImplementInterface` (`self.ActorHitByAttack`) "/Game/Interfaces/BPI_TakeDamage.BPI_TakeDamage_C")
          (message `/Game/Interfaces/BPI_TakeDamage.OnDamage` (`self.ActorHitByAttack`) self (`self.BaseDamage`))))
      (:`then_1`
        (`KismetSystemLibrary.Delay` 0.01) ; To make sure OnDamage runs \neverything first. Only for security.
        (`|ExecutionSequence`
          (:`then_0`
            ;[0.6377 0.8887 1] Call Recive Qi to give the players or the AI certain amount of Qi
            ;;[0.5503 0.59 0.4513] If hit actor implements GiveQi interface
            (if (`KismetSystemLibrary.DoesImplementInterface` (`self.ActorHitByAttack`) "/Game/Interfaces/BPI_GiveQi.BPI_GiveQi_C")
              ;;[0.5801 0.6921 1] Gets the amount of Qi recived
              (bind (_returnamount _giveqitoowner) (message `/Game/Interfaces/BPI_GiveQi.GiveQi` (`self.ActorHitByAttack`) (`self.GiveQi`)))
              (`|ExecutionSequence`
                (:`then_0`
                  ;;[1 0.6561 0.8575] Owner recives Qi
                  (if (`KismetSystemLibrary.DoesImplementInterface` (`self.OwnerActor`) "/Game/Interfaces/BPI_reciveQi.BPI_ReciveQi_C")
                    (message `/Game/Interfaces/BPI_reciveQi.ReciveQi` (`self.OwnerActor`) _returnamount))))))
          (:`then_1`
            ;[1 0.5601 0.5302] Cast Explosion on hit
            (`self.ClientPlayExplosion`)))))))

(fn `DestroyActorAndCastEmitter`
  (params (Emitter :type "ParticleSystem Object Reference") (Sound :type "SoundBase Object Reference"))
  (`/Engine/EditorBlueprintResources/StandardMacros.DoOnce` false
    (:`Completed`
      (bind _returnvalue (`GameplayStatics.SpawnEmitterAtLocation` Emitter (`SceneComponent.K2_GetComponentLocation` (`self.StaticMeshComponent`))))
      (`GameplayStatics.SpawnSoundAttached` Sound _returnvalue "None" (0.0 0.0 0.0) (struct) "KeepRelativeOffset" false 1.0 0.4)
      (`self.K2_DestroyActor`))))

(fn `GetAccelerationFromBaseSpeed`
  (returns (BaseAcceleration :type "Float (double-precision)"))
  (return (+ (* (`self.BaseSpeed`) 0.00045) 0.18)))

(fn `GetPenetration`
  (params (HitAt :type "/Game/VirtualRealityBP/Enumerates/EElementSelected Enum" :default "NewEnumerator0"))
  (returns (Penetration :type "Float (double-precision)"))
  (switch `/Game/VirtualRealityBP/Enumerates/EElementSelected` HitAt
    (:`NewEnumerator0`
      (return 0.0))
    (:`NewEnumerator1`
      (return (`self.FirePenetration`)))
    (:`NewEnumerator2`
      (return (`self.EarthPenetration`)))
    (:`NewEnumerator3`
      (return (`self.WaterPenetration`)))
    (:`NewEnumerator4`
      (return (`self.AirPenetration`)))))

(fn `SetParametersFromDataTable`
  (params (Row :type Name))
  (locals (RowToText :type Text :default "NSLOCTEXT(\"\", \"D9E4EF0F492E2755DA7912BFC410966C\", \"None\")"))
  (bind _returnvalue (`KismetTextLibrary.Conv_NameToText` "None"))
  (bind _returnvalue_2 (`|GetDataTableRow` "/Game/GameData/AdvancedAttackData.AdvancedAttackData" Row)
    (:`then`
      (bind (_damages _qicust _giveqi _projectile) (break `/Game/GameData/RootStructures/SAdvanceAttacks` _returnvalue_2))
      (bind (_basedamage _firepenetration _waterpenetration _earthpenetration _airpenetration) (break `/Game/GameData/SubStructures/SDamage` _damages))
      (set `self.BaseDamage` _basedamage)
      (set `self.FirePenetration` _firepenetration)
      (set `self.WaterPenetration` _waterpenetration)
      (set `self.EarthPenetration` _earthpenetration)
      (set `self.AirPenetration` _airpenetration)
      (set `self.QiCost` _qicust)
      (set `self.GiveQi` _giveqi)
      (bind (_basespeed _maxspeedallow) (break `/Game/GameData/SubStructures/SProjectile` _projectile))
      (set `self.BaseSpeed` _basespeed)
      (set `self.MaxSpeedAllow` _maxspeedallow))
    (:`RowNotFound`
      ;[1 0.3694 0.1989] Find error unless RowToText is equal None.
      (if (`KismetTextLibrary.NotEqual_TextText` _returnvalue (`local.RowToText`))
        (`KismetSystemLibrary.PrintText` (`|FormatText` "Error: Row {name} at data table AdvancedAttack not found." _returnvalue))))))

(fn `UserConstructionScript`
  (locals (DamageTrack :type Name :default "PercentDamage") (ScaleTrack :type Name :default "PercentScale"))
  (`self.SetParametersFromDataTable` (`KismetStringLibrary.Conv_StringToName` (`|GetEnumeratorNameAsString` (`self.MyId`)))))