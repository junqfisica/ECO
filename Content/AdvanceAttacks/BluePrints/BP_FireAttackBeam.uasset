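; BP_FireAttackBeam is an attack beam actor that stretches out, holds, then retracts and destroys itself, reusing air-attack parts (wind stream mesh, tail projectile).
; One timeline scales the arrow forward, then plays in reverse after a delay to detach the actor and shrink the stream mesh.
; Meanwhile, a server-only looping timer spawns projectiles until retraction begins, passing a count derived from effect time and spawn rate.
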(event `Shoot Projectile`
  ;[0.5113 0.2222 1] Shoots Projectile. Only Server shoots
  (if (not (`self.Retracting`))
    (`|SpawnActorFromClass` "/Game/AdvanceAttacks/BluePrints/BP_AirAttackTailProjectile.BP_AirAttackTailProjectile_C" (`SceneComponent.K2_GetComponentToWorld` (`self.ShootProjectileLocation`)) "Undefined" "OverrideRootScale" null (`self.Number of Projectiles`) null (`self.OwnerHands`) null)))

(event `self.ReceiveBeginPlay`
  (`|ExecutionSequence`
    (:`then_0`
      ;[0.5113 0.2222 1] Shoots Projectile. Only Server shoots
      (`/Engine/EditorBlueprintResources/ActorMacros.Switch Has Authority`
        (:`Authority`
          (set `self.Number of Projectiles` (`KismetMathLibrary.Round` (/ (`self.Effect Time`) (`self.Projectile Spawn Rate`))))
          (`KismetSystemLibrary.K2_SetTimerDelegate` (delegate `Shoot Projectile`) (`self.Projectile Spawn Rate`) true))))
    (:`then_1`
      (`TimelineComponent.SetPlayRate` (`self.Timeline_0`) (/ 1.0 (`self.Effect Time`)))
      ;[0.5569 1 0] Scale/Grow/Retract
      (bind (_direction _alpha) (`Timeline|Timeline_0` :!via `PlayFromStart` :!label _label)
        (:`Update`
          (switch `ETimelineDirection` _direction
            (:`Forward`
              (`SceneComponent.SetRelativeScale3D` (`self.Arrow`) (`KismetMathLibrary.VLerp` (1.0 1.0 1.0) (50.0 1.0 1.0) _alpha)))
            (:`Backward`
              (`|ExecutionSequence`
                (:`then_0`
                  (`/Engine/EditorBlueprintResources/StandardMacros.DoOnce` false
                    (:`Completed`
                      (`self.K2_DetachFromActor` self "KeepWorld" "KeepWorld" "KeepWorld"))))
                (:`then_1`
                  (`SceneComponent.SetRelativeScale3D` (`self.SM_WindStream`) (`KismetMathLibrary.VLerp` (0.0 0.0 0.0) (1.0 1.0 1.0) _alpha)))))))
        (:`Finished`
          ;[1 0 0.007957] Retract or Destroy
          (if (`self.Retracting`)
            (`self.K2_DestroyActor`)
            (else
              (`self.Retract`))))))))

(event `Retract`
  ;[0.4255 1 0.7857] Retract
  (`KismetSystemLibrary.Delay` (`self.Effect Time while fully extened`))
  (set `self.Retracting` true)
  (goto _label :!via `Reverse`))

(fn `UserConstructionScript`)