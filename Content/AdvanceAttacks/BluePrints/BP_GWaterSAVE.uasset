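; Water attack actor that raises a water spout below its spawn point, launches a water projectile, then shrinks away and destroys itself.
; BeginPlay line-traces downward to place the barrier shape and disables physics and collision on the static mesh.
; The SpawnWater timeline spawns BP_WaterProjectile on the authority mid-play, passing along target and hands, then triggers shrinking on finish.
; Timeline_0 scales the meshes and plays in reverse for the shrink before destruction.
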(event `self.ReceiveBeginPlay`
  (bind _staticmeshcomponent (`self.StaticMeshComponent`))
  (bind _visiblemesh (`self.VisibleMesh`))
  (bind _returnvalue (`SceneComponent.K2_GetComponentLocation` (`self.P_Projectile`)))
  (bind (_returnvalue_location _returnvalue_rotation) (`KismetMathLibrary.BreakTransform` (`SceneComponent.K2_GetComponentToWorld` (`self.StaticMeshComponent`))))
  (`parent.ReceiveBeginPlay`)
  ;[1 1 1] (Ian)Find location for mesh
  (bind _outhit (`KismetSystemLibrary.LineTraceSingle` _returnvalue (`KismetMathLibrary.MakeVector` (.x _returnvalue) (.y _returnvalue) (* (.z _returnvalue) -1000.0)) "TraceTypeQuery1"))
  (bind _output_get (set `self.SpawnMeshLocation` (`.Location` (`GameplayStatics.BreakHitResult` _outhit))))
  (`SceneComponent.K2_SetWorldLocation` (`self.WIndBarrierShape`) _output_get false false)
  (`/Engine/EditorBlueprintResources/StandardMacros.IsValid` self
    (:`Is Valid`
      (`|ExecutionSequence`
        (:`then_0`
          ;[0.3444 0.5013 1] Turn off physics and collision
          (`PrimitiveComponent.SetSimulatePhysics` _staticmeshcomponent false)
          (`PrimitiveComponent.SetCollisionEnabled` _staticmeshcomponent "NoCollision")
          (set `self.InitialScale` (`SceneComponent.K2_GetComponentScale` (`self.StaticMeshComponent`))))
        (:`then_1`
          (`TimelineComponent.SetPlayRate` (`self.SpawnWater`) 0.5)
          (bind (_direction _scalefactor) (`Timeline|SpawnWater` :!via `PlayFromStart`)
            (:`Finished`
              (`self.Shrink water spout`))
            (:`CastProjectile`
              (`/Engine/EditorBlueprintResources/ActorMacros.Switch Has Authority`
                (:`Authority`
                  (`|SpawnActorFromClass` "/Game/AdvanceAttacks/BluePrints/BP_WaterProjectile.BP_WaterProjectile_C" (`KismetMathLibrary.MakeTransform` _returnvalue_location _returnvalue_rotation) "Undefined" "OverrideRootScale" (`self.GetOwner`) (`self.ProjectileTarget`) (`self.OwnerHands`)))))))
        (:`then_2`
          ;[1 1 1] (ian)Scales down and changes material parameter
          (bind (_direction_2 _scale _scaledownfast) (`Timeline|Timeline_0` :!label _label)
            (:`Update`
              (`SceneComponent.SetRelativeScale3D` (`self.WIndBarrierShape`) (`KismetMathLibrary.MakeVector` 1.0 1.0 _scale))
              (if (`self.Shrinking`)
                (`SceneComponent.SetRelativeScale3D` _visiblemesh (`KismetMathLibrary.Conv_DoubleToVector` _scaledownfast))
                (else
                  (`SceneComponent.SetRelativeScale3D` _visiblemesh (`KismetMathLibrary.Conv_DoubleToVector` _scale)))))
            (:`Finished`
              (if (`self.Shrinking`)
                (`self.K2_DestroyActor`)))))))))

(event `Shrink water spout`
  ;[1 1 1] (ian)Scales down and changes material parameter
  (set `self.Shrinking` true)
  (goto _label :!via `Reverse`))

(fn `UserConstructionScript`
  (`parent.UserConstructionScript`)
  (bind _returnvalue (`PrimitiveComponent.CreateDynamicMaterialInstance` (`self.StaticMeshComponent`) 0 "/Game/ParticleSystems/Defences/Water/Mat_BoxWaterwall_ADV_Attack.Mat_BoxWaterwall_ADV_Attack"))
  (bind _output_get (set `self.NewVar_0` _returnvalue))
  (`MaterialInstanceDynamic.SetScalarParameterValue` _output_get "Opacity" 0.3)
  (`SceneComponent.K2_AttachToComponent` (`self.Tip_PFX`) (`self.PFX_Anchor`) "None" "SnapToTarget" "SnapToTarget" "KeepRelative" true))