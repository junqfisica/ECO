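; Prototype air attack actor that grows a wind stream, then shrinks it away and destroys itself.
; On BeginPlay the GrowAirCylinder timeline stretches the Arrow component along X, then calls Retract on finish.
; Retract, also callable mid-growth, deactivates the particle stream and reverses the same timeline.
; While retracting, the actor detaches once from its parent and a second track uniformly scales the wind mesh until destruction.
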(event `self.ReceiveBeginPlay`
  (bind (_direction _newtrack_0 _newtrack_1) (`Timeline|Grow Air Cylinder` :!label _label)
    (:`Update`
      (if (`self.Retracting`)
        (`|ExecutionSequence`
          (:`then_0`
            (`/Engine/EditorBlueprintResources/StandardMacros.DoOnce` false
              (:`Completed`
                (`self.K2_DetachFromActor` self "KeepWorld" "KeepWorld" "KeepWorld"))))
          (:`then_1`
            (`SceneComponent.SetRelativeScale3D` (`self.SM_WindStream`) (`KismetMathLibrary.MakeVector` _newtrack_1 _newtrack_1 _newtrack_1))))
        (else
          (`SceneComponent.SetRelativeScale3D` (`self.Arrow`) (`KismetMathLibrary.MakeVector` _newtrack_0 1.0 1.0)))))
    (:`Finished`
      (if (`self.Retracting`)
        (`self.K2_DestroyActor`)
        (else
          (`self.Retract`))))))

(event `Retract`
  (set `self.Retracting` true)
  (`ActorComponent.SetActive` (`self.P_WindAdvancedAttackStream`) false false)
  (goto _label :!via `Reverse`))

(fn `UserConstructionScript`)