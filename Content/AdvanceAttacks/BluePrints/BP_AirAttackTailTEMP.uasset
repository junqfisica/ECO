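; Temporary air attack tail actor that extends a wind stream while firing tail projectiles, then retracts and destroys itself.
; On BeginPlay it derives the projectile count from effect time and spawn rate, then starts a looping spawn timer.
; A timeline scaled to the effect time stretches the Arrow forward.
; Its reverse pass stops projectiles and particles, detaches the actor once and shrinks the stream mesh.
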(event `Shoot Projectile`
  ;[0.5113 0.2222 1] Shoots Projectile
  (if (not (`self.Retracting`))
    (`|SpawnActorFromClass` "/Game/AdvanceAttacks/BluePrints/BP_AirAttackTailProjectile.BP_AirAttackTailProjectile_C" (`SceneComponent.K2_GetComponentToWorld` (`self.ShootProjectileLocation`)) "Undefined" "OverrideRootScale" null (`self.Number of Projectiles`) (0.0 0.0 0.0) null (`self.OwnerHands`))))

(event `self.ReceiveBeginPlay`
  (set `self.Number of Projectiles` (`KismetMathLibrary.Round` (/ (`self.Effect Time`) (`self.Projectile Spawn Rate`))))
  (`|ExecutionSequence`
    (:`then_0`
      ;[0.5113 0.2222 1] Shoots Projectile
      (`KismetSystemLibrary.K2_SetTimerDelegate` (delegate `Shoot Projectile`) (`self.Projectile Spawn Rate`) true))
    (:`then_1`
      (`TimelineComponent.SetPlayRate` (`self.Grow Air Cylinder`) (/ 1.0 (`self.Effect Time`)))
      ;[0.5569 1 0] Scale/Grow/Retract
      (bind (_direction _alpha) (`Timeline|Grow Air Cylinder` :!via `PlayFromStart` :!label _label)
        (:`Update`
          (switch `ETimelineDirection` _direction
            (:`Forward`
              (`SceneComponent.SetRelativeScale3D` (`self.Arrow`) (`KismetMathLibrary.VLerp` (1.0 1.0 1.0) (50.0 1.0 1.0) _alpha)))
            (:`Backward`
              (`|ExecutionSequence`
                (:`then_0`
                  (`/Engine/EditorBlueprintResources/StandardMacros.DoOnce` false
                    (:`Completed`
                      (`self.K2_DetachFromActor` self "KeepWorld" "KeepWorld" "KeepWorld"))))
                (:`then_1`
                  (`SceneComponent.SetRelativeScale3D` (`self.SM_WindStream`) (`KismetMathLibrary.VLerp` (0.0 0.0 0.0) (1.0 1.0 1.0) _alpha)))))))
        (:`Finished`
          ;[1 0 0.007957] Retract or Destroy
          (if (`self.Retracting`)
            (`self.K2_DestroyActor`)
            (else
              (`self.Retract`))))))))

(event `Retract`
  ;[0.4255 1 0.7857] Retract
  (set `self.Retracting` true)
  (`ActorComponent.SetActive` (`self.P_WindAdvancedAttackStream`) false false)
  (goto _label :!via `Reverse`))

(fn `UserConstructionScript`
  (`parent.UserConstructionScript`))