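; BP_FireAttackTail is a short-lived tail attack stream that grows, fires projectiles, then retracts and destroys itself, using wind/air components despite its Fire name.
; A looping timer spawns BP_AirAttackTailProjectile at ShootProjectileLocation until retraction begins.
; The GrowAirCylinder timeline stretches the Arrow along X, then reverses on finish.
; Retracting deactivates the wind particles, detaches the actor once and scales SMWindStream uniformly from a second track.
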(event `Shoot Projectile`
  ;[0.5113 0.2222 1] Shoots Projectile
  (if (not (`self.Retracting`))
    (`|SpawnActorFromClass` "/Game/AdvanceAttacks/BluePrints/BP_AirAttackTailProjectile.BP_AirAttackTailProjectile_C" (`SceneComponent.K2_GetComponentToWorld` (`self.ShootProjectileLocation`)) "Undefined" "OverrideRootScale")))

(event `self.ReceiveBeginPlay`
  (`|ExecutionSequence`
    (:`then_0`
      ;[0.5113 0.2222 1] Shoots Projectile
      (`KismetSystemLibrary.K2_SetTimerDelegate` (delegate `Shoot Projectile`) 0.2 true))
    (:`then_1`
      ;[0.5569 1 0] Scale/Grow/Retract
      (bind (_direction _newtrack_0 _newtrack_1) (`Timeline|Grow Air Cylinder` :!label _label)
        (:`Update`
          (if (`self.Retracting`)
            (`|ExecutionSequence`
              (:`then_0`
                (`/Engine/EditorBlueprintResources/StandardMacros.DoOnce` false
                  (:`Completed`
                    (`self.K2_DetachFromActor` self "KeepWorld" "KeepWorld" "KeepWorld"))))
              (:`then_1`
                (`SceneComponent.SetRelativeScale3D` (`self.SM_WindStream`) (`KismetMathLibrary.MakeVector` _newtrack_1 _newtrack_1 _newtrack_1))))
            (else
              (`SceneComponent.SetRelativeScale3D` (`self.Arrow`) (`KismetMathLibrary.MakeVector` _newtrack_0 1.0 1.0)))))
        (:`Finished`
          ;[1 0 0.007957] Retract or Destroy
          (if (`self.Retracting`)
            (`self.K2_DestroyActor`)
            (else
              (`self.Retract`))))))))

(event `Retract`
  ;[0.4255 1 0.7857] Retract
  (set `self.Retracting` true)
  (`ActorComponent.SetActive` (`self.P_WindAdvancedAttackStream`) false false)
  (goto _label :!via `Reverse`))

(fn `UserConstructionScript`)