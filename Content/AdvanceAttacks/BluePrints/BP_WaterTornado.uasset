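; BP_WaterTornado is a water tornado effect actor, apparently for an advance attack, that animates itself on BeginPlay.
; One timeline drives the tornado mesh's Z scale and the upper part's overall scale, which follows a separate ScaleDownFast track when playing forward.
; Shrinkwaterspout reverses the timeline, and the actor destroys itself when the reverse finishes.
; The construction script snaps the upper part to an Arrow component.
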(event `self.ReceiveBeginPlay`
  (`self.StartTornado`))

(event `StartTornado`
  (bind _smupperpart (`self.SMUpperPart`))
  ;[1 1 1] (ian)Scales down and changes material parameter
  (bind (_direction _scale _scaledownfast) (`Timeline|Timeline_0` :!via `PlayFromStart` :!label _label)
    (:`Update`
      (`SceneComponent.SetRelativeScale3D` (`self.SMWaterTornado`) (`KismetMathLibrary.MakeVector` 1.0 1.0 _scale))
      (switch `ETimelineDirection` _direction
        (:`Forward`
          (`SceneComponent.SetRelativeScale3D` _smupperpart (`KismetMathLibrary.Conv_DoubleToVector` _scaledownfast)))
        (:`Backward`
          (`SceneComponent.SetRelativeScale3D` _smupperpart (`KismetMathLibrary.Conv_DoubleToVector` _scale)))))
    (:`Finished`
      (switch `ETimelineDirection` _direction
        (:`Backward`
          (`self.K2_DestroyActor`))))))

(event `Shrink water spout`
  ;[1 1 1] (ian)Scales down and changes material parameter
  (goto _label :!via `Reverse`))

(fn `UserConstructionScript`
  (`SceneComponent.K2_AttachToComponent` (`self.SMUpperPart`) (`self.Arrow`) "None" "SnapToTarget" "KeepRelative" "KeepRelative" true))