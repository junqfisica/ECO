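; BP_GWater01 is a short-lived water attack actor that launches a BP_WaterProjectile.
; On BeginPlay it disables mesh physics and collision, then plays the SpawnWater timeline at half speed to scale the mesh relative to its initial size.
; The timeline's Cast Projectile event spawns the projectile at the mesh transform, passing on owner, target and OwnerHands.
; Scaling and spawning run only with authority, and the actor destroys itself when the timeline finishes.
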(event `self.ReceiveBeginPlay`
  (bind _staticmeshcomponent (`self.StaticMeshComponent`))
  (bind (_returnvalue_location _returnvalue_rotation) (`KismetMathLibrary.BreakTransform` (`SceneComponent.K2_GetComponentToWorld` (`self.StaticMeshComponent`))))
  (`parent.ReceiveBeginPlay`)
  (`|ExecutionSequence`
    (:`then_0`
      ;[0.3444 0.5013 1] Turn off physics and collision
      (`PrimitiveComponent.SetSimulatePhysics` _staticmeshcomponent false)
      (`PrimitiveComponent.SetCollisionEnabled` _staticmeshcomponent "NoCollision")
      (set `self.InitialScale` (`SceneComponent.K2_GetComponentScale` (`self.StaticMeshComponent`))))
    (:`then_2`
      (`TimelineComponent.SetPlayRate` (`self.SpawnWater`) 0.5)
      (bind (_direction _alpha) (`Timeline|SpawnWater` :!via `PlayFromStart`)
        (:`Update`
          ;[0.4549 1 0.7631] Change Scale
          (`/Engine/EditorBlueprintResources/ActorMacros.Switch Has Authority`
            (:`Authority`
              (`SceneComponent.SetWorldScale3D` (`self.StaticMeshComponent`) (* (`self.InitialScale`) _alpha)))))
        (:`Finished`
          (`self.K2_DestroyActor`))
        (:`CastProjectile`
          (`/Engine/EditorBlueprintResources/ActorMacros.Switch Has Authority`
            (:`Authority`
              (`|SpawnActorFromClass` "/Game/AdvanceAttacks/BluePrints/BP_WaterProjectile.BP_WaterProjectile_C" (`KismetMathLibrary.MakeTransform` _returnvalue_location _returnvalue_rotation) "Undefined" "OverrideRootScale" (`self.GetOwner` self) (`self.ProjectileTarget`) (`self.OwnerHands`)))))))))

(fn `UserConstructionScript`
  (`parent.UserConstructionScript`))